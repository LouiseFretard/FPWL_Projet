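; BP_Window_With_Noise is a window Blueprint among the movable interactable objects that keeps two arrow components oscillating during play.
; After the parent BeginPlay, an endless Delay-driven loop swings Arrow and Arrow1 in opposite yaw directions, then back, several times a second.
; Tick and overlap events are disabled, construction only calls the parent, and no noise logic appears in this graph.
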(event EventBeginPlay
  (bind _arrow (Variables|Default|GetArrow))
  (bind _arrow_2 (Variables|Default|GetArrow))
  (bind _arrow1 (Variables|Default|GetArrow1))
  (bind _arrow1_2 (Variables|Default|GetArrow1))
  (bind _relativerotation (Variables|/Script/Engine.SceneComponent|GetRelativeRotation _arrow))
  (bind _relativerotation_2 (Variables|/Script/Engine.SceneComponent|GetRelativeRotation _arrow1))
  (bind _relativerotation_3 (Variables|/Script/Engine.SceneComponent|GetRelativeRotation _arrow_2))
  (bind _relativerotation_4 (Variables|/Script/Engine.SceneComponent|GetRelativeRotation _arrow1_2))
  (|CallParentFunction)
  (Utilities|FlowControl|Delay 0.2 :!label _label)
  (Transformation|SetRelativeRotation _arrow_2 (Math|Rotator|MakeRotator (.roll _relativerotation_3) (.pitch _relativerotation_3) (+ (.yaw _relativerotation_3) 45.0)) false false)
  (Transformation|SetRelativeRotation _arrow1_2 (Math|Rotator|MakeRotator (.roll _relativerotation_4) (.pitch _relativerotation_4) (+ (.yaw _relativerotation_4) -45.0)) false false)
  (Utilities|FlowControl|Delay 0.2)
  (Transformation|SetRelativeRotation _arrow (Math|Rotator|MakeRotator (.roll _relativerotation) (.pitch _relativerotation) (+ (.yaw _relativerotation) -45.0)) false false)
  (Transformation|SetRelativeRotation _arrow1 (Math|Rotator|MakeRotator (.roll _relativerotation_2) (.pitch _relativerotation_2) (+ (.yaw _relativerotation_2) 45.0)) false false)
  (goto _label))

(event Collision|EventActorBeginOverlap
  (params (OtherActor :type Actor%20Object%20Reference))
  (|CallParentFunction OtherActor) ; This node is disabled and will not be called.\nDrag off pins to build functionality.
)

(event EventTick
  (params (DeltaSeconds :type Float%20%28single-precision%29))
  (|CallParentFunction DeltaSeconds) ; This node is disabled and will not be called.\nDrag off pins to build functionality.
)

(event Input|KeyboardEvents|B
  (params (Key :type Key%20Structure :default "None")))

(fn ConstructionScript
  (|CallParentFunction))