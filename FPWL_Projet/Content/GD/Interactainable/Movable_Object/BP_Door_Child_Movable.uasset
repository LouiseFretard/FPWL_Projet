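; Interactable hinged door that swings open and shut via timeline, optionally requiring a letter or held item.
; Activation checks the player's inventories; item use updates inventory, animates a key into the lock, then opens the door.
; Failed attempts wiggle the door or show rust dialogue; unlocked rusted doors snap open and disable collision.
; An overlap shows camera-facing clues when the first inventory item is tagged Second_Key; highlighting uses a runtime-created outline mesh.
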(event OnComponentBeginOverlap(Collision_To_Show_Clue_2)
  (params (OverlappedComponent :type Primitive%20Component%20Object%20Reference) (OtherActor :type Actor%20Object%20Reference) (OtherComp :type Primitive%20Component%20Object%20Reference) (OtherBodyIndex :type Integer) (bFromSweep :type Boolean) (SweepResult :type Hit%20Result%20Structure%20%28by%20ref%29))
  (bind _asbp_diplome_first_person_project (Utilities|Casting|CastToBP_Diplome_First_Person_Project OtherActor))
  (if (Utilities|IsValidClass (Variables|Default|GetGet_Item_Needed_For_Activites))
    (Utilities|IsValid (Utilities|Array|Get(acopy) (Variables|/Game/GD/ThirdPerson/Items_Inventory.Items_Inventory_C|GetAll_Items (Variables|/Game/GD/ThirdPerson/Blueprints/BP_Diplome_First_Person_Project.BP_Diplome_First_Person_Project_C|GetItems_Inventory _asbp_diplome_first_person_project)))
      (:Is%20Valid
        (if (Actor|ActorHasTag (Utilities|Array|Get(acopy) (Variables|/Game/GD/ThirdPerson/Items_Inventory.Items_Inventory_C|GetAll_Items (Variables|/Game/GD/ThirdPerson/Blueprints/BP_Diplome_First_Person_Project.BP_Diplome_First_Person_Project_C|GetItems_Inventory _asbp_diplome_first_person_project))) "Second_Key")
          (Variables|Default|SetCan_Turn_With_Player_? true)
          (Development|SetHiddeninGame (Variables|Default|GetClue_To_How_Get_Item) false false))))))

(event OnComponentEndOverlap(Collision_To_Show_Clue_2)
  (params (OverlappedComponent :type Primitive%20Component%20Object%20Reference) (OtherActor :type Actor%20Object%20Reference) (OtherComp :type Primitive%20Component%20Object%20Reference) (OtherBodyIndex :type Integer))
  (Utilities|Casting|CastToBP_Diplome_First_Person_Project OtherActor)
  (if (Utilities|IsValidClass (Variables|Default|GetGet_Item_Needed_For_Activites))
    (Variables|Default|SetCan_Turn_With_Player_? false)
    (Development|SetHiddeninGame (Variables|Default|GetClue_To_How_Get_Item) true false)))

(event Custom|Open_Doors
  (bind _arrow_door (Variables|Default|GetArrow_Door))
  (bind _relativerotation (Variables|/Script/Engine.SceneComponent|GetRelativeRotation _arrow_door))
  (if (not (Variables|Default|GetRouille_?))
    (if (not (Variables|/Game/GD/ThirdPerson/Blueprints/BP_Diplome_First_Person_Project.BP_Diplome_First_Person_Project_C|GetHidden_Sound_? (Variables|Default|GetFirst_Person)))
      (Audio|PlaySound2D "/Game/GD/Sound/Environment_Noise/SC_Door_Opening_Cue.SC_Door_Opening_Cue" 1.0 1.0 0.0 0 0)
      (else
        (Audio|PlaySound2D "/Game/GD/Sound/Environment_Noise/Hidden_Environment_Sound/SC_Door_Opening_Minecraft_Hidden_Cue.SC_Door_Opening_Minecraft_Hidden_Cue" 1.0 1.0 0.0 0 0)))
    (Collision|SetCollisionEnabled (Variables|Default|GetBox_Back_Collision) "NoCollision")
    (if (not (Variables|Default|GetOpen_?))
      (Variables|Default|SetOpen_? true)
      (Variables|Default|SetDoor_Original_Relative_Rotation (Variables|/Script/Engine.SceneComponent|GetRelativeRotation (Variables|Default|GetArrow_Door)))
      (bind _time_to_move_object (Timeline|Timeline_0 PlayFromStart)
        (:Update
          (Transformation|SetRelativeRotation (Variables|Default|GetArrow_Door) (Math|Rotator|Lerp(Rotator) (Variables|Default|GetDoor_Original_Relative_Rotation) (Math|Rotator|MakeRotator (.roll (Variables|Default|GetDoor_Original_Relative_Rotation)) (.pitch (Variables|Default|GetDoor_Original_Relative_Rotation)) (+ (.yaw (Variables|Default|GetDoor_Original_Relative_Rotation)) (* (Variables|Default|GetWhat_Side_To_Open) 1e+01))) _time_to_move_object) false false))
        (:Finished
          (if (not (Variables|Default|GetSuccess_Dialogue_Said_?))
            (Variables|Default|SetSuccess_Dialogue_Said_? true)
            (if (not (Utilities|Enum|Equal(Enum) (Variables|Default|GetDialogue_De_Succès) ""))
              (Default|TransmissDialogue (Variables|Default|GetFirst_Person) (Variables|Default|GetDialogue_De_Succès))))
          (Collision|SetCollisionProfileName (Variables|Default|GetCollision_To_Show_Clue_2) "NoCollision" true :!class /Script/Engine.PrimitiveComponent)
          (Collision|SetCollisionEnabled (Variables|Default|GetBox_Back_Collision) "QueryAndPhysics")
          (Utilities|FlowControl|Delay 2.0)
          (Default|EndDialogue (Variables|/Game/GD/ThirdPerson/Blueprints/BP_Diplome_First_Person_Project.BP_Diplome_First_Person_Project_C|GetHUD (Variables|Default|GetFirst_Person)))))
      (else
        (Variables|Default|SetOpen_? false)
        (Timeline|Timeline_0 ReverseFromEnd)))
    (else
      (Variables|Default|SetOpen_? true)
      (Transformation|SetRelativeRotation (Variables|Default|GetArrow_Door) (Math|Rotator|MakeRotator (.roll _relativerotation) (.pitch _relativerotation) (+ (.yaw _relativerotation) (* (Variables|Default|GetWhat_Side_To_Open) 9.0))) false false)
      (Default|TransmissDialogue (Variables|Default|GetFirst_Person) (Variables|Default|GetDialogue_Succès_Rouille))
      (Collision|SetCollisionProfileName (Variables|Default|GetBox_Back_Collision) "NoCollision" true :!class /Script/Engine.PrimitiveComponent))))

(event Custom|Animation
  (params (Class_Of_Used_Actor :type Actor%20Class%20Reference))
  (bind _used_object (Variables|Default|GetUsed_Object))
  (bind _used_object_2 (Variables|Default|GetUsed_Object))
  (bind _first_person (Variables|Default|GetFirst_Person))
  (bind _childactor (Variables|/Script/Engine.ChildActorComponent|GetChildActor _used_object))
  (bind _childactor_2 (Variables|/Script/Engine.ChildActorComponent|GetChildActor _used_object_2))
  (Variables|Default|SetCan_Turn_With_Player_? false)
  (Development|SetHiddeninGame (Variables|Default|GetClue_To_How_Get_Item) true false)
  (Utilities|Array|SetArrayElem (Variables|/Game/GD/ThirdPerson/Items_Inventory.Items_Inventory_C|GetAll_Items (Variables|/Game/GD/ThirdPerson/Blueprints/BP_Diplome_First_Person_Project.BP_Diplome_First_Person_Project_C|GetItems_Inventory (Variables|Default|GetFirst_Person))) 0 0)
  (Default|ReorganiseInventory _first_person)
  (Default|SelectedItem (Variables|/Game/GD/ThirdPerson/Blueprints/BP_Diplome_First_Person_Project.BP_Diplome_First_Person_Project_C|GetHUD _first_person) _first_person)
  (Default|ChangeItemHoldinHand _first_person)
  (Transformation|SetWorldLocation (Variables|Default|Get1st_Part_Of_Travel) (Transformation|GetWorldLocation (Variables|/Game/GD/ThirdPerson/Blueprints/BP_Diplome_First_Person_Project.BP_Diplome_First_Person_Project_C|GetHand_Place (Variables|Default|GetFirst_Person))) false false)
  (ChildActorComponent|SetChildActorClass _used_object_2 "/Game/GD/BP_Key_For_Door.BP_Key_For_Door_C")
  (Collision|SetActorEnableCollision _childactor_2 false)
  (bind _item_track (Timeline|Timeline_1 PlayFromStart)
    (:Update
      (Transformation|SetActorLocation _childactor_2 (Math|Vector|Lerp(Vector) (Transformation|GetWorldLocation (Variables|Default|Get1st_Part_Of_Travel)) (Transformation|GetWorldLocation (Variables|Default|Get2nd_Part_Of_Travel)) _item_track) false false))
    (:Finished
      (Variables|Default|SetGet_Item_Needed_For_Activites 0)
      (Variables|Default|SetUsed_Item_Original_Rotation (Transformation|GetActorRotation _childactor))
      (bind _item_track_2 (Timeline|Timeline_2 PlayFromStart)
        (:Update
          (Transformation|SetActorRotation _childactor (Math|Rotator|Lerp(Rotator) (Variables|Default|GetUsed_Item_Original_Rotation) (Math|Rotator|CombineRotators (Variables|Default|GetUsed_Item_Original_Rotation) (Math|Rotator|MakeRotator 0.0 (.pitch (Math|Vector|RotatorfromAxisandAngle "0.000000,1.000000, 0" -9e+01)) 0.0)) _item_track_2)))
        (:Finished
          (Transformation|AttachComponentToComponent _used_object (Variables|Default|GetDoor) "None" "KeepWorld" "KeepWorld" "KeepWorld" true))))))

(event EventBeginPlay
  (|CallParentFunction) ; This node is disabled and will not be called.\nDrag off pins to build functionality.
)

(event Collision|EventActorBeginOverlap
  (params (OtherActor :type Actor%20Object%20Reference))
  (|CallParentFunction OtherActor) ; This node is disabled and will not be called.\nDrag off pins to build functionality.
)

(event EventTick
  (params (DeltaSeconds :type Float%20%28single-precision%29))
  (if (Variables|Default|GetCan_Turn_With_Player_?)
    (bind _asbp_diplome_first_person_project (Utilities|Casting|CastToBP_Diplome_First_Person_Project (Game|GetPlayerCharacter 0)))
    (Transformation|SetWorldRotation (Variables|Default|GetClue_To_How_Get_Item) (Math|Rotator|MakeRotator (.roll (Transformation|GetWorldRotation (Variables|/Game/GD/ThirdPerson/Blueprints/BP_Diplome_First_Person_Project.BP_Diplome_First_Person_Project_C|GetFirst_Person_Camera _asbp_diplome_first_person_project))) (+ (.pitch (Transformation|GetWorldRotation (Variables|/Game/GD/ThirdPerson/Blueprints/BP_Diplome_First_Person_Project.BP_Diplome_First_Person_Project_C|GetFirst_Person_Camera _asbp_diplome_first_person_project))) 9e+01) (.yaw (Transformation|GetWorldRotation (Variables|/Game/GD/ThirdPerson/Blueprints/BP_Diplome_First_Person_Project.BP_Diplome_First_Person_Project_C|GetFirst_Person_Camera _asbp_diplome_first_person_project)))) false false)))

(event EventActivationMovable
  (params (Actor_Hit :type Actor%20Object%20Reference) (Component_Hit :type Primitive%20Component%20Object%20Reference))
  (bind _get_item_needed_for_activites (Variables|Default|GetGet_Item_Needed_For_Activites))
  (bind _get_item_needed_for_activites_2 (Variables|Default|GetGet_Item_Needed_For_Activites))
  (bind _arrow_door (Variables|Default|GetArrow_Door))
  (bind _arrow_door_2 (Variables|Default|GetArrow_Door))
  (bind _dialogue_avec_manque_objet_pour_utilisation (Variables|Default|GetDialogue_Avec_Manque_Objet_Pour_Utilisation))
  (bind _arrow_door_3 (Variables|Default|GetArrow_Door))
  (bind _relativerotation (Variables|/Script/Engine.SceneComponent|GetRelativeRotation _arrow_door_2))
  (bind _relativerotation_2 (Variables|/Script/Engine.SceneComponent|GetRelativeRotation _arrow_door))
  (bind _relativerotation_3 (Variables|/Script/Engine.SceneComponent|GetRelativeRotation _arrow_door_3))
  (bind _asbp_diplome_first_person_project (Utilities|Casting|CastToBP_Diplome_First_Person_Project Actor_Hit))
  (Variables|Default|SetFirst_Person _asbp_diplome_first_person_project)
  (if (== Component_Hit (Variables|Default|GetBox_Back_Collision))
    (if (not (Variables|Default|GetOpen_?))
      (if (Variables|Default|GetOpen_Left_Side_?) :!label _label
        (Variables|Default|SetWhat_Side_To_Open 1e+01 :!label _label_2)
        (if (Utilities|IsValidClass _get_item_needed_for_activites_2) :!label _label_3
          (Utilities|Casting|CastToBP_Base_Parent_Interactainable_DocumentsClass _get_item_needed_for_activites_2
            (:then
              (for _index (range (Variables|/Game/GD/ThirdPerson/Letter_Inventory.Letter_Inventory_C|GetMin_Index (Variables|/Game/GD/ThirdPerson/Blueprints/BP_Diplome_First_Person_Project.BP_Diplome_First_Person_Project_C|GetLetter_Inventory (Variables|Default|GetFirst_Person))) (Variables|/Game/GD/ThirdPerson/Letter_Inventory.Letter_Inventory_C|GetMax_Index (Variables|/Game/GD/ThirdPerson/Blueprints/BP_Diplome_First_Person_Project.BP_Diplome_First_Person_Project_C|GetLetter_Inventory (Variables|Default|GetFirst_Person))))
                (if (== (Utilities|GetClass (Utilities|Array|Get(acopy) (Variables|/Game/GD/ThirdPerson/Letter_Inventory.Letter_Inventory_C|GetAll_Letters (Variables|/Game/GD/ThirdPerson/Blueprints/BP_Diplome_First_Person_Project.BP_Diplome_First_Person_Project_C|GetLetter_Inventory (Variables|Default|GetFirst_Person))) _index)) (Variables|Default|GetGet_Item_Needed_For_Activites))
                  (CallFunction|OpenDoors)
                  (Default|TransmissDialogue (Variables|Default|GetFirst_Person) (Variables|Default|GetDialogue_De_Succès)))))
            (:CastFailed
              (Utilities|Casting|CastToBP_Base_Parent_Inventory_ItemClass _get_item_needed_for_activites_2
                (:then
                  (if (== _get_item_needed_for_activites (Variables|/Script/Engine.ChildActorComponent|GetChildActorClass (Variables|/Game/GD/ThirdPerson/Blueprints/BP_Diplome_First_Person_Project.BP_Diplome_First_Person_Project_C|GetItem_Hold (Variables|Default|GetFirst_Person))))
                    (CallFunction|Animation _get_item_needed_for_activites)
                    (Utilities|FlowControl|Delay 1.0)
                    (CallFunction|OpenDoors)
                    (elif (not (Variables|Default|GetRouille_?))
                      (Audio|PlaySound2D "/Game/GD/Sound/Environment_Noise/SC_Trying_To_Open_Locked_Door_Cue.SC_Trying_To_Open_Locked_Door_Cue" 1.0 1.0 0.0 0 0)
                      (Utilities|FlowControl|DoOnce false :!label _label_4
                        (:Completed
                          (Transformation|SetRelativeRotation _arrow_door_3 (Math|Rotator|MakeRotator (.roll _relativerotation_3) (.pitch _relativerotation_3) (+ (.yaw _relativerotation_3) 2.0)) false false)
                          (Utilities|FlowControl|Delay 0.1)
                          (Transformation|SetRelativeRotation _arrow_door_3 (Math|Rotator|MakeRotator (.roll _relativerotation) (.pitch _relativerotation) (- (.yaw _relativerotation) 4.0)) false false)
                          (Utilities|FlowControl|Delay 0.1)
                          (Transformation|SetRelativeRotation _arrow_door (Math|Rotator|MakeRotator (.roll _relativerotation_2) (.pitch _relativerotation_2) (+ (.yaw _relativerotation_2) 2.0)) false false)
                          (if (not (Utilities|Enum|Equal(Enum) _dialogue_avec_manque_objet_pour_utilisation ""))
                            (Default|TransmissDialogue (Variables|Default|GetFirst_Person) _dialogue_avec_manque_objet_pour_utilisation)
                            (Utilities|FlowControl|Delay 2.0)
                            (Default|EndDialogue (Variables|/Game/GD/ThirdPerson/Blueprints/BP_Diplome_First_Person_Project.BP_Diplome_First_Person_Project_C|GetHUD (Variables|Default|GetFirst_Person)))
                            (goto _label_4 Reset)
                            (else
                              (goto _label_4 Reset)))))
                      (else
                        (Default|TransmissDialogue (Variables|Default|GetFirst_Person) (Variables|Default|GetDialogue_si_rouille))))))
                (:CastFailed
                  (goto _label_4)))))
          (else
            (if (not (Variables|/Game/GD/ThirdPerson/Blueprints/BP_Diplome_First_Person_Project.BP_Diplome_First_Person_Project_C|GetHidden_Sound_? (Variables|Default|GetFirst_Person)))
              (Audio|PlaySound2D "/Game/GD/Sound/Environment_Noise/SC_Door_Opening_Cue.SC_Door_Opening_Cue" 1.0 1.0 0.0 0 0)
              (else
                (Audio|PlaySound2D "/Game/GD/Sound/Environment_Noise/Hidden_Environment_Sound/SC_Door_Opening_Minecraft_Hidden_Cue.SC_Door_Opening_Minecraft_Hidden_Cue" 1.0 1.0 0.0 0 0)))
            (Collision|SetCollisionEnabled (Variables|Default|GetBox_Back_Collision) "NoCollision")
            (if (not (Variables|Default|GetOpen_?))
              (Variables|Default|SetOpen_? true)
              (Variables|Default|SetDoor_Original_Relative_Rotation (Variables|/Script/Engine.SceneComponent|GetRelativeRotation (Variables|Default|GetArrow_Door)))
              (bind _time_to_move_object (Timeline|Timeline_0 PlayFromStart)
                (:Update
                  (Transformation|SetRelativeRotation (Variables|Default|GetArrow_Door) (Math|Rotator|Lerp(Rotator) (Variables|Default|GetDoor_Original_Relative_Rotation) (Math|Rotator|MakeRotator (.roll (Variables|Default|GetDoor_Original_Relative_Rotation)) (.pitch (Variables|Default|GetDoor_Original_Relative_Rotation)) (+ (.yaw (Variables|Default|GetDoor_Original_Relative_Rotation)) (* (Variables|Default|GetWhat_Side_To_Open) 1e+01))) _time_to_move_object) false false))
                (:Finished
                  (if (not (Variables|Default|GetSuccess_Dialogue_Said_?))
                    (Variables|Default|SetSuccess_Dialogue_Said_? true)
                    (if (not (Utilities|Enum|Equal(Enum) (Variables|Default|GetDialogue_De_Succès) ""))
                      (Default|TransmissDialogue (Variables|Default|GetFirst_Person) (Variables|Default|GetDialogue_De_Succès))))
                  (Collision|SetCollisionProfileName (Variables|Default|GetCollision_To_Show_Clue_2) "NoCollision" true :!class /Script/Engine.PrimitiveComponent)
                  (Collision|SetCollisionEnabled (Variables|Default|GetBox_Back_Collision) "QueryAndPhysics")
                  (Utilities|FlowControl|Delay 2.0)
                  (Default|EndDialogue (Variables|/Game/GD/ThirdPerson/Blueprints/BP_Diplome_First_Person_Project.BP_Diplome_First_Person_Project_C|GetHUD (Variables|Default|GetFirst_Person)))))
              (else
                (Variables|Default|SetOpen_? false)
                (Timeline|Timeline_0 ReverseFromEnd)))))
        (elif (Variables|Default|GetOpen_Right_Side_?)
          (Variables|Default|SetWhat_Side_To_Open -1e+01 :!label _label_5)
          (goto _label_3)))
      (else
        (if (Variables|Default|GetOpen_Left_Side_?) :!label _label_6
          (goto _label_2)
          (elif (Variables|Default|GetOpen_Right_Side_?)
            (goto _label_5)))))
    (elif (== Component_Hit (Variables|Default|GetBox_Front_Collision))
      (if (not (Variables|Default|GetOpen_?))
        (goto _label)
        (else
          (goto _label_6))))))

(event EventOnHighlight
  (bind _door (Variables|Default|GetDoor))
  (Utilities|IsValid (Variables|Default|GetOutline_Mesh)
    (:Is%20Valid
      (Rendering|SetVisibility (Variables|Default|GetOutline_Mesh) true false))
    (:Is%20Not%20Valid
      (bind _returnvalue (AddComponent|AddStaticMeshComponent false (Math|Transform|MakeTransform (Variables|/Script/Engine.SceneComponent|GetRelativeLocation _door) (Variables|/Script/Engine.SceneComponent|GetRelativeRotation _door) (Transformation|GetWorldScale _door))))
      (bind _output_get (Variables|Default|SetOutline_Mesh _returnvalue))
      (Components|StaticMesh|SetStaticMesh _output_get (Variables|/Script/Engine.StaticMeshComponent|GetStaticMesh (Variables|Default|GetDoor)))
      (Rendering|Material|SetMaterial (Variables|Default|GetOutline_Mesh) 0 "/Game/GD/M_Test_Outline.M_Test_Outline")
      (Transformation|AttachComponentToComponent (Variables|Default|GetOutline_Mesh) (Variables|Default|GetDoor) "None" "KeepWorld" "KeepWorld" "KeepWorld" true))))

(event EventStopHighlight
  (bind _outline_mesh (Variables|Default|GetOutline_Mesh))
  (Utilities|IsValid _outline_mesh
    (:Is%20Valid
      (Rendering|SetVisibility _outline_mesh false false))))

(fn ConstructionScript
  (|CallParentFunction))