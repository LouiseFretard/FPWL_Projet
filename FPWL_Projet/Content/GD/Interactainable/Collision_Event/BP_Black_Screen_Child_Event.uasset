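; Child collision-event actor that runs a one-shot opening sequence, lifting the black screen and starting the first tutorial part.
; May_Start toggles player input through a FlipFlop, blocks spyglass pickup, then waits out an optional 2D sound before clearing the screen.
; It shows optional timed dialogue, triggers the tutorial, waits, restores input, flags the start as finished and destroys itself.
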(event Custom|May_Start
  (bind _returnvalue (Game|GetPlayerController 0))
  (bind _hud (Variables|Default|GetHUD))
  (bind _sound_to_play_1st (Variables|Default|GetSound_To_Play_1st))
  (bind _dialogue_1 (Variables|Default|GetDialogue_1))
  (CallFunction|DisablePlayerInput)
  (bind _returnvalue_2 (Actor|GetActorOfClass "/Game/GD/Interactainable/Inventory/BP_Spyglass_Child_Inventory.BP_Spyglass_Child_Inventory_C"))
  (Default|Can'tTakeSpyglass _returnvalue_2)
  (Utilities|IsValid _sound_to_play_1st
    (:Is%20Valid
      (Audio|PlaySound2D _sound_to_play_1st 1.0 1.0 0.0 0 0)
      (Utilities|FlowControl|Delay (Variables|/Script/Engine.SoundBase|GetDuration _sound_to_play_1st)))
    (:Is%20Not%20Valid
      _))
  (if (== (Variables|Default|GetBlack_Screen_Off_?) true)
    (Default|BlackScreenOff (Variables|Default|GetHUD))
    (Utilities|FlowControl|Delay 0.2))
  (if (not (Utilities|Enum|Equal(Enum) _dialogue_1 ""))
    (Default|ShowDialogue _hud _dialogue_1)
    (Utilities|FlowControl|Delay (Variables|Default|GetTime_Between_Dialogues_%28in_s%29))
    (Default|EndDialogue _hud))
  (Default|Tutorial1stPart (Variables|Default|GetFirst_Person))
  (Utilities|FlowControl|Delay (Variables|Default|GetDuration))
  (if (Variables|Default|GetDisable_Player_On_?)
    (Input|EnableInput (Variables|Default|GetFirst_Person) _returnvalue)
    (Input|SetInputModeGameOnly _returnvalue)
    (Variables|/Script/Engine.PlayerController|SetbShowMouseCursor _returnvalue false))
  (Default|EndDialogue (Variables|Default|GetHUD))
  (if (Math|Boolean|ORBoolean (not (Utilities|Enum|Equal(Enum) (Variables|Default|GetDialogue_1) "")) (not (Utilities|Enum|Equal(Enum) (Variables|Default|GetDialogue_2) "")) (not (Utilities|Enum|Equal(Enum) (Variables|Default|GetDialogue_3) "")))
    (Default|EndDialogue (Variables|Default|GetHUD)))
  (Variables|/Game/GD/ThirdPerson/Blueprints/BP_Diplome_First_Person_Project.BP_Diplome_First_Person_Project_C|SetStart_Finished_? (Variables|Default|GetFirst_Person) true)
  (Actor|DestroyActor))

(event EventBeginPlay
  (|CallParentFunction))

(event Collision|EventActorBeginOverlap
  (params (OtherActor :type Actor%20Object%20Reference))
  (|CallParentFunction OtherActor))

(event EventTick
  (params (DeltaSeconds :type Float%20%28single-precision%29))
  (|CallParentFunction DeltaSeconds))

(event EventBlackScreen)

(event EventSound)

(event EventDisablePlayerInput
  (Utilities|FlowControl|FlipFlop
    (:A
      (if (Variables|Default|GetDisable_Player_On_?)
        (Input|DisableInput (Variables|Default|GetFirst_Person) (Game|GetPlayerController 0))))
    (:B
      (if (Variables|Default|GetDisable_Player_On_?)
        (Input|EnableInput (Variables|Default|GetFirst_Person) (Game|GetPlayerController 0))))))

(fn ConstructionScript
  (|CallParentFunction))