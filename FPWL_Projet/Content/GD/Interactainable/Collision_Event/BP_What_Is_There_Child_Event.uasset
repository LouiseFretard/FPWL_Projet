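; Child trigger event that plays up to two lines of dialogue when overlapped, then destroys itself.
; Overlap may wait briefly depending on current HUD text, sends the first line through FirstPerson's TransmissDialogue and the second straight to the HUD, with timed pauses, then ends the dialogue.
; A separate DisablePlayerInput event toggles player input when enabled.
; BlackScreen and Sound events are empty; their leftover logic is disconnected.
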(event EventBeginPlay
  (|CallParentFunction) ; This node is disabled and will not be called.\nDrag off pins to build functionality.
)

(event Collision|EventActorBeginOverlap
  (params (OtherActor :type Actor%20Object%20Reference))
  (bind _dialogue_1 (Variables|Default|GetDialogue_1))
  (bind _dialogue_2 (Variables|Default|GetDialogue_2))
  (|CallParentFunction OtherActor)
  (if (Utilities|Enum|NotEqual(Enum) (Class|TextBlock|GetText (Variables|/Game/GD/Widget/HUD.HUD_C|GetHow_To_Show_Dialogue (Variables|Default|GetHUD))) (Variables|Default|GetNewVar_0))
    (Utilities|FlowControl|Delay 2.0))
  (if (not (Utilities|Enum|Equal(Enum) _dialogue_1 ""))
    (Default|TransmissDialogue (Variables|Default|GetFirst_Person) _dialogue_1)
    (Utilities|FlowControl|Delay (Variables|Default|GetTime_Between_Dialogues_%28in_s%29)))
  (if (not (Utilities|Enum|Equal(Enum) _dialogue_2 ""))
    (Default|ShowDialogue (Variables|Default|GetHUD) _dialogue_2)
    (Utilities|FlowControl|Delay (Variables|Default|GetTime_Between_Dialogues_%28in_s%29)))
  (Default|EndDialogue (Variables|Default|GetHUD))
  (if (Math|Boolean|ORBoolean (not (Utilities|Enum|Equal(Enum) (Variables|Default|GetDialogue_1) "")) (not (Utilities|Enum|Equal(Enum) (Variables|Default|GetDialogue_2) "")) (not (Utilities|Enum|Equal(Enum) (Variables|Default|GetDialogue_3) "")))
    (Default|EndDialogue (Variables|Default|GetHUD)))
  (Actor|DestroyActor))

(event EventTick
  (params (DeltaSeconds :type Float%20%28single-precision%29))
  (|CallParentFunction DeltaSeconds))

(event EventBlackScreen)

(event EventSound)

(event EventDisablePlayerInput
  (Utilities|FlowControl|FlipFlop
    (:A
      (if (Variables|Default|GetDisable_Player_On_?)
        (Input|DisableInput (Variables|Default|GetFirst_Person) (Game|GetPlayerController 0))))
    (:B
      (if (Variables|Default|GetDisable_Player_On_?)
        (Input|EnableInput (Variables|Default|GetFirst_Person) (Game|GetPlayerController 0))))))

(fn ConstructionScript
  (|CallParentFunction))