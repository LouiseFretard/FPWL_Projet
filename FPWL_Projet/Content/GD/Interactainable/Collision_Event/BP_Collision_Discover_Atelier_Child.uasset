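; Overlap-triggered child event actor that marks the atelier as discovered and updates the player's objective to calling Cécile back.
; On overlap, a non-empty Dialogue1 starts a delayed sequence sending up to two lines through FirstPerson, then ends the HUD dialogue.
; The same branch flags AtelierDiscovered on BP_Phone_Child_ININNO, plays the objective sound, sets the HUD objective text and destroys the actor.
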(event EventBeginPlay
  (|CallParentFunction) ; This node is disabled and will not be called.\nDrag off pins to build functionality.
)

(event Collision|EventActorBeginOverlap
  (params (OtherActor :type Actor%20Object%20Reference))
  (bind _dialogue_1 (Variables|Default|GetDialogue_1))
  (bind _hud (Variables|Default|GetHUD))
  (bind _dialogue_2 (Variables|Default|GetDialogue_2))
  (|CallParentFunction OtherActor)
  (if (not (Utilities|Enum|Equal(Enum) _dialogue_1 ""))
    (Default|TransmissDialogue (Variables|Default|GetFirst_Person) _dialogue_1)
    (Utilities|FlowControl|Delay (Variables|Default|GetTime_Between_Dialogues_%28in_s%29))
    (if (not (Utilities|Enum|Equal(Enum) _dialogue_2 ""))
      (Default|TransmissDialogue (Variables|Default|GetFirst_Person) _dialogue_2)
      (Utilities|FlowControl|Delay (Variables|Default|GetTime_Between_Dialogues_%28in_s%29)))
    (if (Math|Boolean|ORBoolean (not (Utilities|Enum|Equal(Enum) (Variables|Default|GetDialogue_1) "")) (not (Utilities|Enum|Equal(Enum) (Variables|Default|GetDialogue_2) "")) (not (Utilities|Enum|Equal(Enum) (Variables|Default|GetDialogue_3) "")))
      (Default|EndDialogue _hud))
    (bind _returnvalue (Actor|GetActorOfClass "/Game/GD/Interactainable/Object_Interact_Not_Inspectable_Not_Need_Object/BP_Phone_Child_ININNO.BP_Phone_Child_ININNO_C"))
    (Variables|/Game/GD/Interactainable/Object_Interact_Not_Inspectable_Not_Need_Object/BP_Phone_Child_ININNO.BP_Phone_Child_ININNO_C|SetAtelier_Discovered_? _returnvalue true)
    (Audio|PlaySound2D "/Game/GD/Sound/Environment_Noise/SC_Objectif_Sound_Cue.SC_Objectif_Sound_Cue" 1.0 1.0 0.0 0 0)
    (Rendering|Components|TextRender|SetText (Variables|/Game/GD/Widget/HUD.HUD_C|GetHow_To_Show_Objective _hud) "Objectif : Rappeler Cécile")
    (Actor|DestroyActor)))

(event EventTick
  (params (DeltaSeconds :type Float%20%28single-precision%29))
  (|CallParentFunction DeltaSeconds) ; This node is disabled and will not be called.\nDrag off pins to build functionality.
)

(fn ConstructionScript
  (|CallParentFunction))