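; Collision event actor that gives the player the Morse code decoding objective.
; On overlap it runs the parent logic, then casts the other actor to the first-person player character.
; If the cast succeeds, it sets the French objective text on that character's HUD, plays a 2D objective sound and destroys itself, so it triggers only once.
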(event EventBeginPlay
  (|CallParentFunction) ; This node is disabled and will not be called.\nDrag off pins to build functionality.
)

(event Collision|EventActorBeginOverlap
  (params (OtherActor :type Actor%20Object%20Reference))
  (|CallParentFunction OtherActor)
  (bind _asbp_diplome_first_person_project (Utilities|Casting|CastToBP_Diplome_First_Person_Project OtherActor))
  (Rendering|Components|TextRender|SetText (Variables|/Game/GD/Widget/HUD.HUD_C|GetHow_To_Show_Objective (Variables|/Game/GD/ThirdPerson/Blueprints/BP_Diplome_First_Person_Project.BP_Diplome_First_Person_Project_C|GetHUD _asbp_diplome_first_person_project)) "Objectif : Décoder le morse")
  (Audio|PlaySound2D "/Game/GD/Sound/Environment_Noise/SC_Objectif_Sound_Cue.SC_Objectif_Sound_Cue" 1.0 1.0 0.0 0 0)
  (Actor|DestroyActor))

(event EventTick
  (params (DeltaSeconds :type Float%20%28single-precision%29))
  (|CallParentFunction DeltaSeconds) ; This node is disabled and will not be called.\nDrag off pins to build functionality.
)

(fn ConstructionScript
  (|CallParentFunction))