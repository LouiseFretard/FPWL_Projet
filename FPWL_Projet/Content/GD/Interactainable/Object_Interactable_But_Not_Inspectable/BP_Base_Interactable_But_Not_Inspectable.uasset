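; Base interactable, not inspectable, that checks whether the first-person player's held item carries the required tag.
; On a match, it clears the inventory slot, updates the hand, and a timeline moves an actor found by the held item's class from hand to LocateActorMoving, then calls Success.
; Otherwise, a "Special" item tag calls Special, or a "Quel_Enfer" hit-component tag calls Balance_De_Mort.
; These three outcome events are empty hooks.
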(event Custom|Success)

(event Custom|Got_Right_Object_?
  (params (Pawn :type Pawn%20Object%20Reference) (Get_Hit_Actor :type Actor%20Object%20Reference))
  (Variables|Default|SetGet%20Hit%20Actor Get_Hit_Actor)
  (bind _asbp_diplome_first_person_project (Utilities|Casting|CastToBP_Diplome_First_Person_Project Pawn)
    (:then
      (Variables|Default|SetFirst_Person _asbp_diplome_first_person_project)
      (Development|PrintString "Nice")
      (Variables|Default|SetHold_Class (Utilities|GetClass (Variables|/Script/Engine.ChildActorComponent|GetChildActor (Variables|/Game/GD/ThirdPerson/Blueprints/BP_Diplome_First_Person_Project.BP_Diplome_First_Person_Project_C|GetItem_Hold _asbp_diplome_first_person_project))))
      (if (Actor|ActorHasTag (Variables|/Script/Engine.ChildActorComponent|GetChildActor (Variables|/Game/GD/ThirdPerson/Blueprints/BP_Diplome_First_Person_Project.BP_Diplome_First_Person_Project_C|GetItem_Hold _asbp_diplome_first_person_project)) (Variables|Default|GetTag_Of_Object_To_Be_Used))
        (bind _returnvalue (Actor|GetActorOfClass (Variables|Default|GetHold_Class)))
        (Variables|Default|SetActor_Moving _returnvalue)
        (Utilities|Array|SetArrayElem (Variables|/Game/GD/ThirdPerson/Items_Inventory.Items_Inventory_C|GetAll_Items (Variables|/Game/GD/ThirdPerson/Blueprints/BP_Diplome_First_Person_Project.BP_Diplome_First_Person_Project_C|GetItems_Inventory _asbp_diplome_first_person_project)) (Variables|/Game/GD/ThirdPerson/Items_Inventory.Items_Inventory_C|GetIndex_For_Player (Variables|/Game/GD/ThirdPerson/Blueprints/BP_Diplome_First_Person_Project.BP_Diplome_First_Person_Project_C|GetItems_Inventory _asbp_diplome_first_person_project)) 0)
        (Default|ChangeItemHoldinHand _asbp_diplome_first_person_project)
        (bind _time_to_move_object (Timeline|Timeline_0 PlayFromStart)
          (:Update
            (Transformation|SetActorLocation _returnvalue (Math|Vector|Lerp(Vector) (Transformation|GetWorldLocation (Variables|/Game/GD/ThirdPerson/Blueprints/BP_Diplome_First_Person_Project.BP_Diplome_First_Person_Project_C|GetItem_Hold _asbp_diplome_first_person_project)) (Transformation|GetWorldLocation (Variables|Default|GetLocate_Actor_Moving)) _time_to_move_object) false false))
          (:Finished
            (CallFunction|Success)))
        (elif (Actor|ActorHasTag (Variables|/Script/Engine.ChildActorComponent|GetChildActor (Variables|/Game/GD/ThirdPerson/Blueprints/BP_Diplome_First_Person_Project.BP_Diplome_First_Person_Project_C|GetItem_Hold _asbp_diplome_first_person_project)) "Special")
          (CallFunction|Special (Variables|Default|GetGet%20Hit%20Actor))
          (elif (Components|ComponentHasTag (Variables|/Game/GD/ThirdPerson/Blueprints/BP_Diplome_First_Person_Project.BP_Diplome_First_Person_Project_C|GetHit%20Component _asbp_diplome_first_person_project) "Quel_Enfer")
            (CallFunction|BalanceDeMort (Variables|/Game/GD/ThirdPerson/Blueprints/BP_Diplome_First_Person_Project.BP_Diplome_First_Person_Project_C|GetHit%20Component _asbp_diplome_first_person_project))
            (else
              (Development|PrintString "NOOO"))))))
    (:CastFailed
      (Development|PrintString "WRONG"))))

(event Custom|Special
  (params (Hit_Actor :type Actor%20Object%20Reference)))

(event Custom|Balance_De_Mort
  (params (Hit_Component :type Primitive%20Component%20Object%20Reference)))

(event EventBeginPlay)

(event Collision|EventActorBeginOverlap
  (params (OtherActor :type Actor%20Object%20Reference)))

(event EventTick
  (params (DeltaSeconds :type Float%20%28single-precision%29)))

(fn ConstructionScript)