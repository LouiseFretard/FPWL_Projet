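; Interactable fireplace that takes logs and a mystery box, lights held matches, and shows a flickering fire light.
; On Success, it replaces the moved actor with a child actor that timelines lerp into one of three log slots or the box spot.
; The third log or the box enables CanSetFire.
; Special passes the hit actor to the held match, while Switch_On_Fire ramps up a point light, then loops random intensity timelines.
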(event OnComponentHit(Box)
  (params (HitComponent :type Primitive%20Component%20Object%20Reference) (OtherActor :type Actor%20Object%20Reference) (OtherComp :type Primitive%20Component%20Object%20Reference) (NormalImpulse :type Vector :default "0, 0, 0") (Hit :type Hit%20Result%20Structure%20%28by%20ref%29)))

(event OnComponentBeginOverlap(Box)
  (params (OverlappedComponent :type Primitive%20Component%20Object%20Reference) (OtherActor :type Actor%20Object%20Reference) (OtherComp :type Primitive%20Component%20Object%20Reference) (OtherBodyIndex :type Integer) (bFromSweep :type Boolean) (SweepResult :type Hit%20Result%20Structure%20%28by%20ref%29)))

(event Custom|Switch_On_Fire
  (bind _time_to_move_object (Timeline|Timeline_5 PlayFromStart)
    (:Update
      (Rendering|Components|Light|SetIntensity (Variables|Default|GetPointLight) (Math|Float|Lerp 0.0 1e+03 _time_to_move_object)))
    (:Finished
      (Development|PrintString "Hello")
      (Variables|Default|SetNewVar_1 (Math|Random|RandomIntegerinRange 0 2) :!label _label)
      (Development|PrintString (Utilities|String|ToString(Float) 0.0))
      (if (== (Variables|Default|GetNewVar_1) 0)
        (bind _time_to_move_object_2 (Timeline|Timeline_6 PlayFromStart)
          (:Update
            (Rendering|Components|Light|SetIntensity (Variables|Default|GetPointLight) (Math|Float|Lerp (Variables|/Script/Engine.LightComponentBase|GetIntensity (Variables|Default|GetPointLight)) 6e+02 _time_to_move_object_2)))
          (:Finished
            (Utilities|FlowControl|Delay 0.2 :!label _label_2)
            (Development|PrintString "NANDE")
            (goto _label)))
        (elif (== (Variables|Default|GetNewVar_1) 1)
          (bind _time_to_move_object_3 (Timeline|Timeline_7 PlayFromStart)
            (:Update
              (Rendering|Components|Light|SetIntensity (Variables|Default|GetPointLight) (Math|Float|Lerp (Variables|/Script/Engine.LightComponentBase|GetIntensity (Variables|Default|GetPointLight)) 1e+03 _time_to_move_object_3)))
            (:Finished
              (goto _label_2)))
          (elif (== (Variables|Default|GetNewVar_1) 2)
            (bind _time_to_move_object_4 (Timeline|Timeline_8 PlayFromStart)
              (:Update
                (Rendering|Components|Light|SetIntensity (Variables|Default|GetPointLight) (Math|Float|Lerp (Variables|/Script/Engine.LightComponentBase|GetIntensity (Variables|Default|GetPointLight)) 1e+03 _time_to_move_object_4)))
              (:Finished
                (goto _label_2)))))))))

(event EventBeginPlay
  (|CallParentFunction) ; This node is disabled and will not be called.\nDrag off pins to build functionality.
)

(event Collision|EventActorBeginOverlap
  (params (OtherActor :type Actor%20Object%20Reference))
  (|CallParentFunction OtherActor) ; This node is disabled and will not be called.\nDrag off pins to build functionality.
)

(event EventTick
  (params (DeltaSeconds :type Float%20%28single-precision%29))
  (|CallParentFunction DeltaSeconds) ; This node is disabled and will not be called.\nDrag off pins to build functionality.
)

(event EventSuccess
  (bind _actor_moving (Variables|Default|GetActor_Moving))
  (bind _first_log (Variables|Default|GetFirst_Log))
  (bind _first_log_2 (Variables|Default|GetFirst_Log))
  (bind _second_log (Variables|Default|GetSecond_Log))
  (bind _third_log (Variables|Default|GetThird_Log))
  (bind _childactor (Variables|/Script/Engine.ChildActorComponent|GetChildActor _first_log))
  (bind _returnvalue (Utilities|IsValid _childactor))
  (Collision|SetCollisionProfileName (Variables|Default|GetBox1) "BlockAll" true :!class /Script/Engine.PrimitiveComponent)
  (Utilities|FlowControl|Delay 0.5)
  (if (Actor|ActorHasTag (Variables|Default|GetActor_Moving) "Log")
    (Development|PrintString (Utilities|String|ToString(Boolean) _returnvalue))
    (if (not _returnvalue)
      (Development|PrintString "1ST")
      (ChildActorComponent|SetChildActorClass _first_log_2 (Utilities|GetClass (Variables|Default|GetActor_Moving)))
      (Collision|SetActorEnableCollision (Variables|/Script/Engine.ChildActorComponent|GetChildActor _first_log_2) false)
      (Variables|Default|SetLocation_Of_Actor_To_Spawn (Transformation|GetActorLocation (Variables|Default|GetActor_Moving)))
      (Actor|DestroyActor (Variables|Default|GetActor_Moving))
      (bind _time_to_move_object (Timeline|Timeline_2 PlayFromStart)
        (:Update
          (Transformation|SetActorLocationAndRotation (Variables|/Script/Engine.ChildActorComponent|GetChildActor (Variables|Default|GetFirst_Log)) (Math|Vector|Lerp(Vector) (Variables|Default|GetLocation_Of_Actor_To_Spawn) (Transformation|GetWorldLocation (Variables|Default|GetFirst_Log_Place)) _time_to_move_object) (Math|Rotator|Lerp(Rotator) (Transformation|GetActorRotation (Variables|/Script/Engine.ChildActorComponent|GetChildActor (Variables|Default|GetFirst_Log))) (Transformation|GetWorldRotation (Variables|Default|GetFirst_Log_Place)) _time_to_move_object))))
      (elif (not (Utilities|IsValid (Variables|/Script/Engine.ChildActorComponent|GetChildActor (Variables|Default|GetSecond_Log))))
        (ChildActorComponent|SetChildActorClass _second_log (Utilities|GetClass (Variables|Default|GetActor_Moving)))
        (Collision|SetActorEnableCollision (Variables|/Script/Engine.ChildActorComponent|GetChildActor _second_log) false)
        (Variables|Default|SetLocation_Of_Actor_To_Spawn (Transformation|GetActorLocation (Variables|Default|GetActor_Moving)))
        (Actor|DestroyActor (Variables|Default|GetActor_Moving))
        (bind _time_to_move_object_2 (Timeline|Timeline_1 PlayFromStart)
          (:Update
            (Transformation|SetActorLocationAndRotation (Variables|/Script/Engine.ChildActorComponent|GetChildActor (Variables|Default|GetSecond_Log)) (Math|Vector|Lerp(Vector) (Variables|Default|GetLocation_Of_Actor_To_Spawn) (Transformation|GetWorldLocation (Variables|Default|GetSecond_Log_Place)) _time_to_move_object_2) (Math|Rotator|Lerp(Rotator) (Transformation|GetActorRotation (Variables|/Script/Engine.ChildActorComponent|GetChildActor (Variables|Default|GetSecond_Log))) (Transformation|GetWorldRotation (Variables|Default|GetSecond_Log_Place)) _time_to_move_object_2))))
        (elif (not (Utilities|IsValid (Variables|/Script/Engine.ChildActorComponent|GetChildActor (Variables|Default|GetThird_Log))))
          (ChildActorComponent|SetChildActorClass _third_log (Utilities|GetClass (Variables|Default|GetActor_Moving)))
          (Collision|SetActorEnableCollision (Variables|/Script/Engine.ChildActorComponent|GetChildActor _third_log) false)
          (Variables|Default|SetLocation_Of_Actor_To_Spawn (Transformation|GetActorLocation (Variables|Default|GetActor_Moving)))
          (Actor|DestroyActor (Variables|Default|GetActor_Moving))
          (bind _time_to_move_object_3 (Timeline|Timeline_3 PlayFromStart)
            (:Update
              (Transformation|SetActorLocationAndRotation (Variables|/Script/Engine.ChildActorComponent|GetChildActor (Variables|Default|GetThird_Log)) (Math|Vector|Lerp(Vector) (Variables|Default|GetLocation_Of_Actor_To_Spawn) (Transformation|GetWorldLocation (Variables|Default|GetThird_Log_Place)) _time_to_move_object_3) (Math|Rotator|Lerp(Rotator) (Transformation|GetActorRotation (Variables|/Script/Engine.ChildActorComponent|GetChildActor (Variables|Default|GetThird_Log))) (Transformation|GetWorldRotation (Variables|Default|GetThird_Log_Place)) _time_to_move_object_3)))
            (:Finished
              (Variables|Default|SetCan_Set_Fire_? true))))))
    (elif (Actor|ActorHasTag (Variables|Default|GetActor_Moving) "Mystery_Box")
      (ChildActorComponent|SetChildActorClass (Variables|Default|GetBox_To_Burn) (Utilities|GetClass (Variables|Default|GetActor_Moving)))
      (Variables|Default|SetLocation_Of_Actor_To_Spawn (Transformation|GetActorLocation _actor_moving))
      (Actor|DestroyActor _actor_moving)
      (bind _time_to_move_object_4 (Timeline|Timeline_4 PlayFromStart)
        (:Update
          (Transformation|SetActorLocationAndRotation (Variables|/Script/Engine.ChildActorComponent|GetChildActor (Variables|Default|GetBox_To_Burn)) (Math|Vector|Lerp(Vector) (Variables|Default|GetLocation_Of_Actor_To_Spawn) (Transformation|GetWorldLocation (Variables|Default|GetBox_To_Burn_Places)) _time_to_move_object_4) (Math|Rotator|Lerp(Rotator) (Transformation|GetActorRotation (Variables|/Script/Engine.ChildActorComponent|GetChildActor (Variables|Default|GetBox_To_Burn))) (Transformation|GetWorldRotation (Variables|Default|GetBox_To_Burn_Places)) _time_to_move_object_4)))
        (:Finished
          (Variables|Default|SetCan_Set_Fire_? true)))
      (elif (Actor|ActorHasTag (Variables|Default|GetActor_Moving) "Mystery_Box")
        _))))

(event EventSpecial
  (params (Hit_Actor :type Actor%20Object%20Reference))
  (bind _asbp_match_child_inventory (Utilities|Casting|CastToBP_Match_Child_Inventory (Variables|/Script/Engine.ChildActorComponent|GetChildActor (Variables|/Game/GD/ThirdPerson/Blueprints/BP_Diplome_First_Person_Project.BP_Diplome_First_Person_Project_C|GetItem_Hold (Variables|Default|GetFirst_Person)))))
  (Default|SetFiretoMatch _asbp_match_child_inventory Hit_Actor))

(fn ConstructionScript
  (|CallParentFunction))