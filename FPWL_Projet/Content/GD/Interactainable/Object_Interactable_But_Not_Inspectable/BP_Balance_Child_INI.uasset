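; Interactive balance-scale puzzle where weights tip the scale and leveling it reveals a reward.
; Success moves ActorMoving into the first empty of four child-actor slots by timeline lerp, then applies its Poids to arrow and support rotation.
; BalanceDeMort hands slot weights back to FirstPerson, negating Poids except for the fourth slot.
; A near-zero arrow roll spawns the Reward child actor and slides HiddenReward.
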(event Custom|Balance_Movement
  (params (Poids :type Float%20%28double-precision%29))
  (bind _returnvalue (* Poids 1e+01))
  (bind _arrow (Variables|Default|GetArrow))
  (bind _right_support (Variables|Default|GetRight_Support))
  (bind _relativerotation (Variables|/Script/Engine.SceneComponent|GetRelativeRotation _arrow))
  (bind _relativerotation_2 (Variables|/Script/Engine.SceneComponent|GetRelativeRotation _right_support))
  (Development|PrintString (Utilities|String|ToString(Float) Poids))
  (Transformation|SetRelativeRotation _arrow (Math|Rotator|MakeRotator (+ (.roll _relativerotation) _returnvalue) (.pitch _relativerotation) (.yaw _relativerotation)) false false)
  (Transformation|SetRelativeRotation (Variables|Default|GetLeft_Support) (Math|Rotator|MakeRotator (.roll _relativerotation_2) (- (.pitch _relativerotation_2) _returnvalue) (.yaw _relativerotation_2)) false false)
  (CallFunction|BalancePerfected?))

(event Custom|Balance_Perfected_?
  (bind _arrow (Variables|Default|GetArrow))
  (bind _hidden_reward (Variables|Default|GetHidden_Reward))
  (bind _returnvalue (Transformation|GetWorldRotation _arrow))
  (bind _relativelocation (Variables|/Script/Engine.SceneComponent|GetRelativeLocation _hidden_reward))
  (Development|PrintString (Utilities|String|ToString(Float) (.roll _returnvalue)))
  (if (and (< (.roll _returnvalue) 1.0) (> (.roll _returnvalue) -1.0))
    (ChildActorComponent|SetChildActorClass (Variables|Default|GetReward) (Variables|Default|GetActor_To_Get))
    (bind _time_to_move_object (Timeline|Timeline_5 PlayFromStart)
      (:Update
        (Transformation|SetRelativeLocation (Variables|Default|GetHidden_Reward) (Math|Vector|Lerp(Vector) _relativelocation (+ _relativelocation "0,3.000000,0") _time_to_move_object) false false)))))

(event EventBeginPlay
  (|CallParentFunction) ; This node is disabled and will not be called.\nDrag off pins to build functionality.
)

(event Collision|EventActorBeginOverlap
  (params (OtherActor :type Actor%20Object%20Reference))
  (|CallParentFunction OtherActor) ; This node is disabled and will not be called.\nDrag off pins to build functionality.
)

(event EventTick
  (params (DeltaSeconds :type Float%20%28single-precision%29)))

(event EventSuccess
  (bind _first_poids (Variables|Default|GetFirst_Poids))
  (bind _childactor (Variables|/Script/Engine.ChildActorComponent|GetChildActor _first_poids))
  (bind _returnvalue (Utilities|IsValid _childactor))
  (Development|PrintString (Utilities|String|ToString(Boolean) _returnvalue))
  (if (not _returnvalue)
    (Development|PrintString "1ST")
    (ChildActorComponent|SetChildActorClass (Variables|Default|GetFirst_Poids) (Utilities|GetClass (Variables|Default|GetActor_Moving)))
    (Variables|Default|SetLocation_Of_Actor_To_Spawn (Transformation|GetActorLocation (Variables|Default|GetActor_Moving)))
    (Actor|DestroyActor (Variables|Default|GetActor_Moving))
    (bind _time_to_move_object (Timeline|Timeline_1 PlayFromStart)
      (:Update
        (Transformation|SetActorLocation (Variables|/Script/Engine.ChildActorComponent|GetChildActor (Variables|Default|GetFirst_Poids)) (Math|Vector|Lerp(Vector) (Variables|Default|GetLocation_Of_Actor_To_Spawn) (Transformation|GetWorldLocation (Variables|Default|GetPlace_For_First_Poids)) _time_to_move_object) false false))
      (:Finished
        (bind _asbp_poids_child_inventory (Utilities|Casting|CastToBp_Poids_Child_Inventory (Variables|/Script/Engine.ChildActorComponent|GetChildActor (Variables|Default|GetFirst_Poids))))
        (CallFunction|BalanceMovement (Variables|/Game/GD/Interactainable/Inventory/Bp_Poids_Child_Inventory.Bp_Poids_Child_Inventory_C|GetPoids _asbp_poids_child_inventory))))
    (elif (not (Utilities|IsValid (Variables|/Script/Engine.ChildActorComponent|GetChildActor (Variables|Default|GetSecond_Poids))))
      (Development|PrintString "2ND")
      (ChildActorComponent|SetChildActorClass (Variables|Default|GetSecond_Poids) (Utilities|GetClass (Variables|Default|GetActor_Moving)))
      (Variables|Default|SetLocation_Of_Actor_To_Spawn (Transformation|GetActorLocation (Variables|Default|GetActor_Moving)))
      (Actor|DestroyActor (Variables|Default|GetActor_Moving))
      (bind _time_to_move_object_2 (Timeline|Timeline_2 PlayFromStart)
        (:Update
          (Transformation|SetActorLocation (Variables|/Script/Engine.ChildActorComponent|GetChildActor (Variables|Default|GetSecond_Poids)) (Math|Vector|Lerp(Vector) (Variables|Default|GetLocation_Of_Actor_To_Spawn) (Transformation|GetWorldLocation (Variables|Default|GetPlace_For_Second_Poids)) _time_to_move_object_2) false false))
        (:Finished
          (bind _asbp_poids_child_inventory_2 (Utilities|Casting|CastToBp_Poids_Child_Inventory (Variables|/Script/Engine.ChildActorComponent|GetChildActor (Variables|Default|GetSecond_Poids))))
          (CallFunction|BalanceMovement (Variables|/Game/GD/Interactainable/Inventory/Bp_Poids_Child_Inventory.Bp_Poids_Child_Inventory_C|GetPoids _asbp_poids_child_inventory_2))))
      (elif (not (Utilities|IsValid (Variables|/Script/Engine.ChildActorComponent|GetChildActor (Variables|Default|GetThird_Poids))))
        (Development|PrintString "2ND")
        (ChildActorComponent|SetChildActorClass (Variables|Default|GetThird_Poids) (Utilities|GetClass (Variables|Default|GetActor_Moving)))
        (Variables|Default|SetLocation_Of_Actor_To_Spawn (Transformation|GetActorLocation (Variables|Default|GetActor_Moving)))
        (Actor|DestroyActor (Variables|Default|GetActor_Moving))
        (bind _time_to_move_object_3 (Timeline|Timeline_3 PlayFromStart)
          (:Update
            (Transformation|SetActorLocation (Variables|/Script/Engine.ChildActorComponent|GetChildActor (Variables|Default|GetThird_Poids)) (Math|Vector|Lerp(Vector) (Variables|Default|GetLocation_Of_Actor_To_Spawn) (Transformation|GetWorldLocation (Variables|Default|GetPlace_For_Third_Poids)) _time_to_move_object_3) false false))
          (:Finished
            (bind _asbp_poids_child_inventory_3 (Utilities|Casting|CastToBp_Poids_Child_Inventory (Variables|/Script/Engine.ChildActorComponent|GetChildActor (Variables|Default|GetThird_Poids))))
            (CallFunction|BalanceMovement (Variables|/Game/GD/Interactainable/Inventory/Bp_Poids_Child_Inventory.Bp_Poids_Child_Inventory_C|GetPoids _asbp_poids_child_inventory_3))))
        (elif (not (Utilities|IsValid (Variables|/Script/Engine.ChildActorComponent|GetChildActor (Variables|Default|GetFourth_Poids))))
          (Development|PrintString "2ND")
          (ChildActorComponent|SetChildActorClass (Variables|Default|GetFourth_Poids) (Utilities|GetClass (Variables|Default|GetActor_Moving)))
          (Variables|Default|SetLocation_Of_Actor_To_Spawn (Transformation|GetActorLocation (Variables|Default|GetActor_Moving)))
          (Actor|DestroyActor (Variables|Default|GetActor_Moving))
          (bind _time_to_move_object_4 (Timeline|Timeline_4 PlayFromStart)
            (:Update
              (Transformation|SetActorLocation (Variables|/Script/Engine.ChildActorComponent|GetChildActor (Variables|Default|GetFourth_Poids)) (Math|Vector|Lerp(Vector) (Variables|Default|GetLocation_Of_Actor_To_Spawn) (Transformation|GetWorldLocation (Variables|Default|GetPlace_For_Fourth_Poids)) _time_to_move_object_4) false false))
            (:Finished
              (bind _asbp_poids_child_inventory_4 (Utilities|Casting|CastToBp_Poids_Child_Inventory (Variables|/Script/Engine.ChildActorComponent|GetChildActor (Variables|Default|GetFourth_Poids))))
              (CallFunction|BalanceMovement (Variables|/Game/GD/Interactainable/Inventory/Bp_Poids_Child_Inventory.Bp_Poids_Child_Inventory_C|GetPoids _asbp_poids_child_inventory_4)))))))))

(event EventBalanceDeMort
  (params (Hit_Component :type Primitive%20Component%20Object%20Reference))
  (bind _fourth_poids (Variables|Default|GetFourth_Poids))
  (bind _first_poids (Variables|Default|GetFirst_Poids))
  (bind _second_poids (Variables|Default|GetSecond_Poids))
  (bind _third_poids (Variables|Default|GetThird_Poids))
  (if (== Hit_Component (Variables|Default|GetPlace_For_First_Poids))
    (bind _returnvalue (Game|SpawnActorfromClass (Utilities|GetClass (Variables|/Script/Engine.ChildActorComponent|GetChildActor _first_poids)) (Math|Transform|MakeTransform (Transformation|GetWorldLocation _first_poids) "0, 0, 0" "1.000000,1.000000,1.000000") "Undefined" 0 0))
    (ChildActorComponent|SetChildActorClass _first_poids 0)
    (Development|PrintString (Utilities|GetDisplayName _returnvalue))
    (Default|GetActorfromBalance (Variables|Default|GetFirst_Person) _returnvalue)
    (bind _asbp_poids_child_inventory (Utilities|Casting|CastToBp_Poids_Child_Inventory _returnvalue))
    (CallFunction|BalanceMovement (- (Variables|/Game/GD/Interactainable/Inventory/Bp_Poids_Child_Inventory.Bp_Poids_Child_Inventory_C|GetPoids _asbp_poids_child_inventory) (* (Variables|/Game/GD/Interactainable/Inventory/Bp_Poids_Child_Inventory.Bp_Poids_Child_Inventory_C|GetPoids _asbp_poids_child_inventory) 2.0)))
    (elif (== Hit_Component (Variables|Default|GetPlace_For_Second_Poids))
      (bind _returnvalue_2 (Game|SpawnActorfromClass (Utilities|GetClass (Variables|/Script/Engine.ChildActorComponent|GetChildActor _second_poids)) (Math|Transform|MakeTransform (Transformation|GetWorldLocation _second_poids) "0, 0, 0" "1.000000,1.000000,1.000000") "Undefined" 0 0))
      (ChildActorComponent|SetChildActorClass _second_poids 0)
      (Development|PrintString (Utilities|GetDisplayName _returnvalue_2))
      (Default|GetActorfromBalance (Variables|Default|GetFirst_Person) _returnvalue_2)
      (bind _asbp_poids_child_inventory_2 (Utilities|Casting|CastToBp_Poids_Child_Inventory _returnvalue_2))
      (CallFunction|BalanceMovement (- (Variables|/Game/GD/Interactainable/Inventory/Bp_Poids_Child_Inventory.Bp_Poids_Child_Inventory_C|GetPoids _asbp_poids_child_inventory_2) (* (Variables|/Game/GD/Interactainable/Inventory/Bp_Poids_Child_Inventory.Bp_Poids_Child_Inventory_C|GetPoids _asbp_poids_child_inventory_2) 2.0)))
      (elif (== Hit_Component (Variables|Default|GetPlace_For_Fourth_Poids))
        (bind _returnvalue_3 (Game|SpawnActorfromClass (Utilities|GetClass (Variables|/Script/Engine.ChildActorComponent|GetChildActor _fourth_poids)) (Math|Transform|MakeTransform (Transformation|GetWorldLocation _fourth_poids) "0, 0, 0" "1.000000,1.000000,1.000000") "Undefined" 0 0))
        (ChildActorComponent|SetChildActorClass _fourth_poids 0)
        (Development|PrintString (Utilities|GetDisplayName _returnvalue_3))
        (Default|GetActorfromBalance (Variables|Default|GetFirst_Person) _returnvalue_3)
        (bind _asbp_poids_child_inventory_3 (Utilities|Casting|CastToBp_Poids_Child_Inventory _returnvalue_3))
        (CallFunction|BalanceMovement (Variables|/Game/GD/Interactainable/Inventory/Bp_Poids_Child_Inventory.Bp_Poids_Child_Inventory_C|GetPoids _asbp_poids_child_inventory_3))
        (elif (== 0 (Variables|Default|GetPlace_For_Third_Poids))
          (bind _returnvalue_4 (Game|SpawnActorfromClass (Utilities|GetClass (Variables|/Script/Engine.ChildActorComponent|GetChildActor _third_poids)) (Math|Transform|MakeTransform (Transformation|GetWorldLocation _third_poids) "0, 0, 0" "1.000000,1.000000,1.000000") "Undefined" 0 0))
          (ChildActorComponent|SetChildActorClass _third_poids 0)
          (Development|PrintString (Utilities|GetDisplayName _returnvalue_4))
          (Default|GetActorfromBalance (Variables|Default|GetFirst_Person) _returnvalue_4)
          (bind _asbp_poids_child_inventory_4 (Utilities|Casting|CastToBp_Poids_Child_Inventory _returnvalue_4))
          (CallFunction|BalanceMovement (- (Variables|/Game/GD/Interactainable/Inventory/Bp_Poids_Child_Inventory.Bp_Poids_Child_Inventory_C|GetPoids _asbp_poids_child_inventory_4) (* (Variables|/Game/GD/Interactainable/Inventory/Bp_Poids_Child_Inventory.Bp_Poids_Child_Inventory_C|GetPoids _asbp_poids_child_inventory_4) 2.0))))))))

(event Input|KeyboardEvents|M
  (params (Key :type Key%20Structure :default "None")))

(fn ConstructionScript
  (|CallParentFunction))