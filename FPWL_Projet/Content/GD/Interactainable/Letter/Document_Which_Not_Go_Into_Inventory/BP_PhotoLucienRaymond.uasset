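; BP_PhotoLucienRaymond is an interactable photo prop, filed with documents that do not go into the inventory; this graph only handles its highlight.
; OnHighlight shows an outline mesh, creating it on first use as a copy of the static mesh with an outline material at the same relative transform.
; StopHighlight hides the cached outline so later highlights can reuse it.
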(event EventBeginPlay
  (|CallParentFunction) ; This node is disabled and will not be called.\nDrag off pins to build functionality.
)

(event Collision|EventActorBeginOverlap
  (params (OtherActor :type Actor%20Object%20Reference))
  (|CallParentFunction OtherActor) ; This node is disabled and will not be called.\nDrag off pins to build functionality.
)

(event EventStopHighlight
  (Utilities|IsValid (Variables|Default|GetOutline_Mesh)
    (:Is%20Valid
      (Rendering|SetVisibility (Variables|Default|GetOutline_Mesh) false false))))

(event EventTick
  (params (DeltaSeconds :type Float%20%28single-precision%29))
  (|CallParentFunction DeltaSeconds) ; This node is disabled and will not be called.\nDrag off pins to build functionality.
)

(event EventOnHighlight
  (bind _staticmesh (Variables|Default|GetStaticMesh))
  (Utilities|IsValid (Variables|Default|GetOutline_Mesh)
    (:Is%20Valid
      (Rendering|SetVisibility (Variables|Default|GetOutline_Mesh) true false))
    (:Is%20Not%20Valid
      (bind _returnvalue (AddComponent|AddStaticMeshComponent false (Math|Transform|MakeTransform (Variables|/Script/Engine.SceneComponent|GetRelativeLocation _staticmesh) (Variables|/Script/Engine.SceneComponent|GetRelativeRotation _staticmesh) (Variables|/Script/Engine.SceneComponent|GetRelativeScale3D _staticmesh))))
      (bind _output_get (Variables|Default|SetOutline_Mesh _returnvalue))
      (Components|StaticMesh|SetStaticMesh _output_get (Variables|/Script/Engine.StaticMeshComponent|GetStaticMesh _staticmesh))
      (Rendering|Material|SetMaterial (Variables|Default|GetOutline_Mesh) 0 "/Game/GD/M_Test_Outline.M_Test_Outline"))))

(fn ConstructionScript
  (|CallParentFunction))