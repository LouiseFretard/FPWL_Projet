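; Clock puzzle (Horloge Enigme) interactable, filed among letter documents that do not go into the inventory.
; On BeginPlay it puts a dynamic material instance on its mesh, whose "Activate" parameter drives the highlight.
; Highlight events toggle that parameter while IsActivate is true, and Tick forces it off otherwise.
; StopCollision and StartCollision switch several components between NoCollision and BlockAll, also setting CanBeUsed and the highlight.
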(event Custom|StopCollision
  (Variables|Default|SetCan_Be_Used_? false)
  (Collision|SetCollisionProfileName (Variables|Default|GetStaticMesh1) "NoCollision" true :!class /Script/Engine.PrimitiveComponent)
  (Rendering|Material|SetScalarParameterValue (Variables|Default|GetM_inst) "Activate" 0.0 :!class /Script/Engine.MaterialInstanceDynamic))

(event Custom|StartCollision
  (Variables|Default|SetCan_Be_Used_? true)
  (Collision|SetCollisionProfileName (Variables|Default|GetStaticMesh1) "BlockAll" true :!class /Script/Engine.PrimitiveComponent)
  (Rendering|Material|SetScalarParameterValue (Variables|Default|GetM_inst) "Activate" 1.0 :!class /Script/Engine.MaterialInstanceDynamic))

(event EventBeginPlay
  (bind _returnvalue (Rendering|Material|CreateDynamicMaterialInstance "/Game/TA/Materials/Gameplay/Maison/HorlogeMulti.HorlogeMulti" "None" "None" :!class /Script/Engine.KismetMaterialLibrary))
  (bind _output_get (Variables|Default|SetM_inst _returnvalue))
  (Rendering|Material|SetMaterial (Variables|Default|GetStaticMesh) 0 _output_get)
  (Rendering|Material|SetScalarParameterValue (Variables|Default|GetM_inst) "Activate" 0.0 :!class /Script/Engine.MaterialInstanceDynamic)
  (Variables|Default|SetCan_Be_Used_? true)
  (Variables|Default|SetisActivate true))

(event Collision|EventActorBeginOverlap
  (params (OtherActor :type Actor%20Object%20Reference))
  (|CallParentFunction OtherActor) ; This node is disabled and will not be called.\nDrag off pins to build functionality.
)

(event EventStopHighlight
  (if (Variables|Default|GetisActivate)
    (Rendering|Material|SetScalarParameterValue (Variables|Default|GetM_inst) "Activate" 0.0 :!class /Script/Engine.MaterialInstanceDynamic)))

(event EventOnHighlight
  (if (Variables|Default|GetisActivate)
    (Rendering|Material|SetScalarParameterValue (Variables|Default|GetM_inst) "Activate" 1.0 :!class /Script/Engine.MaterialInstanceDynamic)))

(event EventTick
  (params (DeltaSeconds :type Float%20%28single-precision%29))
  (if (not (Variables|Default|GetisActivate))
    (Rendering|Material|SetScalarParameterValue (Variables|Default|GetM_inst) "Activate" 0.0 :!class /Script/Engine.MaterialInstanceDynamic)))

(fn ConstructionScript
  (|CallParentFunction))