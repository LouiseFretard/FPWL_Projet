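; Base parent Blueprint for interactable documents that the first-person player inspects and rotates.
; Start_Inspect stores the player and moves input from the character to the document, letting mouse axes rotate its Arrow component.
; Space asks the player to show text; C ends inspection or returns to the document journal.
; Rotation and exit require zero HUD blur; proximity clue and letter-switching logic is disconnected.
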(event OnComponentBeginOverlap(Collision_To_Show_Clue)
  (params (OverlappedComponent :type Primitive%20Component%20Object%20Reference) (OtherActor :type Actor%20Object%20Reference) (OtherComp :type Primitive%20Component%20Object%20Reference) (OtherBodyIndex :type Integer) (bFromSweep :type Boolean) (SweepResult :type Hit%20Result%20Structure%20%28by%20ref%29)))

(event OnComponentEndOverlap(Collision_To_Show_Clue)
  (params (OverlappedComponent :type Primitive%20Component%20Object%20Reference) (OtherActor :type Actor%20Object%20Reference) (OtherComp :type Primitive%20Component%20Object%20Reference) (OtherBodyIndex :type Integer)))

(event Custom|Start_Inspect
  (params (Inspector :type Pawn%20Object%20Reference) (Enigmes_Accomplie_? :type Boolean))
  (bind _returnvalue (Game|GetPlayerController 0))
  (bind _asbp_diplome_first_person_project (Utilities|Casting|CastToBP_Diplome_First_Person_Project Inspector))
  (Variables|Default|SetFirst_Person _asbp_diplome_first_person_project)
  (Input|DisableInput Inspector _returnvalue)
  (Input|EnableInput _returnvalue))

(event EventBeginPlay)

(event Collision|EventActorBeginOverlap
  (params (OtherActor :type Actor%20Object%20Reference)))

(event EventTick
  (params (DeltaSeconds :type Float%20%28single-precision%29)))

(event Input|MouseEvents|MouseX
  (params (AxisValue :type Float%20%28single-precision%29))
  (if (== (Variables|/Script/UMG.BackgroundBlur|GetBlurStrength (Variables|/Game/GD/Widget/HUD.HUD_C|GetBackgroundBlur_0 (Variables|/Game/GD/ThirdPerson/Blueprints/BP_Diplome_First_Person_Project.BP_Diplome_First_Person_Project_C|GetHUD (Variables|Default|GetFirst_Person)))) 0.0)
    (Transformation|SetRelativeRotation (Variables|Default|GetArrow) (Math|Rotator|CombineRotators (Variables|/Script/Engine.SceneComponent|GetRelativeRotation (Variables|Default|GetArrow)) (Math|Rotator|MakeRotator 0.0 0.0 (* AxisValue -1.0))) false false)))

(event Input|MouseEvents|MouseY
  (params (AxisValue :type Float%20%28single-precision%29))
  (if (== (Variables|/Script/UMG.BackgroundBlur|GetBlurStrength (Variables|/Game/GD/Widget/HUD.HUD_C|GetBackgroundBlur_0 (Variables|/Game/GD/ThirdPerson/Blueprints/BP_Diplome_First_Person_Project.BP_Diplome_First_Person_Project_C|GetHUD (Variables|Default|GetFirst_Person)))) 0.0)
    (Transformation|SetRelativeRotation (Variables|Default|GetArrow) (Math|Rotator|CombineRotators (Variables|/Script/Engine.SceneComponent|GetRelativeRotation (Variables|Default|GetArrow)) (Math|Rotator|MakeRotator 0.0 (* AxisValue -1.0) 0.0)) false false)))

(event Input|KeyboardEvents|SpaceBar
  (params (Key :type Key%20Structure :default "None"))
  (:Pressed
    (Default|TexttoPrintforPlayer (Variables|Default|GetFirst_Person))))

(event Input|KeyboardEvents|C
  (params (Key :type Key%20Structure :default "None"))
  (bind _first_person (Variables|Default|GetFirst_Person))
  (:Pressed
    (if (== (Variables|/Script/UMG.BackgroundBlur|GetBlurStrength (Variables|/Game/GD/Widget/HUD.HUD_C|GetBackgroundBlur_0 (Variables|/Game/GD/ThirdPerson/Blueprints/BP_Diplome_First_Person_Project.BP_Diplome_First_Person_Project_C|GetHUD (Variables|Default|GetFirst_Person)))) 0.0)
      (Input|DisableInput (Game|GetPlayerController 0))
      (Default|HideHowtoGetOutOfInspection (Variables|/Game/GD/ThirdPerson/Blueprints/BP_Diplome_First_Person_Project.BP_Diplome_First_Person_Project_C|GetHUD (Variables|Default|GetFirst_Person)))
      (if (not (Variables|/Game/GD/ThirdPerson/Blueprints/BP_Diplome_First_Person_Project.BP_Diplome_First_Person_Project_C|GetDoc's_Journal_Open_? _first_person))
        (Default|Inspect _first_person false)
        (else
          (Default|ReturntoDocJournal _first_person))))))

(event Input|MouseEvents|MouseWheelDown
  (params (Key :type Key%20Structure :default "None")))

(event Input|MouseEvents|MouseWheelUp
  (params (Key :type Key%20Structure :default "None")))

(fn ConstructionScript)