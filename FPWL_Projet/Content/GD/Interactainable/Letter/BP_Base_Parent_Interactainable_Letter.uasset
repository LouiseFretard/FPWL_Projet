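; Base actor for inspectable letters that the first-person character can examine.
; Start_Inspect moves input from the inspector to the letter, letting mouse movement rotate its Arrow component.
; Space toggles the character's ShowText flag, which blocks rotation and exit while set.
; Tab or right-click releases input and either ends inspection or returns to the document journal; the wheel calls ChangeLetter when the letter inventory is open.
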(event Custom|Start_Inspect
  (params (Inspector :type Pawn%20Object%20Reference) (Enigmes_Accomplie_? :type Boolean))
  (bind _returnvalue (Game|GetPlayerController 0))
  (bind _asbp_diplome_first_person_project (Utilities|Casting|CastToBP_Diplome_First_Person_Project Inspector))
  (Variables|Default|SetFirst_Person _asbp_diplome_first_person_project)
  (Input|DisableInput Inspector _returnvalue)
  (Input|EnableInput _returnvalue))

(event EventBeginPlay)

(event Collision|EventActorBeginOverlap
  (params (OtherActor :type Actor%20Object%20Reference)))

(event EventTick
  (params (DeltaSeconds :type Float%20%28single-precision%29)))

(event Input|MouseEvents|MouseX
  (params (AxisValue :type Float%20%28single-precision%29))
  (if (not (Variables|/Game/GD/ThirdPerson/Blueprints/BP_Diplome_First_Person_Project.BP_Diplome_First_Person_Project_C|GetShow_Text_? (Variables|Default|GetFirst_Person)))
    (Transformation|SetRelativeRotation (Variables|Default|GetArrow) (Math|Rotator|CombineRotators (Variables|/Script/Engine.SceneComponent|GetRelativeRotation (Variables|Default|GetArrow)) (Math|Rotator|MakeRotator 0.0 0.0 (* AxisValue -1.0))) false false)))

(event Input|MouseEvents|MouseY
  (params (AxisValue :type Float%20%28single-precision%29))
  (if (not (Variables|/Game/GD/ThirdPerson/Blueprints/BP_Diplome_First_Person_Project.BP_Diplome_First_Person_Project_C|GetShow_Text_? (Variables|Default|GetFirst_Person)))
    (Transformation|SetRelativeRotation (Variables|Default|GetArrow) (Math|Rotator|CombineRotators (Variables|/Script/Engine.SceneComponent|GetRelativeRotation (Variables|Default|GetArrow)) (Math|Rotator|MakeRotator 0.0 (* AxisValue -1.0) 0.0)) false false)))

(event Input|MouseEvents|RightMouseButton
  (params (Key :type Key%20Structure :default "None"))
  (bind _first_person (Variables|Default|GetFirst_Person))
  (:Pressed
    (if (not (Variables|/Game/GD/ThirdPerson/Blueprints/BP_Diplome_First_Person_Project.BP_Diplome_First_Person_Project_C|GetShow_Text_? (Variables|Default|GetFirst_Person)))
      (Input|DisableInput (Game|GetPlayerController 0))
      (if (not (Variables|/Game/GD/ThirdPerson/Blueprints/BP_Diplome_First_Person_Project.BP_Diplome_First_Person_Project_C|GetDoc's_Journal_Open_? _first_person))
        (Default|Inspect _first_person false)
        (else
          (Default|ReturntoDocJournal _first_person))))))

(event Input|KeyboardEvents|SpaceBar
  (params (Key :type Key%20Structure :default "None"))
  (bind _first_person (Variables|Default|GetFirst_Person))
  (:Pressed
    (Utilities|FlowControl|FlipFlop
      (:A
        (Variables|/Game/GD/ThirdPerson/Blueprints/BP_Diplome_First_Person_Project.BP_Diplome_First_Person_Project_C|SetShow_Text_? _first_person true))
      (:B
        (Variables|/Game/GD/ThirdPerson/Blueprints/BP_Diplome_First_Person_Project.BP_Diplome_First_Person_Project_C|SetShow_Text_? _first_person false)))))

(event Input|KeyboardEvents|Tab
  (params (Key :type Key%20Structure :default "None"))
  (bind _first_person (Variables|Default|GetFirst_Person))
  (:Pressed
    (if (not (Variables|/Game/GD/ThirdPerson/Blueprints/BP_Diplome_First_Person_Project.BP_Diplome_First_Person_Project_C|GetShow_Text_? (Variables|Default|GetFirst_Person)))
      (Input|DisableInput (Game|GetPlayerController 0))
      (if (not (Variables|/Game/GD/ThirdPerson/Blueprints/BP_Diplome_First_Person_Project.BP_Diplome_First_Person_Project_C|GetDoc's_Journal_Open_? _first_person))
        (Default|Inspect _first_person false)
        (else
          (Default|ReturntoDocJournal _first_person))))))

(event Input|MouseEvents|MouseWheelDown
  (params (Key :type Key%20Structure :default "None"))
  (:Pressed
    (bind _asbp_diplome_first_person_project (Utilities|Casting|CastToBP_Diplome_First_Person_Project (stale Custom|Start_Inspect Inspector)))
    (if (== (Variables|/Game/GD/ThirdPerson/Blueprints/BP_Diplome_First_Person_Project.BP_Diplome_First_Person_Project_C|GetLetter_Inventory_Open_? _asbp_diplome_first_person_project) true)
      (if (== (stale Input|MouseEvents|MouseWheelUp Key) "MouseScrollUp")
        (Default|ChangeLetter _asbp_diplome_first_person_project (stale Input|MouseEvents|MouseWheelUp Key))
        (else
          (Default|ChangeLetter _asbp_diplome_first_person_project Key))))))

(event Input|MouseEvents|MouseWheelUp
  (params (Key :type Key%20Structure :default "None"))
  (:Pressed
    (bind _asbp_diplome_first_person_project (Utilities|Casting|CastToBP_Diplome_First_Person_Project (stale Custom|Start_Inspect Inspector)))
    (if (== (Variables|/Game/GD/ThirdPerson/Blueprints/BP_Diplome_First_Person_Project.BP_Diplome_First_Person_Project_C|GetLetter_Inventory_Open_? _asbp_diplome_first_person_project) true)
      (if (== Key "MouseScrollUp")
        (Default|ChangeLetter _asbp_diplome_first_person_project Key)
        (else
          (Default|ChangeLetter _asbp_diplome_first_person_project (stale Input|MouseEvents|MouseWheelDown Key)))))))

(fn ConstructionScript)