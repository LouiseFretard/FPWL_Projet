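; Electric meter puzzle actor in which five levers must light five bulbs.
; Success swings both cover sides open on a timeline; hitting the Box then freezes player movement and narrows FOV until right-click restores both.
; Each lever toggles signed offsets on several bulb counters, and bulbs light when their counter is positive.
; All five lit prints a win message and disables lever collision; older intensity-based lever logic remains unconnected.
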(event Custom|State_Of_Bulb
  (bind _bulb_2 (Variables|Default|GetBulb_2))
  (bind _bulb_3 (Variables|Default|GetBulb_3))
  (bind _bulb_4 (Variables|Default|GetBulb_4))
  (bind _bulb_5 (Variables|Default|GetBulb_5))
  (if (> (Variables|Default|GetBulb_1_Value) 0)
    (Rendering|Components|Light|SetIntensity (Variables|Default|GetBulb_1) 5e+01)
    (else
      (Rendering|Components|Light|SetIntensity (Variables|Default|GetBulb_1) 0.0)))
  (if (> (Variables|Default|GetBulb_2_Value) 0)
    (Rendering|Components|Light|SetIntensity _bulb_2 5e+01)
    (else
      (Rendering|Components|Light|SetIntensity _bulb_2 0.0)))
  (if (> (Variables|Default|GetBulb_3_Value) 0)
    (Rendering|Components|Light|SetIntensity _bulb_3 5e+01)
    (else
      (Rendering|Components|Light|SetIntensity _bulb_3 0.0)))
  (if (> (Variables|Default|GetBulb_4_Value) 0)
    (Rendering|Components|Light|SetIntensity _bulb_4 5e+01)
    (else
      (Rendering|Components|Light|SetIntensity _bulb_4 0.0)))
  (if (> (Variables|Default|GetBulb_5_Value) 0)
    (Rendering|Components|Light|SetIntensity _bulb_5 5e+01)
    (CallFunction|Finished)
    (else
      (Rendering|Components|Light|SetIntensity _bulb_5 0.0))))

(event Custom|Finished
  (if (Math|Boolean|ANDBoolean (> (Variables|Default|GetBulb_1_Value) 0) (> (Variables|Default|GetBulb_2_Value) 0) (> (Variables|Default|GetBulb_3_Value) 0) (> (Variables|Default|GetBulb_4_Value) 0) (> (Variables|Default|GetBulb_5_Value) 0))
    (Development|PrintString "GG wp")
    (Collision|SetCollisionEnabled (Variables|Default|GetLever_3) "NoCollision")))

(event Custom|Level_1_Implication
  (if (not (Variables|Default|GetLever_1_Switch_On_?))
    (Variables|Default|SetLever_1_Switch_On_? true)
    (Variables|Default|SetBulb_1_Value (+ (Variables|Default|GetBulb_1_Value) 1))
    (Variables|Default|SetBulb_3_Value (+ (Variables|Default|GetBulb_3_Value) 1))
    (Variables|Default|SetBulb_4_Value (+ (Variables|Default|GetBulb_4_Value) 1))
    (else
      (Variables|Default|SetLever_1_Switch_On_? false)
      (Variables|Default|SetBulb_1_Value (+ (Variables|Default|GetBulb_1_Value) -1))
      (Variables|Default|SetBulb_3_Value (+ (Variables|Default|GetBulb_3_Value) -1))
      (Variables|Default|SetBulb_4_Value (+ (Variables|Default|GetBulb_4_Value) -1))))
  (CallFunction|StateOfBulb))

(event Custom|Level_2_Implication
  (if (not (Variables|Default|GetLever_2_Switch_On_?))
    (Variables|Default|SetLever_2_Switch_On_? true)
    (Variables|Default|SetBulb_1_Value (+ (Variables|Default|GetBulb_1_Value) -1))
    (Variables|Default|SetBulb_2_Value (+ (Variables|Default|GetBulb_2_Value) 1))
    (Variables|Default|SetBulb_4_Value (+ (Variables|Default|GetBulb_4_Value) 1))
    (else
      (Variables|Default|SetLever_2_Switch_On_? false)
      (Variables|Default|SetBulb_1_Value (+ (Variables|Default|GetBulb_1_Value) 1))
      (Variables|Default|SetBulb_2_Value (+ (Variables|Default|GetBulb_2_Value) -1))
      (Variables|Default|SetBulb_4_Value (+ (Variables|Default|GetBulb_4_Value) -1))))
  (CallFunction|StateOfBulb))

(event Custom|Level_5_Implication
  (if (not (Variables|Default|GetLever_5_Switch_On_?))
    (Variables|Default|SetLever_5_Switch_On_? true)
    (Variables|Default|SetBulb_1_Value (+ (Variables|Default|GetBulb_1_Value) 1))
    (Variables|Default|SetBulb_5_Value (+ (Variables|Default|GetBulb_5_Value) 1))
    (else
      (Variables|Default|SetLever_5_Switch_On_? false)
      (Variables|Default|SetBulb_1_Value (+ (Variables|Default|GetBulb_1_Value) -1))
      (Variables|Default|SetBulb_5_Value (+ (Variables|Default|GetBulb_5_Value) -1))))
  (CallFunction|StateOfBulb))

(event Custom|Level_3_Implication
  (if (not (Variables|Default|GetLever_3_Switch_On_?))
    (Variables|Default|SetLever_3_Switch_On_? true)
    (Variables|Default|SetBulb_2_Value (+ (Variables|Default|GetBulb_2_Value) -1))
    (Variables|Default|SetBulb_4_Value (+ (Variables|Default|GetBulb_4_Value) -1))
    (Variables|Default|SetBulb_5_Value (+ (Variables|Default|GetBulb_5_Value) 1))
    (else
      (Variables|Default|SetLever_3_Switch_On_? false)
      (Variables|Default|SetBulb_2_Value (+ (Variables|Default|GetBulb_2_Value) 1))
      (Variables|Default|SetBulb_4_Value (+ (Variables|Default|GetBulb_4_Value) 1))
      (Variables|Default|SetBulb_5_Value (+ (Variables|Default|GetBulb_5_Value) -1))))
  (CallFunction|StateOfBulb))

(event Custom|Level_4_Implication
  (if (not (Variables|Default|GetLever_4_Switch_On_?))
    (Variables|Default|SetLever_4_Switch_On_? true)
    (Variables|Default|SetBulb_2_Value (+ (Variables|Default|GetBulb_2_Value) 1))
    (Variables|Default|SetBulb_3_Value (+ (Variables|Default|GetBulb_3_Value) -1))
    (Variables|Default|SetBulb_4_Value (+ (Variables|Default|GetBulb_4_Value) 1))
    (Variables|Default|SetBulb_5_Value (+ (Variables|Default|GetBulb_5_Value) 1))
    (else
      (Variables|Default|SetLever_4_Switch_On_? false)
      (Variables|Default|SetBulb_2_Value (+ (Variables|Default|GetBulb_2_Value) -1))
      (Variables|Default|SetBulb_3_Value (+ (Variables|Default|GetBulb_3_Value) 1))
      (Variables|Default|SetBulb_4_Value (+ (Variables|Default|GetBulb_4_Value) -1))
      (Variables|Default|SetBulb_5_Value (+ (Variables|Default|GetBulb_5_Value) -1))))
  (CallFunction|StateOfBulb))

(event EventBeginPlay
  (|CallParentFunction) ; This node is disabled and will not be called.\nDrag off pins to build functionality.
)

(event Collision|EventActorBeginOverlap
  (params (OtherActor :type Actor%20Object%20Reference))
  (|CallParentFunction OtherActor) ; This node is disabled and will not be called.\nDrag off pins to build functionality.
)

(event EventTick
  (params (DeltaSeconds :type Float%20%28single-precision%29))
  (|CallParentFunction DeltaSeconds) ; This node is disabled and will not be called.\nDrag off pins to build functionality.
)

(event EventSuccess
  (Collision|SetCollisionEnabled (Variables|Default|GetRighy_Side_To_Be_Open) "NoCollision")
  (Transformation|SetActorLocation (Variables|Default|GetActor_Moving) "0, 0, 0" false false)
  (Variables|Default|SetLeft_Side_Original_Relative_Rotation (Variables|/Script/Engine.SceneComponent|GetRelativeRotation (Variables|Default|GetOpen_Left_Side_Arrow)))
  (Variables|Default|SetRight_Side_Original_Relative_Rotation (Variables|/Script/Engine.SceneComponent|GetRelativeRotation (Variables|Default|GetOpen_Right_Side_Arrow)))
  (bind _time_to_move_object (Timeline|Timeline_1 PlayFromStart)
    (:Update
      (Transformation|SetRelativeRotation (Variables|Default|GetOpen_Left_Side_Arrow) (Math|Rotator|Lerp(Rotator) (Variables|Default|GetLeft_Side_Original_Relative_Rotation) (Math|Rotator|MakeRotator (.roll (Variables|Default|GetLeft_Side_Original_Relative_Rotation)) (.pitch (Variables|Default|GetLeft_Side_Original_Relative_Rotation)) (+ (.yaw (Variables|Default|GetLeft_Side_Original_Relative_Rotation)) 1.5e+02)) _time_to_move_object) false false)
      (Transformation|SetRelativeRotation (Variables|Default|GetOpen_Right_Side_Arrow) (Math|Rotator|Lerp(Rotator) (Variables|Default|GetRight_Side_Original_Relative_Rotation) (Math|Rotator|MakeRotator (.roll (Variables|Default|GetRight_Side_Original_Relative_Rotation)) (.pitch (Variables|Default|GetRight_Side_Original_Relative_Rotation)) (+ (.yaw (Variables|Default|GetRight_Side_Original_Relative_Rotation)) -1.5e+02)) _time_to_move_object) false false))
    (:Finished
      (Variables|Default|SetOpened_? true))))

(event EventHitComponent
  (params (Hit_Component :type Primitive%20Component%20Object%20Reference))
  (bind _first_person (Variables|Default|GetFirst_Person))
  (if (Variables|Default|GetOpened_?)
    (if (== Hit_Component (Variables|Default|GetBox))
      (Pawn|Components|CharacterMovement|DisableMovement (Variables|/Script/Engine.Character|GetCharacterMovement _first_person))
      (Camera|SetFieldOfView (Variables|/Game/GD/ThirdPerson/Blueprints/BP_Diplome_First_Person_Project.BP_Diplome_First_Person_Project_C|GetFirst_Person_Camera _first_person) 8e+01)
      (Collision|SetCollisionProfileName (Variables|Default|GetBox) "NoCollision" true :!class /Script/Engine.PrimitiveComponent)
      (elif (== Hit_Component (Variables|Default|GetLever_1))
        (CallFunction|Level1Implication)
        (elif (== Hit_Component (Variables|Default|GetLever_2))
          (CallFunction|Level2Implication)
          (elif (== Hit_Component (Variables|Default|GetLever_3))
            (CallFunction|Level3Implication)
            (elif (== Hit_Component (Variables|Default|GetLever_4))
              (CallFunction|Level4Implication)
              (elif (== Hit_Component (Variables|Default|GetLever_5))
                (CallFunction|Level5Implication)))))))))

(event Input|MouseEvents|RightMouseButton
  (params (Key :type Key%20Structure :default "None"))
  (bind _first_person (Variables|Default|GetFirst_Person))
  (bind _charactermovement (Variables|/Script/Engine.Character|GetCharacterMovement _first_person))
  (:Pressed
    (if (not (Pawn|Components|CharacterMovement|IsWalking _charactermovement))
      (Pawn|Components|CharacterMovement|SetMovementMode _charactermovement "MOVE_Walking" 0)
      (Collision|SetCollisionProfileName (Variables|Default|GetBox) "BlockAll" true :!class /Script/Engine.PrimitiveComponent)
      (Camera|SetFieldOfView (Variables|/Game/GD/ThirdPerson/Blueprints/BP_Diplome_First_Person_Project.BP_Diplome_First_Person_Project_C|GetFirst_Person_Camera _first_person) 9e+01))))

(fn ConstructionScript
  (|CallParentFunction))