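; BP_New_Base_Collision_For_Dialogue is an interactable actor Blueprint that plays dialogue when its ActionWithoutObject event fires.
; The event passes DialogueOtherPossibilities to the first-person character's TransmissDialogue at order 5.
; After a four-second delay, it ends that dialogue through the character's HUD.
; BeginPlay, overlap and Tick are disabled stubs, and the construction script only calls its parent.
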(event EventBeginPlay
  (|CallParentFunction) ; This node is disabled and will not be called.\nDrag off pins to build functionality.
)

(event Collision|EventActorBeginOverlap
  (params (OtherActor :type Actor%20Object%20Reference))
  (|CallParentFunction OtherActor) ; This node is disabled and will not be called.\nDrag off pins to build functionality.
)

(event EventTick
  (params (DeltaSeconds :type Float%20%28single-precision%29))
  (|CallParentFunction DeltaSeconds) ; This node is disabled and will not be called.\nDrag off pins to build functionality.
)

(event EventActionWithoutObject
  (bind _first_person (Variables|Default|GetFirst_Person))
  (Default|TransmissDialogue _first_person (Variables|Default|GetDialogue_Other_Possibilities) 5)
  (Utilities|FlowControl|Delay 4.0)
  (Default|EndDialogue (Variables|/Game/GD/ThirdPerson/Blueprints/BP_Diplome_First_Person_Project.BP_Diplome_First_Person_Project_C|GetHUD _first_person) 5))

(fn ConstructionScript
  (|CallParentFunction))