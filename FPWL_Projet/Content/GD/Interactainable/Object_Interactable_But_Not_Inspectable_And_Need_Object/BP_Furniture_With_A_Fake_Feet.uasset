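; Interactable furniture puzzle where the player swaps a held missing-foot item for the reward at its front-left foot.
; BeginPlay hides that foot and spawns the reward without collision when usable.
; BalanceDeMort validates the hit and held item, clears the inventory slot, then chains three timeline lerps to insert the item and move foot and reward out.
; Success enables reward collision and plays dialogue; failure wobbles the Arrow component with problem dialogue.
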(event EventBeginPlay
  (bind _reward (Variables|Default|GetReward))
  (|CallParentFunction)
  (if (and (== (Variables|Default|GetCan_Be_Used_?) true) (== (Utilities|IsValidClass (Variables|Default|GetActor_To_Get)) true))
    (Development|SetHiddeninGame (Variables|Default|GetFront_Left_Foot) true false)
    (ChildActorComponent|SetChildActorClass _reward (Variables|Default|GetActor_To_Get))
    (Collision|SetActorEnableCollision (Variables|/Script/Engine.ChildActorComponent|GetChildActor _reward) false)
    (else
      (Development|SetHiddeninGame (Variables|Default|GetFront_Left_Foot) false false))))

(event Collision|EventActorBeginOverlap
  (params (OtherActor :type Actor%20Object%20Reference))
  (|CallParentFunction OtherActor) ; This node is disabled and will not be called.\nDrag off pins to build functionality.
)

(event EventBalanceDeMort
  (params (Hit_Component :type Primitive%20Component%20Object%20Reference))
  (bind _first_person (Variables|Default|GetFirst_Person))
  (bind _arrow (Variables|Default|GetArrow))
  (bind _arrow_2 (Variables|Default|GetArrow))
  (bind _first_person_2 (Variables|Default|GetFirst_Person))
  (bind _items_inventory (Variables|/Game/GD/ThirdPerson/Blueprints/BP_Diplome_First_Person_Project.BP_Diplome_First_Person_Project_C|GetItems_Inventory _first_person))
  (bind _relativerotation (Variables|/Script/Engine.SceneComponent|GetRelativeRotation _arrow))
  (bind _relativerotation_2 (Variables|/Script/Engine.SceneComponent|GetRelativeRotation _arrow_2))
  (if (and (== Hit_Component (Variables|Default|GetFront_Left_Foot)) (== (Utilities|GetClass (Variables|/Script/Engine.ChildActorComponent|GetChildActor (Variables|/Game/GD/ThirdPerson/Blueprints/BP_Diplome_First_Person_Project.BP_Diplome_First_Person_Project_C|GetItem_Hold (Variables|Default|GetFirst_Person)))) "/Game/GD/Interactainable/Inventory/BP_Missing_Foot_Child_Inventory.BP_Missing_Foot_Child_Inventory_C"))
    (ChildActorComponent|SetChildActorClass (Variables|Default|GetStock_Actor) (Variables|/Script/Engine.ChildActorComponent|GetChildActorClass (Variables|/Game/GD/ThirdPerson/Blueprints/BP_Diplome_First_Person_Project.BP_Diplome_First_Person_Project_C|GetItem_Hold _first_person)))
    (Collision|SetActorEnableCollision (Variables|/Script/Engine.ChildActorComponent|GetChildActor (Variables|Default|GetStock_Actor)) false)
    (Utilities|Array|SetArrayElem (Variables|/Game/GD/ThirdPerson/Items_Inventory.Items_Inventory_C|GetAll_Items _items_inventory) (Variables|/Game/GD/ThirdPerson/Items_Inventory.Items_Inventory_C|GetIndex_For_Player _items_inventory) 0)
    (Default|ReorganiseInventory _first_person_2)
    (Default|SelectedItem (Variables|/Game/GD/ThirdPerson/Blueprints/BP_Diplome_First_Person_Project.BP_Diplome_First_Person_Project_C|GetHUD _first_person_2) _first_person_2)
    (Default|ChangeItemHoldinHand _first_person_2)
    (Transformation|SetWorldLocation (Variables|Default|GetStock_Actor) (Transformation|GetWorldLocation (Variables|/Game/GD/ThirdPerson/Blueprints/BP_Diplome_First_Person_Project.BP_Diplome_First_Person_Project_C|GetItem_Hold _first_person_2)) false false)
    (bind _time_to_move_object (Timeline|Timeline_1 PlayFromStart)
      (:Update
        (Transformation|SetWorldLocation (Variables|Default|GetStock_Actor) (Math|Vector|Lerp(Vector) (Transformation|GetWorldLocation (Variables|Default|GetStock_Actor)) (Transformation|GetWorldLocation (Variables|Default|GetLocate_Actor_Moving)) _time_to_move_object) false false))
      (:Finished
        (bind _time_to_move_object_2 (Timeline|Timeline_2 PlayFromStart)
          (:Update
            (Transformation|SetWorldLocation (Variables|Default|GetStock_Actor) (Math|Vector|Lerp(Vector) (Transformation|GetWorldLocation (Variables|Default|GetStock_Actor)) (Transformation|GetWorldLocation (Variables|Default|GetFront_Left_Foot)) _time_to_move_object_2) false false))
          (:Finished
            (bind _time_to_move_object_3 (Timeline|Timeline_3 PlayFromStart)
              (:Update
                (Transformation|SetWorldLocation (Variables|Default|GetFront_Left_Foot) (Math|Vector|Lerp(Vector) (Transformation|GetWorldLocation (Variables|Default|GetFront_Left_Foot)) (Transformation|GetWorldLocation (Variables|Default|GetNew_Place_For_Poids)) _time_to_move_object_3) false false))
              (:Finished
                (Variables|Default|SetCan_Poids_Be_Taken_? true)
                (Default|TransmissDialogue (Variables|Default|GetFirst_Person) (Variables|Default|GetDialogue_When_Finished))
                (Collision|SetActorEnableCollision (Variables|/Script/Engine.ChildActorComponent|GetChildActor (Variables|Default|GetReward)) true)))))))
    (else
      (Transformation|SetRelativeRotation _arrow (Math|Rotator|MakeRotator (+ (.roll _relativerotation) 2.0) (.pitch _relativerotation) (.yaw _relativerotation)) false false)
      (Utilities|FlowControl|Delay 0.2)
      (Transformation|SetRelativeRotation _arrow_2 (Math|Rotator|MakeRotator (+ (.roll _relativerotation_2) -4.0) (.pitch _relativerotation_2) (.yaw _relativerotation_2)) false false)
      (Utilities|FlowControl|Delay 0.2)
      (Transformation|SetRelativeRotation (Variables|Default|GetArrow) (Math|Rotator|MakeRotator 0.0 0.0 0.0) false false)
      (Default|TransmissDialogue (Variables|Default|GetFirst_Person) (Variables|Default|GetDialogue_When_Problem)))))

(event EventTick
  (params (DeltaSeconds :type Float%20%28single-precision%29))
  (bind _box (Variables|Default|GetBox))
  (if (Utilities|Operators|NotEqual(!=) :A (Variables|/Script/Engine.SceneComponent|GetRelativeRotation _box))
    (Transformation|SetRelativeRotation _box "0, 0, 0" false false)))

(fn ConstructionScript
  (|CallParentFunction))