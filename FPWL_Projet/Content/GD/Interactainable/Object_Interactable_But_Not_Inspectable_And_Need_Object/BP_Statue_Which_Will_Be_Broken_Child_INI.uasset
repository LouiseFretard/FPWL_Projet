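; Interactable statue puzzle object that, once enabled by Start_Statue, works a single time without an object and sets up a partition document as its child-actor reward.
; The tag on the player's second letter-inventory entry picks the partition variant, which Box1 overlaps reapply after use.
; A timeline slides the Arrow component and partway through unlocks the library interactable.
; Dynamic materials on statue and pedestal drive highlighting.
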(event OnComponentBeginOverlap(Box1)
  (params (OverlappedComponent :type Primitive%20Component%20Object%20Reference) (OtherActor :type Actor%20Object%20Reference) (OtherComp :type Primitive%20Component%20Object%20Reference) (OtherBodyIndex :type Integer) (bFromSweep :type Boolean) (SweepResult :type Hit%20Result%20Structure%20%28by%20ref%29))
  (bind _stock_actor1 (Variables|Default|GetStock_Actor1))
  (Utilities|Casting|CastToBP_Diplome_First_Person_Project OtherActor)
  (if (Variables|Default|GetAnimation_Of_Object_Used_?)
    (if (Actor|ActorHasTag (Utilities|Array|Get(acopy) (Variables|/Game/GD/ThirdPerson/Letter_Inventory.Letter_Inventory_C|GetAll_Letters (Variables|/Game/GD/ThirdPerson/Blueprints/BP_Diplome_First_Person_Project.BP_Diplome_First_Person_Project_C|GetLetter_Inventory (Variables|Default|GetFirst_Person))) 1) "P_1")
      (ChildActorComponent|SetChildActorClass _stock_actor1 "/Game/GD/Interactainable/Letter/BP_Partition_1-2_Part_Child_Document.BP_Partition_1-2_Part_Child_Document_C")
      (bind _asbp_partition_1_2_part_child_document (Utilities|Casting|CastToBP_Partition_1-2_Part_Child_Document (Variables|/Script/Engine.ChildActorComponent|GetChildActor (Variables|Default|GetStock_Actor1))))
      (Rendering|Material|SetMaterial (Variables|/Game/GD/Interactainable/Letter/BP_Base_Parent_Interactainable_Documents.BP_Base_Parent_Interactainable_Documents_C|GetStaticMesh _asbp_partition_1_2_part_child_document) 0 "/Game/TA/Materials/DocumentsINGAME/Partitions/M_Partition2.M_Partition2")
      (elif (Actor|ActorHasTag (Utilities|Array|Get(acopy) (Variables|/Game/GD/ThirdPerson/Letter_Inventory.Letter_Inventory_C|GetAll_Letters (Variables|/Game/GD/ThirdPerson/Blueprints/BP_Diplome_First_Person_Project.BP_Diplome_First_Person_Project_C|GetLetter_Inventory (Variables|Default|GetFirst_Person))) 1) "P_1_3")
        (ChildActorComponent|SetChildActorClass _stock_actor1 "/Game/GD/Interactainable/Letter/BP_Partition_1-2-3_Child_Document.BP_Partition_1-2-3_Child_Document_C")
        (bind _asbp_partition_1_2_3_child_document (Utilities|Casting|CastToBP_Partition_1-2-3_Child_Document (Variables|/Script/Engine.ChildActorComponent|GetChildActor (Variables|Default|GetStock_Actor1))))
        (Rendering|Material|SetMaterial (Variables|/Game/GD/Interactainable/Letter/BP_Base_Parent_Interactainable_Documents.BP_Base_Parent_Interactainable_Documents_C|GetStaticMesh _asbp_partition_1_2_3_child_document) 0 "/Game/TA/Materials/DocumentsINGAME/Partitions/M_Partition2.M_Partition2")))))

(event Custom|Start_Statue
  (Variables|Default|SetCan_Be_Used_? true))

(event EventBeginPlay
  (|CallParentFunction)
  (bind _returnvalue (Rendering|Material|CreateDynamicMaterialInstance "/Game/TA/Materials/Gameplay/Appartement/Statue.Statue" "None" "None" :!class /Script/Engine.KismetMaterialLibrary))
  (bind _output_get (Variables|Default|SetM_inst _returnvalue))
  (Rendering|Material|SetMaterial (Variables|Default|GetStaticMesh) 0 _output_get)
  (Rendering|Material|SetScalarParameterValue (Variables|Default|GetM_inst) "Activate" 0.0 :!class /Script/Engine.MaterialInstanceDynamic)
  (bind _returnvalue_2 (Rendering|Material|CreateDynamicMaterialInstance "/Game/TA/Materials/Gameplay/Appartement/Pied_Statue.Pied_Statue" "None" "None" :!class /Script/Engine.KismetMaterialLibrary))
  (bind _output_get_2 (Variables|Default|SetM_inst2 _returnvalue_2))
  (Rendering|Material|SetMaterial (Variables|Default|GetStaticMesh10) 0 _output_get_2)
  (Rendering|Material|SetScalarParameterValue (Variables|Default|GetM_inst2) "Activate" 0.0 :!class /Script/Engine.MaterialInstanceDynamic))

(event Collision|EventActorBeginOverlap
  (params (OtherActor :type Actor%20Object%20Reference))
  (|CallParentFunction OtherActor) ; This node is disabled and will not be called.\nDrag off pins to build functionality.
)

(event EventTick
  (params (DeltaSeconds :type Float%20%28single-precision%29))
  (|CallParentFunction DeltaSeconds) ; This node is disabled and will not be called.\nDrag off pins to build functionality.
)

(event EventSuccess)

(event EventActionWithoutObject
  (bind _stock_actor1 (Variables|Default|GetStock_Actor1))
  (if (Variables|Default|GetCan_Be_Used_?)
    (Variables|Default|SetCan_Be_Used_? false)
    (Collision|SetCollisionEnabled (Variables|Default|GetBox) "NoCollision")
    (Utilities|FlowControl|DoOnce false
      (:Completed
        (Variables|Default|SetArrow_Original_Relative_Location (Variables|/Script/Engine.SceneComponent|GetRelativeLocation (Variables|Default|GetArrow)))
        (if (Actor|ActorHasTag (Utilities|Array|Get(acopy) (Variables|/Game/GD/ThirdPerson/Letter_Inventory.Letter_Inventory_C|GetAll_Letters (Variables|/Game/GD/ThirdPerson/Blueprints/BP_Diplome_First_Person_Project.BP_Diplome_First_Person_Project_C|GetLetter_Inventory (Variables|Default|GetFirst_Person))) 1) "P_1")
          (ChildActorComponent|SetChildActorClass _stock_actor1 "/Game/GD/Interactainable/Letter/BP_Partition_1-2_Part_Child_Document.BP_Partition_1-2_Part_Child_Document_C")
          (bind _asbp_partition_1_2_part_child_document (Utilities|Casting|CastToBP_Partition_1-2_Part_Child_Document (Variables|/Script/Engine.ChildActorComponent|GetChildActor _stock_actor1)))
          (Rendering|Material|SetMaterial (Variables|/Game/GD/Interactainable/Letter/BP_Base_Parent_Interactainable_Documents.BP_Base_Parent_Interactainable_Documents_C|GetStaticMesh _asbp_partition_1_2_part_child_document) 0 "/Game/TA/Materials/DocumentsINGAME/Partitions/M_Partition2.M_Partition2")
          (Variables|Default|SetReward_Original_Relative_Location (Variables|/Script/Engine.SceneComponent|GetRelativeLocation (Variables|Default|GetStock_Actor1)) :!label _label)
          (bind _item_track (Timeline|Timeline_1 PlayFromStart)
            (:Update
              (Transformation|SetRelativeLocation (Variables|Default|GetArrow) (Math|Vector|Lerp(Vector) (Variables|Default|GetArrow_Original_Relative_Location) (Math|Vector|MakeVector 5e+01 (.Y (Math|Vector|BreakVector (Variables|Default|GetArrow_Original_Relative_Location))) (.Z (Math|Vector|BreakVector (Variables|Default|GetArrow_Original_Relative_Location)))) _item_track) false false)
              (if (> _item_track 0.25)
                (Utilities|FlowControl|DoOnce false
                  (:Completed
                    (Variables|Default|SetAnimation_Of_Object_Used_? true)
                    (bind _returnvalue (Actor|GetActorOfClass "/Game/GD/Interactainable/Object_Interact_Not_Inspectable_Not_Need_Object/BP_Library_Child_ININNO.BP_Library_Child_ININNO_C"))
                    (Collision|SetCollisionProfileName (Variables|/Game/GD/Interactainable/Object_Interact_Not_Inspectable_Not_Need_Object/BP_Library_Child_ININNO.BP_Library_Child_ININNO_C|GetBox _returnvalue) "BlockAll" true :!class /Script/Engine.PrimitiveComponent)
                    (Variables|/Game/GD/Interactainable/Object_Interact_Not_Inspectable_Not_Need_Object/BP_Base_Interact_Not_Inspectable_Not_Need_Object.BP_Base_Interact_Not_Inspectable_Not_Need_Object_C|SetCan_Be_Used_? _returnvalue true))))))
          (elif (Actor|ActorHasTag (Utilities|Array|Get(acopy) (Variables|/Game/GD/ThirdPerson/Letter_Inventory.Letter_Inventory_C|GetAll_Letters (Variables|/Game/GD/ThirdPerson/Blueprints/BP_Diplome_First_Person_Project.BP_Diplome_First_Person_Project_C|GetLetter_Inventory (Variables|Default|GetFirst_Person))) 1) "P_1_3")
            (ChildActorComponent|SetChildActorClass _stock_actor1 "/Game/GD/Interactainable/Letter/BP_Partition_1-2-3_Child_Document.BP_Partition_1-2-3_Child_Document_C")
            (bind _asbp_partition_1_2_3_child_document (Utilities|Casting|CastToBP_Partition_1-2-3_Child_Document (Variables|/Script/Engine.ChildActorComponent|GetChildActor (Variables|Default|GetStock_Actor1))))
            (Rendering|Material|SetMaterial (Variables|/Game/GD/Interactainable/Letter/BP_Base_Parent_Interactainable_Documents.BP_Base_Parent_Interactainable_Documents_C|GetStaticMesh _asbp_partition_1_2_3_child_document) 0 "/Game/TA/Materials/DocumentsINGAME/Partitions/M_Partition2.M_Partition2")
            (goto _label)))))))

(event EventOnHighlight
  (Rendering|Material|SetScalarParameterValue (Variables|Default|GetM_inst) "Activate" 1.0 :!class /Script/Engine.MaterialInstanceDynamic)
  (Rendering|Material|SetScalarParameterValue (Variables|Default|GetM_inst2) "Activate" 1.0 :!class /Script/Engine.MaterialInstanceDynamic))

(event EventStopHighlight
  (Rendering|Material|SetScalarParameterValue (Variables|Default|GetM_inst) "Activate" 0.0 :!class /Script/Engine.MaterialInstanceDynamic)
  (Rendering|Material|SetScalarParameterValue (Variables|Default|GetM_inst2) "Activate" 0.0 :!class /Script/Engine.MaterialInstanceDynamic))

(fn ConstructionScript
  (|CallParentFunction))