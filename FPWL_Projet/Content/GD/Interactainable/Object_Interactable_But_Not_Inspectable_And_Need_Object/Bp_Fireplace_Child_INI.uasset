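; Fireplace puzzle interactable where the player places a log, lights it with a held match and burns a mystery box to spawn a reward actor.
; Success identifies the placed item by tag, respawns it as a child actor and lerps it into position.
; Switch_On_Fire fades in the light, takes the match from the inventory, burns any placed box, then loops random timelines for flicker.
; The box burns whichever comes last, fire or box.
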(event OnComponentHit(Box)
  (params (HitComponent :type Primitive%20Component%20Object%20Reference) (OtherActor :type Actor%20Object%20Reference) (OtherComp :type Primitive%20Component%20Object%20Reference) (NormalImpulse :type Vector :default "0, 0, 0") (Hit :type Hit%20Result%20Structure%20%28by%20ref%29)))

(event OnComponentBeginOverlap(Box)
  (params (OverlappedComponent :type Primitive%20Component%20Object%20Reference) (OtherActor :type Actor%20Object%20Reference) (OtherComp :type Primitive%20Component%20Object%20Reference) (OtherBodyIndex :type Integer) (bFromSweep :type Boolean) (SweepResult :type Hit%20Result%20Structure%20%28by%20ref%29)))

(event Custom|Switch_On_Fire
  (bind _first_person (Variables|Default|GetFirst_Person))
  (bind _first_person_2 (Variables|Default|GetFirst_Person))
  (bind _item_hold (Variables|/Game/GD/ThirdPerson/Blueprints/BP_Diplome_First_Person_Project.BP_Diplome_First_Person_Project_C|GetItem_Hold _first_person))
  (bind _items_inventory (Variables|/Game/GD/ThirdPerson/Blueprints/BP_Diplome_First_Person_Project.BP_Diplome_First_Person_Project_C|GetItems_Inventory _first_person_2))
  (bind _childactor (Variables|/Script/Engine.ChildActorComponent|GetChildActor _item_hold))
  (bind _returnvalue (Transformation|GetActorLocation _childactor))
  (bind _time_to_move_object (Timeline|Timeline_5 PlayFromStart)
    (:Update
      (Rendering|Components|Light|SetIntensity (Variables|Default|GetPointLight) (Math|Float|Lerp 0.0 1e+03 _time_to_move_object)))
    (:Finished
      (Variables|Default|SetFire_Set_? true)
      (bind _outhit (Collision|CapsuleTraceByChannel _returnvalue (+ _returnvalue (+ (* (Math|Vector|GetForwardVector (Variables|/Script/Engine.Actor|GetRootComponent _childactor)) 2e+03) "0,0,-1000.000000")) 2e+01 2e+01 "TraceTypeQuery1" false (Utilities|Array|MakeArray _childactor) "ForDuration"))
      (bind _returnvalue_2 (Game|SpawnActorfromClass (Utilities|GetClass _childactor) (Math|Transform|MakeTransform "-343.000000,-65.000000,77.000000" "0, 0, 0" "1.000000,1.000000,1.000000") "Undefined" 0 0))
      (Collision|SetActorEnableCollision _returnvalue_2 false)
      (Utilities|Array|SetArrayElem (Variables|/Game/GD/ThirdPerson/Items_Inventory.Items_Inventory_C|GetAll_Items _items_inventory) (Variables|/Game/GD/ThirdPerson/Items_Inventory.Items_Inventory_C|GetIndex_For_Player _items_inventory) 0)
      (Default|ChangeItemHoldinHand _first_person_2)
      (if (Variables|Default|GetBox_Places_?)
        (CallFunction|DestroyBox))
      (Variables|Default|SetNewVar_1 (Math|Random|RandomIntegerinRange 0 2) :!label _label)
      (if (== (Variables|Default|GetNewVar_1) 0)
        (bind _time_to_move_object_2 (Timeline|Timeline_6 PlayFromStart)
          (:Update
            (Rendering|Components|Light|SetIntensity (Variables|Default|GetPointLight) (Math|Float|Lerp (Variables|/Script/Engine.LightComponentBase|GetIntensity (Variables|Default|GetPointLight)) 6e+02 _time_to_move_object_2)))
          (:Finished
            (Utilities|FlowControl|Delay 0.2 :!label _label_2)
            (goto _label)))
        (elif (== (Variables|Default|GetNewVar_1) 1)
          (bind _time_to_move_object_3 (Timeline|Timeline_7 PlayFromStart)
            (:Update
              (Rendering|Components|Light|SetIntensity (Variables|Default|GetPointLight) (Math|Float|Lerp (Variables|/Script/Engine.LightComponentBase|GetIntensity (Variables|Default|GetPointLight)) 1e+03 _time_to_move_object_3)))
            (:Finished
              (goto _label_2)))
          (elif (== (Variables|Default|GetNewVar_1) 2)
            (bind _time_to_move_object_4 (Timeline|Timeline_8 PlayFromStart)
              (:Update
                (Rendering|Components|Light|SetIntensity (Variables|Default|GetPointLight) (Math|Float|Lerp (Variables|/Script/Engine.LightComponentBase|GetIntensity (Variables|Default|GetPointLight)) 1e+03 _time_to_move_object_4)))
              (:Finished
                (goto _label_2)))))))))

(event Custom|Destroy_Box
  (ChildActorComponent|SetChildActorClass (Variables|Default|GetBox_To_Burn) 0)
  (Game|SpawnActorfromClass (Variables|Default|GetActor_To_Get) (Math|Transform|MakeTransform (Transformation|GetWorldLocation (Variables|Default|GetBox_To_Burn_Places)) "0, 0, 0" "1.000000,1.000000,1.000000") "Undefined" 0 0)
  (Utilities|FlowControl|Delay 0.2)
  (Collision|SetCollisionProfileName (Variables|Default|GetBox1) "NoCollision" true :!class /Script/Engine.PrimitiveComponent))

(event EventBeginPlay
  (|CallParentFunction) ; This node is disabled and will not be called.\nDrag off pins to build functionality.
)

(event Collision|EventActorBeginOverlap
  (params (OtherActor :type Actor%20Object%20Reference))
  (|CallParentFunction OtherActor) ; This node is disabled and will not be called.\nDrag off pins to build functionality.
)

(event EventTick
  (params (DeltaSeconds :type Float%20%28single-precision%29))
  (|CallParentFunction DeltaSeconds) ; This node is disabled and will not be called.\nDrag off pins to build functionality.
)

(event EventSuccess
  (bind _actor_moving (Variables|Default|GetActor_Moving))
  (bind _first_log (Variables|Default|GetFirst_Log))
  (Collision|SetCollisionProfileName (Variables|Default|GetBox1) "BlockAll" true :!class /Script/Engine.PrimitiveComponent)
  (Utilities|FlowControl|Delay 0.5)
  (if (Actor|ActorHasTag (Variables|Default|GetActor_Moving) "Log")
    (if (not (Utilities|IsValid (Variables|/Script/Engine.ChildActorComponent|GetChildActor (Variables|Default|GetFirst_Log))))
      (ChildActorComponent|SetChildActorClass _first_log (Utilities|GetClass (Variables|Default|GetActor_Moving)))
      (Collision|SetActorEnableCollision (Variables|/Script/Engine.ChildActorComponent|GetChildActor _first_log) false)
      (Variables|Default|SetLocation_Of_Actor_To_Spawn (Transformation|GetActorLocation (Variables|Default|GetActor_Moving)))
      (Actor|DestroyActor (Variables|Default|GetActor_Moving))
      (bind _time_to_move_object (Timeline|Timeline_2 PlayFromStart)
        (:Update
          (Transformation|SetActorLocationAndRotation (Variables|/Script/Engine.ChildActorComponent|GetChildActor (Variables|Default|GetFirst_Log)) (Math|Vector|Lerp(Vector) (Variables|Default|GetLocation_Of_Actor_To_Spawn) (Transformation|GetWorldLocation (Variables|Default|GetFirst_Log_Place)) _time_to_move_object) (Math|Rotator|Lerp(Rotator) (Transformation|GetActorRotation (Variables|/Script/Engine.ChildActorComponent|GetChildActor (Variables|Default|GetFirst_Log))) (Transformation|GetWorldRotation (Variables|Default|GetFirst_Log_Place)) _time_to_move_object)))
        (:Finished
          (Variables|Default|SetCan_Set_Fire_? true))))
    (elif (Actor|ActorHasTag (Variables|Default|GetActor_Moving) "Mystery_Box")
      (ChildActorComponent|SetChildActorClass (Variables|Default|GetBox_To_Burn) (Utilities|GetClass (Variables|Default|GetActor_Moving)))
      (Variables|Default|SetLocation_Of_Actor_To_Spawn (Transformation|GetActorLocation _actor_moving))
      (Actor|DestroyActor _actor_moving)
      (bind _time_to_move_object_2 (Timeline|Timeline_4 PlayFromStart)
        (:Update
          (Transformation|SetActorLocationAndRotation (Variables|/Script/Engine.ChildActorComponent|GetChildActor (Variables|Default|GetBox_To_Burn)) (Math|Vector|Lerp(Vector) (Variables|Default|GetLocation_Of_Actor_To_Spawn) (Transformation|GetWorldLocation (Variables|Default|GetBox_To_Burn_Places)) _time_to_move_object_2) (Math|Rotator|Lerp(Rotator) (Transformation|GetActorRotation (Variables|/Script/Engine.ChildActorComponent|GetChildActor (Variables|Default|GetBox_To_Burn))) (Transformation|GetWorldRotation (Variables|Default|GetBox_To_Burn_Places)) _time_to_move_object_2)))
        (:Finished
          (Variables|Default|SetBox_Places_? true)
          (if (Variables|Default|GetFire_Set_?)
            (CallFunction|DestroyBox)))))))

(event EventSpecial
  (params (Hit_Actor :type Actor%20Object%20Reference))
  (bind _first_person (Variables|Default|GetFirst_Person))
  (bind _item_hold (Variables|/Game/GD/ThirdPerson/Blueprints/BP_Diplome_First_Person_Project.BP_Diplome_First_Person_Project_C|GetItem_Hold _first_person))
  (bind _childactor (Variables|/Script/Engine.ChildActorComponent|GetChildActor _item_hold))
  (if (and (== (Utilities|GetClass _childactor) "/Game/GD/Interactainable/Inventory/BP_Match_Child_Inventory.BP_Match_Child_Inventory_C") (== (Variables|Default|GetCan_Set_Fire_?) true))
    (bind _asbp_match_child_inventory (Utilities|Casting|CastToBP_Match_Child_Inventory _childactor))
    (Default|SetFiretoMatch _asbp_match_child_inventory Hit_Actor)))

(fn ConstructionScript
  (|CallParentFunction))