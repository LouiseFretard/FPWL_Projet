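; Piano interactable that reacts when all music partitions (sheet music) are gathered.
; Interacting without an object asks FirstPerson to check whether all partitions are held.
; On All_Partition_Gathered, a DoOnce swaps three child actors to partition document classes and disables their collision.
; A timeline then lerps each onto its placement component's transform, and on finish sends a "Driiiiing" dialogue to the player.
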(event Custom|All_Partition_Gathered
  (bind _second_partition (Variables|Default|GetSecond_Partition))
  (bind _first_partition_place (Variables|Default|GetFirst_Partition_Place))
  (bind _second_partition_place (Variables|Default|GetSecond_Partition_Place))
  (bind _third_partition_place (Variables|Default|GetThird_Partition_Place))
  (bind _third_partition (Variables|Default|GetThird_Partition))
  (bind _first_partition (Variables|Default|GetFirst_Partition))
  (bind _returnvalue (Transformation|GetWorldTransform _third_partition_place))
  (bind _returnvalue_2 (Transformation|GetWorldTransform _first_partition_place))
  (bind _returnvalue_3 (Transformation|GetWorldTransform _second_partition_place))
  (bind _childactor (Variables|/Script/Engine.ChildActorComponent|GetChildActor _third_partition))
  (bind _childactor_2 (Variables|/Script/Engine.ChildActorComponent|GetChildActor _first_partition))
  (bind _childactor_3 (Variables|/Script/Engine.ChildActorComponent|GetChildActor _second_partition))
  (Utilities|FlowControl|DoOnce false
    (:Completed
      (ChildActorComponent|SetChildActorClass _first_partition "/Game/GD/Interactainable/Letter/BP_First_Partition_Lucien_Child_Documents.BP_First_Partition_Lucien_Child_Documents_C")
      (ChildActorComponent|SetChildActorClass _second_partition "/Game/GD/Interactainable/Letter/BP_Partition_1-2_Part_Child_Document.BP_Partition_1-2_Part_Child_Document_C")
      (ChildActorComponent|SetChildActorClass _third_partition "/Game/GD/Interactainable/Letter/BP_Partition_1-2-3_Child_Document.BP_Partition_1-2-3_Child_Document_C")
      (Collision|SetActorEnableCollision _childactor_2 false)
      (Variables|Default|SetFirst_Partition_Transform (Transformation|GetActorTransform _childactor_2))
      (Variables|Default|SetSecond_Partition_Transform (Transformation|GetActorTransform _childactor_3))
      (Variables|Default|SetThird_Partition_Transform (Transformation|GetActorTransform _childactor))
      (bind _replace_object (Timeline|Timeline_1 PlayFromStart)
        (:Update
          (Transformation|SetActorTransform _childactor_2 (Math|Transform|Lerp(Transform) (Variables|Default|GetFirst_Partition_Transform) (Math|Transform|MakeTransform (.location _returnvalue_2) (.rotation _returnvalue_2) "1.000000,1.000000,1.000000") _replace_object))
          (Transformation|SetActorTransform _childactor_3 (Math|Transform|Lerp(Transform) (Variables|Default|GetSecond_Partition_Transform) (Math|Transform|MakeTransform (.location _returnvalue_3) (.rotation _returnvalue_3) "1.000000,1.000000,1.000000") _replace_object))
          (Transformation|SetActorTransform _childactor (Math|Transform|Lerp(Transform) (Variables|Default|GetThird_Partition_Transform) (Math|Transform|MakeTransform (.location _returnvalue) (.rotation _returnvalue) "1.000000,1.000000,1.000000") _replace_object)))
        (:Finished
          (Default|TransmissDialogue (Variables|Default|GetFirst_Person) "Driiiiing"))))))

(event EventBeginPlay
  (|CallParentFunction) ; This node is disabled and will not be called.\nDrag off pins to build functionality.
)

(event Collision|EventActorBeginOverlap
  (params (OtherActor :type Actor%20Object%20Reference))
  (|CallParentFunction OtherActor) ; This node is disabled and will not be called.\nDrag off pins to build functionality.
)

(event EventTick
  (params (DeltaSeconds :type Float%20%28single-precision%29))
  (|CallParentFunction DeltaSeconds) ; This node is disabled and will not be called.\nDrag off pins to build functionality.
)

(event EventActionWithoutObject
  (Default|CheckifAllPartition (Variables|Default|GetFirst_Person)))

(fn ConstructionScript
  (|CallParentFunction))