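; Weight-box puzzle where the player places up to four inventory weights on a balance to level its arrow and reveal a reward.
; Success glides the incoming weight into the first empty slot via timelines; BalanceDeMort returns a clicked slot's weight to FirstPerson, with third and fourth slot references mixed up.
; Each change rolls the arrow by weight.
; A near-zero-roll check spawns the reward and shifts HiddenReward, but no live code here calls it.
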(event Custom|Balance_Movement
  (params (Poids :type Float%20%28double-precision%29))
  (bind _arrow (Variables|Default|GetArrow))
  (bind _relativerotation (Variables|/Script/Engine.SceneComponent|GetRelativeRotation _arrow))
  (Transformation|SetRelativeRotation _arrow (Math|Rotator|MakeRotator (+ (.roll _relativerotation) (* Poids 1e+01)) (.pitch _relativerotation) (.yaw _relativerotation)) false false))

(event Custom|Balance_Perfected_?
  (bind _arrow (Variables|Default|GetArrow))
  (bind _returnvalue (Transformation|GetWorldRotation _arrow))
  (if (not (Variables|Default|GetRIddle_Finished_?))
    (if (and (< (.roll _returnvalue) 1.0) (> (.roll _returnvalue) -1.0))
      (ChildActorComponent|SetChildActorClass (Variables|Default|GetReward) (Variables|Default|GetActor_To_Get))
      (Transformation|SetRelativeLocation (Variables|Default|GetHidden_Reward) (+ (Variables|/Script/Engine.SceneComponent|GetRelativeLocation (Variables|Default|GetHidden_Reward)) "0,50.000000,0") false false))))

(event EventBeginPlay
  (|CallParentFunction) ; This node is disabled and will not be called.\nDrag off pins to build functionality.
)

(event Collision|EventActorBeginOverlap
  (params (OtherActor :type Actor%20Object%20Reference))
  (|CallParentFunction OtherActor) ; This node is disabled and will not be called.\nDrag off pins to build functionality.
)

(event EventTick
  (params (DeltaSeconds :type Float%20%28single-precision%29)))

(event EventSuccess
  (if (not (Utilities|IsValid (Variables|/Script/Engine.ChildActorComponent|GetChildActor (Variables|Default|GetFirst_Poids))))
    (ChildActorComponent|SetChildActorClass (Variables|Default|GetFirst_Poids) (Utilities|GetClass (Variables|Default|GetActor_Moving)))
    (Variables|Default|SetLocation_Of_Actor_To_Spawn (Transformation|GetActorLocation (Variables|Default|GetActor_Moving)))
    (Actor|DestroyActor (Variables|Default|GetActor_Moving))
    (bind _time_to_move_object (Timeline|Timeline_1 PlayFromStart)
      (:Update
        (Transformation|SetActorLocation (Variables|/Script/Engine.ChildActorComponent|GetChildActor (Variables|Default|GetFirst_Poids)) (Math|Vector|Lerp(Vector) (Variables|Default|GetLocation_Of_Actor_To_Spawn) (Transformation|GetWorldLocation (Variables|Default|GetPlace_For_First_Poids)) _time_to_move_object) false false))
      (:Finished
        (bind _asbp_poids_child_inventory (Utilities|Casting|CastToBp_Poids_Child_Inventory (Variables|/Script/Engine.ChildActorComponent|GetChildActor (Variables|Default|GetFirst_Poids))))
        (Collision|SetCollisionProfileName (Variables|Default|GetPlace_For_First_Poids) "BlockAll" true :!class /Script/Engine.PrimitiveComponent)
        (CallFunction|BalanceMovement (Variables|/Game/GD/Interactainable/Inventory/Bp_Poids_Child_Inventory.Bp_Poids_Child_Inventory_C|GetPoids _asbp_poids_child_inventory))))
    (elif (not (Utilities|IsValid (Variables|/Script/Engine.ChildActorComponent|GetChildActor (Variables|Default|GetSecond_Poids))))
      (ChildActorComponent|SetChildActorClass (Variables|Default|GetSecond_Poids) (Utilities|GetClass (Variables|Default|GetActor_Moving)))
      (Variables|Default|SetLocation_Of_Actor_To_Spawn (Transformation|GetActorLocation (Variables|Default|GetActor_Moving)))
      (Actor|DestroyActor (Variables|Default|GetActor_Moving))
      (bind _time_to_move_object_2 (Timeline|Timeline_2 PlayFromStart)
        (:Update
          (Transformation|SetActorLocation (Variables|/Script/Engine.ChildActorComponent|GetChildActor (Variables|Default|GetSecond_Poids)) (Math|Vector|Lerp(Vector) (Variables|Default|GetLocation_Of_Actor_To_Spawn) (Transformation|GetWorldLocation (Variables|Default|GetPlace_For_Second_Poids)) _time_to_move_object_2) false false))
        (:Finished
          (bind _asbp_poids_child_inventory_2 (Utilities|Casting|CastToBp_Poids_Child_Inventory (Variables|/Script/Engine.ChildActorComponent|GetChildActor (Variables|Default|GetSecond_Poids))))
          (Collision|SetCollisionProfileName (Variables|Default|GetPlace_For_Second_Poids) "BlockAll" true :!class /Script/Engine.PrimitiveComponent)
          (CallFunction|BalanceMovement (Variables|/Game/GD/Interactainable/Inventory/Bp_Poids_Child_Inventory.Bp_Poids_Child_Inventory_C|GetPoids _asbp_poids_child_inventory_2))))
      (elif (not (Utilities|IsValid (Variables|/Script/Engine.ChildActorComponent|GetChildActor (Variables|Default|GetThird_Poids))))
        (ChildActorComponent|SetChildActorClass (Variables|Default|GetThird_Poids) (Utilities|GetClass (Variables|Default|GetActor_Moving)))
        (Variables|Default|SetLocation_Of_Actor_To_Spawn (Transformation|GetActorLocation (Variables|Default|GetActor_Moving)))
        (Actor|DestroyActor (Variables|Default|GetActor_Moving))
        (bind _time_to_move_object_3 (Timeline|Timeline_3 PlayFromStart)
          (:Update
            (Transformation|SetActorLocation (Variables|/Script/Engine.ChildActorComponent|GetChildActor (Variables|Default|GetThird_Poids)) (Math|Vector|Lerp(Vector) (Variables|Default|GetLocation_Of_Actor_To_Spawn) (Transformation|GetWorldLocation (Variables|Default|GetPlace_For_Third_Poids)) _time_to_move_object_3) false false))
          (:Finished
            (bind _asbp_poids_child_inventory_3 (Utilities|Casting|CastToBp_Poids_Child_Inventory (Variables|/Script/Engine.ChildActorComponent|GetChildActor (Variables|Default|GetThird_Poids))))
            (Collision|SetCollisionProfileName (Variables|Default|GetPlace_For_Third_Poids) "BlockAll" true :!class /Script/Engine.PrimitiveComponent)
            (CallFunction|BalanceMovement (Variables|/Game/GD/Interactainable/Inventory/Bp_Poids_Child_Inventory.Bp_Poids_Child_Inventory_C|GetPoids _asbp_poids_child_inventory_3))))
        (elif (not (Utilities|IsValid (Variables|/Script/Engine.ChildActorComponent|GetChildActor (Variables|Default|GetFourth_Poids))))
          (ChildActorComponent|SetChildActorClass (Variables|Default|GetFourth_Poids) (Utilities|GetClass (Variables|Default|GetActor_Moving)))
          (Variables|Default|SetLocation_Of_Actor_To_Spawn (Transformation|GetActorLocation (Variables|Default|GetActor_Moving)))
          (Actor|DestroyActor (Variables|Default|GetActor_Moving))
          (bind _time_to_move_object_4 (Timeline|Timeline_4 PlayFromStart)
            (:Update
              (Transformation|SetActorLocation (Variables|/Script/Engine.ChildActorComponent|GetChildActor (Variables|Default|GetFourth_Poids)) (Math|Vector|Lerp(Vector) (Variables|Default|GetLocation_Of_Actor_To_Spawn) (Transformation|GetWorldLocation (Variables|Default|GetPlace_For_Fourth_Poids)) _time_to_move_object_4) false false))
            (:Finished
              (bind _asbp_poids_child_inventory_4 (Utilities|Casting|CastToBp_Poids_Child_Inventory (Variables|/Script/Engine.ChildActorComponent|GetChildActor (Variables|Default|GetFourth_Poids))))
              (Collision|SetCollisionProfileName (Variables|Default|GetPlace_For_Fourth_Poids) "BlockAll" true :!class /Script/Engine.PrimitiveComponent)
              (CallFunction|BalanceMovement (Variables|/Game/GD/Interactainable/Inventory/Bp_Poids_Child_Inventory.Bp_Poids_Child_Inventory_C|GetPoids _asbp_poids_child_inventory_4)))))))))

(event EventBalanceDeMort
  (params (Hit_Component :type Primitive%20Component%20Object%20Reference))
  (bind _first_person (Variables|Default|GetFirst_Person))
  (bind _first_poids (Variables|Default|GetFirst_Poids))
  (bind _third_poids (Variables|Default|GetThird_Poids))
  (bind _second_poids (Variables|Default|GetSecond_Poids))
  (bind _third_poids_2 (Variables|Default|GetThird_Poids))
  (Default|CheckifInventoryItemIsFull _first_person)
  (if (not (Variables|/Game/GD/ThirdPerson/Blueprints/BP_Diplome_First_Person_Project.BP_Diplome_First_Person_Project_C|GetInventory_Item_Full_? _first_person))
    (if (== Hit_Component (Variables|Default|GetPlace_For_First_Poids))
      (bind _returnvalue (Game|SpawnActorfromClass (Utilities|GetClass (Variables|/Script/Engine.ChildActorComponent|GetChildActor _first_poids)) (Math|Transform|MakeTransform (Transformation|GetWorldLocation _first_poids) "0, 0, 0" "1.000000,1.000000,1.000000") "Undefined" 0 0))
      (ChildActorComponent|SetChildActorClass _first_poids 0)
      (Default|GetActorfromBalance (Variables|Default|GetFirst_Person) _returnvalue)
      (Collision|SetCollisionProfileName (Variables|Default|GetPlace_For_First_Poids) "NoCollision" true :!class /Script/Engine.PrimitiveComponent)
      (bind _asbp_poids_child_inventory (Utilities|Casting|CastToBp_Poids_Child_Inventory _returnvalue))
      (CallFunction|BalanceMovement (- (Variables|/Game/GD/Interactainable/Inventory/Bp_Poids_Child_Inventory.Bp_Poids_Child_Inventory_C|GetPoids _asbp_poids_child_inventory) (* (Variables|/Game/GD/Interactainable/Inventory/Bp_Poids_Child_Inventory.Bp_Poids_Child_Inventory_C|GetPoids _asbp_poids_child_inventory) 2.0)))
      (elif (== Hit_Component (Variables|Default|GetPlace_For_Second_Poids))
        (bind _returnvalue_2 (Game|SpawnActorfromClass (Utilities|GetClass (Variables|/Script/Engine.ChildActorComponent|GetChildActor _second_poids)) (Math|Transform|MakeTransform (Transformation|GetWorldLocation _second_poids) "0, 0, 0" "1.000000,1.000000,1.000000") "Undefined" 0 0))
        (ChildActorComponent|SetChildActorClass _second_poids 0)
        (Default|GetActorfromBalance (Variables|Default|GetFirst_Person) _returnvalue_2)
        (Collision|SetCollisionProfileName (Variables|Default|GetPlace_For_Second_Poids) "NoCollision" true :!class /Script/Engine.PrimitiveComponent)
        (bind _asbp_poids_child_inventory_2 (Utilities|Casting|CastToBp_Poids_Child_Inventory _returnvalue_2))
        (CallFunction|BalanceMovement (- (Variables|/Game/GD/Interactainable/Inventory/Bp_Poids_Child_Inventory.Bp_Poids_Child_Inventory_C|GetPoids _asbp_poids_child_inventory_2) (* (Variables|/Game/GD/Interactainable/Inventory/Bp_Poids_Child_Inventory.Bp_Poids_Child_Inventory_C|GetPoids _asbp_poids_child_inventory_2) 2.0)))
        (elif (== Hit_Component (Variables|Default|GetPlace_For_Third_Poids))
          (bind _returnvalue_3 (Game|SpawnActorfromClass (Utilities|GetClass (Variables|/Script/Engine.ChildActorComponent|GetChildActor _third_poids_2)) (Math|Transform|MakeTransform (Transformation|GetWorldLocation _third_poids_2) "0, 0, 0" "1.000000,1.000000,1.000000") "Undefined" 0 0))
          (ChildActorComponent|SetChildActorClass (Variables|Default|GetFourth_Poids) 0)
          (Default|GetActorfromBalance (Variables|Default|GetFirst_Person) _returnvalue_3)
          (Collision|SetCollisionProfileName (Variables|Default|GetPlace_For_Third_Poids) "NoCollision" true :!class /Script/Engine.PrimitiveComponent)
          (bind _asbp_poids_child_inventory_3 (Utilities|Casting|CastToBp_Poids_Child_Inventory _returnvalue_3))
          (CallFunction|BalanceMovement (- (Variables|/Game/GD/Interactainable/Inventory/Bp_Poids_Child_Inventory.Bp_Poids_Child_Inventory_C|GetPoids _asbp_poids_child_inventory_3) (* (Variables|/Game/GD/Interactainable/Inventory/Bp_Poids_Child_Inventory.Bp_Poids_Child_Inventory_C|GetPoids _asbp_poids_child_inventory_3) 2.0)))
          (elif (== 0 (Variables|Default|GetPlace_For_Third_Poids))
            (bind _returnvalue_4 (Game|SpawnActorfromClass (Utilities|GetClass (Variables|/Script/Engine.ChildActorComponent|GetChildActor _third_poids)) (Math|Transform|MakeTransform (Transformation|GetWorldLocation _third_poids) "0, 0, 0" "1.000000,1.000000,1.000000") "Undefined" 0 0))
            (ChildActorComponent|SetChildActorClass _third_poids 0)
            (Default|GetActorfromBalance (Variables|Default|GetFirst_Person) _returnvalue_4)
            (Collision|SetCollisionProfileName (Variables|Default|GetPlace_For_Fourth_Poids) "NoCollision" true :!class /Script/Engine.PrimitiveComponent)
            (bind _asbp_poids_child_inventory_4 (Utilities|Casting|CastToBp_Poids_Child_Inventory _returnvalue_4))
            (CallFunction|BalanceMovement (- (Variables|/Game/GD/Interactainable/Inventory/Bp_Poids_Child_Inventory.Bp_Poids_Child_Inventory_C|GetPoids _asbp_poids_child_inventory_4) (* (Variables|/Game/GD/Interactainable/Inventory/Bp_Poids_Child_Inventory.Bp_Poids_Child_Inventory_C|GetPoids _asbp_poids_child_inventory_4) 2.0)))))))))

(event Input|KeyboardEvents|M
  (params (Key :type Key%20Structure :default "None")))

(fn ConstructionScript
  (|CallParentFunction))