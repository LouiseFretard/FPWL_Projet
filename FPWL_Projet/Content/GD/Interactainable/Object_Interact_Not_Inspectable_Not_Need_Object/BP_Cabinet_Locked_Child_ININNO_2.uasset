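; Locked cabinet with a four-wheel combination lock minigame that opens its doors and spawns a reward when solved.
; PartHit on the Box shows the lock widget and blends the player's cinematic camera to the lock; right-click backs out.
; Wheel events step wrapping counters and animate rotation through a shared timeline, then check the hard-coded code.
; Timelines drive camera blends and door swings; the fourth wheel's turn guard never engages.
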(event Custom|Got_Right_Combination_?
  (bind _first_person_0 (Variables|Default|GetFirst_Person_0))
  (bind _first_person_0_2 (Variables|Default|GetFirst_Person_0))
  (bind _first_person_0_3 (Variables|Default|GetFirst_Person_0))
  (bind _first_person_0_4 (Variables|Default|GetFirst_Person_0))
  (if (Math|Boolean|ANDBoolean (== (Variables|Default|GetHow_Many_Time_First_Roulettes_Rolled_?) 1.0) (== (Variables|Default|GetHow_Many_Time_Second_Roulette_Rolled_?) 8.0) (== (Variables|Default|GetHow_Many_Time_Third_Roulettes_Rolled_?) 9.0) (== (Variables|Default|GetHow_Many_Time_Fourth_Roulettes_Rolled_?) 9.0))
    (Input|DisableInput (Variables|Default|GetFirst_Person_0) (Game|GetPlayerController 0))
    (Variables|Default|SetMay_Get_Out_Of_The_Minigame_? false)
    (Variables|/Script/Engine.PlayerController|SetbShowMouseCursor (Game|GetPlayerController 0) false)
    (Collision|SetCollisionProfileName (Variables|Default|GetBox) "NoCollision" true :!class /Script/Engine.PrimitiveComponent)
    (bind _time_to_move_object (Timeline|Timeline_3 PlayFromStart)
      (:Update
        (Transformation|SetWorldTransform (Variables|/Game/GD/ThirdPerson/Blueprints/BP_Diplome_First_Person_Project.BP_Diplome_First_Person_Project_C|GetCinematic_Camera _first_person_0_2) (Math|Transform|Lerp(Transform) (Variables|Default|GetFollow_Camera_Transform) (Transformation|GetWorldTransform (Variables|/Game/GD/ThirdPerson/Blueprints/BP_Diplome_First_Person_Project.BP_Diplome_First_Person_Project_C|GetFirst_Person_Camera _first_person_0_2)) _time_to_move_object) false false))
      (:Finished
        (Components|Activation|SetActive (Variables|/Game/GD/ThirdPerson/Blueprints/BP_Diplome_First_Person_Project.BP_Diplome_First_Person_Project_C|GetCinematic_Camera _first_person_0_3) false false)
        (Components|Activation|SetActive (Variables|/Game/GD/ThirdPerson/Blueprints/BP_Diplome_First_Person_Project.BP_Diplome_First_Person_Project_C|GetFirst_Person_Camera _first_person_0_3) true false)
        (Variables|/Game/GD/ThirdPerson/Blueprints/BP_Diplome_First_Person_Project.BP_Diplome_First_Person_Project_C|SetInto_Minigame_? _first_person_0_3 false)
        (Widget|RemovefromParent (Variables|Default|GetWidget_For_Minigame))
        (Variables|Default|SetOriginal_Relative_Rotation_Right_Door_Arrow (Variables|/Script/Engine.SceneComponent|GetRelativeRotation (Variables|Default|GetRight_Door_Arrow)))
        (Variables|Default|SetOriginal_Relative_Rotation_Left_Door_Arrow (Variables|/Script/Engine.SceneComponent|GetRelativeRotation (Variables|Default|GetLeft_Door_Arrow)))
        (bind _time_to_move_object_2 (Timeline|Timeline_4 PlayFromStart)
          (:Update
            (Transformation|SetRelativeRotation (Variables|Default|GetRight_Door_Arrow) (Math|Rotator|Lerp(Rotator) (Variables|Default|GetOriginal_Relative_Rotation_Right_Door_Arrow) (Math|Rotator|MakeRotator (.roll (Variables|Default|GetOriginal_Relative_Rotation_Right_Door_Arrow)) (.pitch (Variables|Default|GetOriginal_Relative_Rotation_Right_Door_Arrow)) (+ (.yaw (Variables|Default|GetOriginal_Relative_Rotation_Right_Door_Arrow)) -1.6e+02)) _time_to_move_object_2) false false)
            (Transformation|SetRelativeRotation (Variables|Default|GetLeft_Door_Arrow) (Math|Rotator|Lerp(Rotator) (Variables|Default|GetOriginal_Relative_Rotation_Left_Door_Arrow) (Math|Rotator|MakeRotator (.roll (Variables|Default|GetOriginal_Relative_Rotation_Left_Door_Arrow)) (.pitch (Variables|Default|GetOriginal_Relative_Rotation_Left_Door_Arrow)) (+ (.yaw (Variables|Default|GetOriginal_Relative_Rotation_Left_Door_Arrow)) 1.6e+02)) _time_to_move_object_2) false false))
          (:Finished
            (ChildActorComponent|SetChildActorClass (Variables|Default|GetReward_For_Player) (Variables|Default|GetReward))
            (Collision|SetCollisionEnabled (Variables|Default|GetStaticMesh9) "NoCollision")
            (bind _time_to_move_object_3 (Timeline|Timeline_1 PlayFromStart)
              (:Update
                (Transformation|SetWorldTransform (Variables|/Game/GD/ThirdPerson/Blueprints/BP_Diplome_First_Person_Project.BP_Diplome_First_Person_Project_C|GetCinematic_Camera _first_person_0_4) (Math|Transform|Lerp(Transform) (Variables|Default|GetFollow_Camera_Transform) (Transformation|GetWorldTransform (Variables|/Game/GD/ThirdPerson/Blueprints/BP_Diplome_First_Person_Project.BP_Diplome_First_Person_Project_C|GetFirst_Person_Camera _first_person_0_4)) _time_to_move_object_3) false false))
              (:Finished
                (Components|Activation|SetActive (Variables|/Game/GD/ThirdPerson/Blueprints/BP_Diplome_First_Person_Project.BP_Diplome_First_Person_Project_C|GetCinematic_Camera _first_person_0) false false)
                (Components|Activation|SetActive (Variables|/Game/GD/ThirdPerson/Blueprints/BP_Diplome_First_Person_Project.BP_Diplome_First_Person_Project_C|GetFirst_Person_Camera _first_person_0) true false)
                (Variables|/Game/GD/ThirdPerson/Blueprints/BP_Diplome_First_Person_Project.BP_Diplome_First_Person_Project_C|SetInto_Minigame_? _first_person_0 false)
                (Widget|RemovefromParent (Variables|Default|GetWidget_For_Minigame))
                (Input|EnableInput (Variables|Default|GetFirst_Person_0) (Game|GetPlayerController 0))))))))))

(event Custom|Fourth_Wheel_Down
  (if (not (Variables|Default|GetFourth_Roulette_May_Turn_?))
    (Variables|Default|SetWheel_Which_Turn (Variables|Default|GetFouth_Roulette))
    (Variables|Default|SetFourth_Roulette_May_Turn_? false)
    (Variables|Default|SetSide_To_Turn 36.0)
    (if (> (+ (Variables|Default|GetHow_Many_Time_Fourth_Roulettes_Rolled_?) 1.0) (Variables|Default|GetMax_Roulette))
      (Variables|Default|SetHow_Many_Time_Fourth_Roulettes_Rolled_? (Variables|Default|GetMin_Roulette))
      (else
        (Variables|Default|SetHow_Many_Time_Fourth_Roulettes_Rolled_? (+ (Variables|Default|GetHow_Many_Time_Fourth_Roulettes_Rolled_?) 1.0))))
    (CallFunction|TurnAWheel)))

(event Custom|First_Wheel_Up
  (if (not (Variables|Default|GetFirst_Roulette_May_Turn_?))
    (Variables|Default|SetWheel_Which_Turn (Variables|Default|GetFirst_Roulette))
    (Variables|Default|SetFirst_Roulette_May_Turn_? true)
    (Variables|Default|SetSide_To_Turn -36.0)
    (if (< (- (Variables|Default|GetHow_Many_Time_First_Roulettes_Rolled_?) 1.0) (Variables|Default|GetMin_Roulette))
      (Variables|Default|SetHow_Many_Time_First_Roulettes_Rolled_? (Variables|Default|GetMax_Roulette))
      (else
        (Variables|Default|SetHow_Many_Time_First_Roulettes_Rolled_? (- (Variables|Default|GetHow_Many_Time_First_Roulettes_Rolled_?) 1.0))))
    (CallFunction|TurnAWheel)))

(event Custom|First_Wheel_Down
  (if (not (Variables|Default|GetFirst_Roulette_May_Turn_?))
    (Variables|Default|SetWheel_Which_Turn (Variables|Default|GetFirst_Roulette))
    (Variables|Default|SetFirst_Roulette_May_Turn_? true)
    (Variables|Default|SetSide_To_Turn 36.0)
    (if (> (+ (Variables|Default|GetHow_Many_Time_First_Roulettes_Rolled_?) 1.0) (Variables|Default|GetMax_Roulette))
      (Variables|Default|SetHow_Many_Time_First_Roulettes_Rolled_? (Variables|Default|GetMin_Roulette))
      (else
        (Variables|Default|SetHow_Many_Time_First_Roulettes_Rolled_? (+ (Variables|Default|GetHow_Many_Time_First_Roulettes_Rolled_?) 1.0))))
    (CallFunction|TurnAWheel)))

(event Custom|Third_Wheel_Up
  (if (not (Variables|Default|GetThird_Roulette_May_Turn_?))
    (Variables|Default|SetWheel_Which_Turn (Variables|Default|GetThird_Roulette))
    (Variables|Default|SetThird_Roulette_May_Turn_? true)
    (Variables|Default|SetSide_To_Turn -36.0)
    (if (< (- (Variables|Default|GetHow_Many_Time_Third_Roulettes_Rolled_?) 1.0) (Variables|Default|GetMin_Roulette))
      (Variables|Default|SetHow_Many_Time_Third_Roulettes_Rolled_? (Variables|Default|GetMax_Roulette))
      (else
        (Variables|Default|SetHow_Many_Time_Third_Roulettes_Rolled_? (- (Variables|Default|GetHow_Many_Time_Third_Roulettes_Rolled_?) 1.0))))
    (CallFunction|TurnAWheel)))

(event Custom|Second_Wheel_Up
  (if (not (Variables|Default|GetSecond_Roulette_May_Turn_?))
    (Variables|Default|SetWheel_Which_Turn (Variables|Default|GetSecond_Roulette))
    (Variables|Default|SetSecond_Roulette_May_Turn_? true)
    (Variables|Default|SetSide_To_Turn -36.0)
    (if (< (- (Variables|Default|GetHow_Many_Time_Second_Roulette_Rolled_?) 1.0) (Variables|Default|GetMin_Roulette))
      (Variables|Default|SetHow_Many_Time_Second_Roulette_Rolled_? (Variables|Default|GetMax_Roulette))
      (else
        (Variables|Default|SetHow_Many_Time_Second_Roulette_Rolled_? (- (Variables|Default|GetHow_Many_Time_Second_Roulette_Rolled_?) 1.0))))
    (CallFunction|TurnAWheel)))

(event Custom|Second_Wheel_Down
  (if (not (Variables|Default|GetSecond_Roulette_May_Turn_?))
    (Variables|Default|SetWheel_Which_Turn (Variables|Default|GetSecond_Roulette))
    (Variables|Default|SetSecond_Roulette_May_Turn_? true)
    (Variables|Default|SetSide_To_Turn 36.0)
    (if (> (+ (Variables|Default|GetHow_Many_Time_Second_Roulette_Rolled_?) 1.0) (Variables|Default|GetMax_Roulette))
      (Variables|Default|SetHow_Many_Time_Second_Roulette_Rolled_? (Variables|Default|GetMin_Roulette))
      (else
        (Variables|Default|SetHow_Many_Time_Second_Roulette_Rolled_? (+ (Variables|Default|GetHow_Many_Time_Second_Roulette_Rolled_?) 1.0))))
    (CallFunction|TurnAWheel)))

(event Custom|Turn_A_Wheel
  (Variables|Default|SetOriginal_Relative_Rotation_From_Wheel_Which_Turn (Variables|/Script/Engine.SceneComponent|GetRelativeRotation (Variables|Default|GetWheel_Which_Turn)))
  (bind _item_track (Timeline|Timeline_2 PlayFromStart)
    (:Update
      (Transformation|SetRelativeRotation (Variables|Default|GetWheel_Which_Turn) (Math|Rotator|Lerp(Rotator) (Variables|Default|GetOriginal_Relative_Rotation_From_Wheel_Which_Turn) (Math|Rotator|MakeRotator (+ (.roll (Variables|Default|GetOriginal_Relative_Rotation_From_Wheel_Which_Turn)) (Variables|Default|GetSide_To_Turn)) (.pitch (Variables|Default|GetOriginal_Relative_Rotation_From_Wheel_Which_Turn)) (.yaw (Variables|Default|GetOriginal_Relative_Rotation_From_Wheel_Which_Turn))) _item_track) false false))
    (:Finished
      (CallFunction|GotRightCombination?)
      (if (== (Variables|Default|GetWheel_Which_Turn) (Variables|Default|GetFirst_Roulette))
        (Variables|Default|SetFirst_Roulette_May_Turn_? false)
        (elif (== (Variables|Default|GetWheel_Which_Turn) (Variables|Default|GetSecond_Roulette))
          (Variables|Default|SetSecond_Roulette_May_Turn_? false)
          (elif (== (Variables|Default|GetWheel_Which_Turn) (Variables|Default|GetThird_Roulette))
            (Variables|Default|SetThird_Roulette_May_Turn_? false)
            (elif (== (Variables|Default|GetWheel_Which_Turn) (Variables|Default|GetFouth_Roulette))
              (Variables|Default|SetFourth_Roulette_May_Turn_? false))))))))

(event Custom|Third_Wheel_Down
  (if (not (Variables|Default|GetThird_Roulette_May_Turn_?))
    (Variables|Default|SetWheel_Which_Turn (Variables|Default|GetThird_Roulette))
    (Variables|Default|SetThird_Roulette_May_Turn_? true)
    (Variables|Default|SetSide_To_Turn 36.0)
    (if (> (+ (Variables|Default|GetHow_Many_Time_Third_Roulettes_Rolled_?) 1.0) (Variables|Default|GetMax_Roulette))
      (Variables|Default|SetHow_Many_Time_Third_Roulettes_Rolled_? (Variables|Default|GetMin_Roulette))
      (else
        (Variables|Default|SetHow_Many_Time_Third_Roulettes_Rolled_? (+ (Variables|Default|GetHow_Many_Time_Third_Roulettes_Rolled_?) 1.0))))
    (CallFunction|TurnAWheel)))

(event Custom|Fourth_Wheel_Up
  (if (not (Variables|Default|GetFourth_Roulette_May_Turn_?))
    (Variables|Default|SetWheel_Which_Turn (Variables|Default|GetFouth_Roulette))
    (Variables|Default|SetFourth_Roulette_May_Turn_? false)
    (Variables|Default|SetSide_To_Turn -36.0)
    (if (< (- (Variables|Default|GetHow_Many_Time_Fourth_Roulettes_Rolled_?) 1.0) (Variables|Default|GetMin_Roulette))
      (Variables|Default|SetHow_Many_Time_Fourth_Roulettes_Rolled_? (Variables|Default|GetMax_Roulette))
      (else
        (Variables|Default|SetHow_Many_Time_Fourth_Roulettes_Rolled_? (- (Variables|Default|GetHow_Many_Time_Fourth_Roulettes_Rolled_?) 1.0))))
    (CallFunction|TurnAWheel)))

(event EventBeginPlay
  (|CallParentFunction) ; This node is disabled and will not be called.\nDrag off pins to build functionality.
)

(event Collision|EventActorBeginOverlap
  (params (OtherActor :type Actor%20Object%20Reference))
  (|CallParentFunction OtherActor) ; This node is disabled and will not be called.\nDrag off pins to build functionality.
)

(event EventTick
  (params (DeltaSeconds :type Float%20%28single-precision%29))
  (|CallParentFunction DeltaSeconds) ; This node is disabled and will not be called.\nDrag off pins to build functionality.
)

(event EventPartHit
  (params (Hit_Component :type Primitive%20Component%20Object%20Reference) (Pawn :type Pawn%20Object%20Reference))
  (bind _asbp_diplome_first_person_project (Utilities|Casting|CastToBP_Diplome_First_Person_Project Pawn))
  (Utilities|IsValid (Variables|Default|GetFirst_Person_0)
    (:Is%20Valid
      _)
    (:Is%20Not%20Valid
      (Variables|Default|SetFirst_Person_0 _asbp_diplome_first_person_project)))
  (if (== Hit_Component (Variables|Default|GetBox))
    (Variables|/Game/GD/ThirdPerson/Blueprints/BP_Diplome_First_Person_Project.BP_Diplome_First_Person_Project_C|SetInto_Minigame_? (Variables|Default|GetFirst_Person_0) true)
    (Variables|/Script/Engine.PlayerController|SetbShowMouseCursor (Game|GetPlayerController 0) true)
    (Collision|SetCollisionProfileName (Variables|Default|GetBox) "None" true :!class /Script/Engine.PrimitiveComponent)
    (bind _returnvalue (UserInterface|CreateWidget "/Game/GD/Widget/Menu_Minigame_Locker_3.Menu_Minigame_Locker_3_C"))
    (UserInterface|Viewport|AddtoViewport _returnvalue 0)
    (Variables|Default|SetWidget_For_Minigame _returnvalue)
    (Transformation|SetWorldTransform (Variables|/Game/GD/ThirdPerson/Blueprints/BP_Diplome_First_Person_Project.BP_Diplome_First_Person_Project_C|GetCinematic_Camera (Variables|Default|GetFirst_Person_0)) (Transformation|GetWorldTransform (Variables|/Game/GD/ThirdPerson/Blueprints/BP_Diplome_First_Person_Project.BP_Diplome_First_Person_Project_C|GetFirst_Person_Camera (Variables|Default|GetFirst_Person_0))) false false)
    (Variables|Default|SetFollow_Camera_Transform (Transformation|GetWorldTransform (Variables|/Game/GD/ThirdPerson/Blueprints/BP_Diplome_First_Person_Project.BP_Diplome_First_Person_Project_C|GetCinematic_Camera (Variables|Default|GetFirst_Person_0))))
    (Components|Activation|SetActive (Variables|/Game/GD/ThirdPerson/Blueprints/BP_Diplome_First_Person_Project.BP_Diplome_First_Person_Project_C|GetCinematic_Camera (Variables|Default|GetFirst_Person_0)) true false)
    (Components|Activation|SetActive (Variables|/Game/GD/ThirdPerson/Blueprints/BP_Diplome_First_Person_Project.BP_Diplome_First_Person_Project_C|GetFirst_Person_Camera (Variables|Default|GetFirst_Person_0)) false false)
    (bind _time_to_move_object (Timeline|Timeline_0 PlayFromStart)
      (:Update
        (Transformation|SetWorldTransform (Variables|/Game/GD/ThirdPerson/Blueprints/BP_Diplome_First_Person_Project.BP_Diplome_First_Person_Project_C|GetCinematic_Camera (Variables|Default|GetFirst_Person_0)) (Math|Transform|Lerp(Transform) (Variables|Default|GetFollow_Camera_Transform) (Transformation|GetWorldTransform (Variables|Default|GetCube6)) _time_to_move_object) false false))
      (:Finished
        (Variables|Default|SetFollow_Camera_Transform (Transformation|GetWorldTransform (Variables|/Game/GD/ThirdPerson/Blueprints/BP_Diplome_First_Person_Project.BP_Diplome_First_Person_Project_C|GetCinematic_Camera (Variables|Default|GetFirst_Person_0))))
        (Variables|Default|SetMay_Get_Out_Of_The_Minigame_? true)))))

(event Input|MouseEvents|RightMouseButton
  (params (Key :type Key%20Structure :default "None"))
  (bind _first_person_0 (Variables|Default|GetFirst_Person_0))
  (bind _first_person_0_2 (Variables|Default|GetFirst_Person_0))
  (:Pressed
    (if (Variables|Default|GetMay_Get_Out_Of_The_Minigame_?)
      (Variables|Default|SetMay_Get_Out_Of_The_Minigame_? false)
      (Variables|/Script/Engine.PlayerController|SetbShowMouseCursor (Game|GetPlayerController 0) false)
      (Collision|SetCollisionProfileName (Variables|Default|GetBox) "BlockAll" true :!class /Script/Engine.PrimitiveComponent)
      (bind _time_to_move_object (Timeline|Timeline_1 PlayFromStart)
        (:Update
          (Transformation|SetWorldTransform (Variables|/Game/GD/ThirdPerson/Blueprints/BP_Diplome_First_Person_Project.BP_Diplome_First_Person_Project_C|GetCinematic_Camera _first_person_0_2) (Math|Transform|Lerp(Transform) (Variables|Default|GetFollow_Camera_Transform) (Transformation|GetWorldTransform (Variables|/Game/GD/ThirdPerson/Blueprints/BP_Diplome_First_Person_Project.BP_Diplome_First_Person_Project_C|GetFirst_Person_Camera _first_person_0_2)) _time_to_move_object) false false))
        (:Finished
          (Components|Activation|SetActive (Variables|/Game/GD/ThirdPerson/Blueprints/BP_Diplome_First_Person_Project.BP_Diplome_First_Person_Project_C|GetCinematic_Camera _first_person_0) false false)
          (Components|Activation|SetActive (Variables|/Game/GD/ThirdPerson/Blueprints/BP_Diplome_First_Person_Project.BP_Diplome_First_Person_Project_C|GetFirst_Person_Camera _first_person_0) true false)
          (Variables|/Game/GD/ThirdPerson/Blueprints/BP_Diplome_First_Person_Project.BP_Diplome_First_Person_Project_C|SetInto_Minigame_? _first_person_0 false)
          (Widget|RemovefromParent (Variables|Default|GetWidget_For_Minigame))
          (Input|EnableInput (Variables|Default|GetFirst_Person_0) (Game|GetPlayerController 0)))))))

(fn ConstructionScript
  (|CallParentFunction))