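; Interactable light switch that plays a click, flips its lever and can give the player the objective to restore the power.
; PartHit on its box drives a FlipFlop that plays a rotation timeline forward or backward.
; When that finishes with no HUD objective text, it shows dialogue, then sets and slides in the objective once.
; Highlighting toggles a dynamic material parameter; older outline-mesh logic is left unconnected.
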(event EventBeginPlay
  (|CallParentFunction)
  (bind _returnvalue (Rendering|Material|CreateDynamicMaterialInstance "/Game/TA/Materials/Gameplay/Appartement/Interrupteur.Interrupteur" "None" "None" :!class /Script/Engine.KismetMaterialLibrary))
  (bind _output_get (Variables|Default|SetM_inst _returnvalue))
  (Rendering|Material|SetMaterial (Variables|Default|GetStaticMesh) 0 _output_get)
  (Rendering|Material|SetScalarParameterValue (Variables|Default|GetM_inst) "Activate" 0.0 :!class /Script/Engine.MaterialInstanceDynamic))

(event Collision|EventActorBeginOverlap
  (params (OtherActor :type Actor%20Object%20Reference))
  (|CallParentFunction OtherActor) ; This node is disabled and will not be called.\nDrag off pins to build functionality.
)

(event EventTick
  (params (DeltaSeconds :type Float%20%28single-precision%29))
  (|CallParentFunction DeltaSeconds) ; This node is disabled and will not be called.\nDrag off pins to build functionality.
)

(event EventPartHit
  (params (Hit_Component :type Primitive%20Component%20Object%20Reference) (Pawn :type Pawn%20Object%20Reference))
  (if (Math|Boolean|ANDBoolean (== Hit_Component (Variables|Default|GetBox)) (== (Variables|Default|GetAnimation_Going) false) (== (Variables|Default|GetCan_Be_Used_?) true))
    (Audio|PlaySound2D "/Game/GD/Sound/Environment_Noise/SC_Light_Switch_Cue.SC_Light_Switch_Cue" 0.5 1.0 0.0 0 0)
    (Utilities|FlowControl|FlipFlop
      (:A
        (Variables|Default|SetAnimation_Going true)
        (bind _item_track (Timeline|Timeline_0 PlayFromStart)
          (:Update
            (Transformation|SetRelativeRotation (Variables|Default|GetArrow1) (Math|Rotator|Lerp(Rotator) "0.000000,0.000000,-15.000000" "0.000000, 0,15.000000" _item_track) false false))
          (:Finished
            (bind _asbp_diplome_first_person_project (Utilities|Casting|CastToBP_Diplome_First_Person_Project Pawn))
            (Variables|Default|SetAnimation_Going false)
            (if (Utilities|Enum|Equal(Enum) (Class|TextBlock|GetText (Variables|/Game/GD/Widget/HUD.HUD_C|GetHow_To_Show_Objective (Variables|/Game/GD/ThirdPerson/Blueprints/BP_Diplome_First_Person_Project.BP_Diplome_First_Person_Project_C|GetHUD _asbp_diplome_first_person_project))) (Variables|Default|GetNull))
              (Default|TransmissDialogue _asbp_diplome_first_person_project (Variables|Default|GetDialogue))
              (Utilities|FlowControl|Delay 1.0)
              (Default|EndDialogue (Variables|/Game/GD/ThirdPerson/Blueprints/BP_Diplome_First_Person_Project.BP_Diplome_First_Person_Project_C|GetHUD _asbp_diplome_first_person_project))
              (if (not (Variables|Default|GetObjective_Activated_?))
                (Variables|Default|SetObjective_Activated_? true)
                (Audio|PlaySound2D "/Game/GD/Sound/Environment_Noise/Objectif_Sound.Objectif_Sound" 1.0 1.0 0.0 0 0)
                (Widget|SetRenderOpacity (Variables|/Game/GD/Widget/HUD.HUD_C|GetBorder_Objective (Variables|/Game/GD/ThirdPerson/Blueprints/BP_Diplome_First_Person_Project.BP_Diplome_First_Person_Project_C|GetHUD _asbp_diplome_first_person_project)) 1.0)
                (Rendering|Components|TextRender|SetText (Variables|/Game/GD/Widget/HUD.HUD_C|GetHow_To_Show_Objective (Variables|/Game/GD/ThirdPerson/Blueprints/BP_Diplome_First_Person_Project.BP_Diplome_First_Person_Project_C|GetHUD _asbp_diplome_first_person_project)) "Objectif : Rallumer le courant ")
                (Variables|Default|SetAnimation_Going false)
                (bind _item_track_2 (Timeline|Timeline_1 PlayFromStart)
                  (:Update
                    (Class|Widget|SetRenderTranslation (Variables|/Game/GD/Widget/HUD.HUD_C|GetBorder_Objective (Variables|/Game/GD/ThirdPerson/Blueprints/BP_Diplome_First_Person_Project.BP_Diplome_First_Person_Project_C|GetHUD _asbp_diplome_first_person_project)) (Math|Vector2D|MakeVector2D (Math|Float|Lerp 565.0 -1.8e+02 _item_track_2) (.y (.translation (Variables|/Script/UMG.Widget|GetRenderTransform (Variables|/Game/GD/Widget/HUD.HUD_C|GetBorder_Objective (Variables|/Game/GD/ThirdPerson/Blueprints/BP_Diplome_First_Person_Project.BP_Diplome_First_Person_Project_C|GetHUD _asbp_diplome_first_person_project)))))))))
                (else
                  (Variables|Default|SetAnimation_Going false)))))))
      (:B
        (Variables|Default|SetAnimation_Going true)
        (Timeline|Timeline_0 ReverseFromEnd)))))

(event EventOnHighlight
  (Rendering|Material|SetScalarParameterValue (Variables|Default|GetM_inst) "Activate" 1.0 :!class /Script/Engine.MaterialInstanceDynamic))

(event EventStopHighlight
  (Rendering|Material|SetScalarParameterValue (Variables|Default|GetM_inst) "Activate" 0.0 :!class /Script/Engine.MaterialInstanceDynamic))

(fn ConstructionScript
  (|CallParentFunction))