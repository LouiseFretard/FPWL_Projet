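; Interactable piano sealed by a four-wheel combination padlock minigame, refusing use with a dialogue line until Start_Piano enables it.
; Interaction blends a cinematic camera to the lock, where left-clicks on hit boxes spin wheels via timelines and right-click exits.
; Each turn checks a hardcoded code; success animates lock and lid open, spawns the reward child actor and restores player control.
; Later interactions call the player's partition-completion check.
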(event Custom|Got_Right_Combination_?
  (bind _first_person_0 (Variables|Default|GetFirst_Person_0))
  (bind _first_person_0_2 (Variables|Default|GetFirst_Person_0))
  (bind _first_person_0_3 (Variables|Default|GetFirst_Person_0))
  (bind _first_person_0_4 (Variables|Default|GetFirst_Person_0))
  (bind _first_person_0_5 (Variables|Default|GetFirst_Person_0))
  (if (Math|Boolean|ANDBoolean (== (Variables|Default|GetHow_Many_Time_First_Roulettes_Rolled_?) 1.0) (== (Variables|Default|GetHow_Many_Time_Second_Roulette_Rolled_?) 8.0) (== (Variables|Default|GetHow_Many_Time_Third_Roulettes_Rolled_?) 7.0) (== (Variables|Default|GetHow_Many_Time_Fourth_Roulettes_Rolled_?) 6.0))
    (Input|DisableInput (Variables|Default|GetFirst_Person_0) (Game|GetPlayerController 0))
    (Variables|Default|SetMay_Get_Out_Of_The_Minigame_? false)
    (Variables|/Script/Engine.PlayerController|SetbShowMouseCursor (Game|GetPlayerController 0) false)
    (Collision|SetCollisionProfileName (Variables|Default|GetBox) "NoCollision" true :!class /Script/Engine.PrimitiveComponent)
    (bind _time_to_move_object (Timeline|Timeline_3 PlayFromStart)
      (:Update
        (Transformation|SetWorldTransform (Variables|/Game/GD/ThirdPerson/Blueprints/BP_Diplome_First_Person_Project.BP_Diplome_First_Person_Project_C|GetCinematic_Camera _first_person_0_2) (Math|Transform|Lerp(Transform) (Variables|Default|GetFollow_Camera_Transform) (Transformation|GetWorldTransform (Variables|/Game/GD/ThirdPerson/Blueprints/BP_Diplome_First_Person_Project.BP_Diplome_First_Person_Project_C|GetFirst_Person_Camera _first_person_0_2)) _time_to_move_object) false false))
      (:Finished
        (Components|Activation|SetActive (Variables|/Game/GD/ThirdPerson/Blueprints/BP_Diplome_First_Person_Project.BP_Diplome_First_Person_Project_C|GetCinematic_Camera _first_person_0_4) false false)
        (Components|Activation|SetActive (Variables|/Game/GD/ThirdPerson/Blueprints/BP_Diplome_First_Person_Project.BP_Diplome_First_Person_Project_C|GetFirst_Person_Camera _first_person_0_4) true false)
        (Variables|/Game/GD/ThirdPerson/Blueprints/BP_Diplome_First_Person_Project.BP_Diplome_First_Person_Project_C|SetInto_Minigame_? _first_person_0_4 false)
        (Variables|Default|SetRelative_Rotation_Locker_Openin (Variables|/Script/Engine.SceneComponent|GetRelativeRotation (Variables|Default|GetCadenas_UE_Ouverture_LP1)))
        (Utilities|FlowControl|Sequence
          (:then_0
            (bind _time_to_move_object_2 (Timeline|Timeline_4 PlayFromStart)
              (:Update
                (Transformation|SetRelativeRotation (Variables|Default|GetCadenas_UE_Ouverture_LP1) (Math|Rotator|Lerp(Rotator) (Variables|Default|GetRelative_Rotation_Locker_Openin) (Math|Rotator|MakeRotator (+ (.Roll (Math|Rotator|BreakRotator (Variables|Default|GetRelative_Rotation_Locker_Openin))) 9e+01) (.Pitch (Math|Rotator|BreakRotator (Variables|Default|GetRelative_Rotation_Locker_Openin))) (.Yaw (Math|Rotator|BreakRotator (Variables|Default|GetRelative_Rotation_Locker_Openin)))) _time_to_move_object_2) false false)
                (Utilities|FlowControl|DoOnce false
                  (:Completed
                    (Variables|Default|SetArrow_Opening_Piano (Variables|/Script/Engine.SceneComponent|GetRelativeRotation (Variables|Default|GetArrow_Chest_Open)))
                    (bind _time_to_move_object_3 (Timeline|Timeline_5 PlayFromStart)
                      (:Update
                        (Transformation|SetRelativeRotation (Variables|Default|GetArrow_Chest_Open) (Math|Rotator|Lerp(Rotator) (Variables|Default|GetArrow_Opening_Piano) (Math|Rotator|MakeRotator (.Roll (Math|Rotator|BreakRotator (Variables|Default|GetArrow_Opening_Piano))) (+ (.Pitch (Math|Rotator|BreakRotator (Variables|Default|GetArrow_Opening_Piano))) 9e+01) (.Yaw (Math|Rotator|BreakRotator (Variables|Default|GetArrow_Opening_Piano)))) _time_to_move_object_3) false false))))))))
          (:then_1
            (ChildActorComponent|SetChildActorClass (Variables|Default|GetReward_For_Player) (Variables|Default|GetReward))
            (Variables|Default|SetUnlock_Ended_? true)
            (Variables|Default|SetCan_Be_Used_? false)
            (Collision|SetCollisionProfileName (Variables|Default|GetBox) "BlockAll" true :!class /Script/Engine.PrimitiveComponent)
            (bind _time_to_move_object_4 (Timeline|Timeline_1 PlayFromStart)
              (:Update
                (Transformation|SetWorldTransform (Variables|/Game/GD/ThirdPerson/Blueprints/BP_Diplome_First_Person_Project.BP_Diplome_First_Person_Project_C|GetCinematic_Camera _first_person_0_5) (Math|Transform|Lerp(Transform) (Variables|Default|GetFollow_Camera_Transform) (Transformation|GetWorldTransform (Variables|/Game/GD/ThirdPerson/Blueprints/BP_Diplome_First_Person_Project.BP_Diplome_First_Person_Project_C|GetFirst_Person_Camera _first_person_0_5)) _time_to_move_object_4) false false))
              (:Finished
                (Components|Activation|SetActive (Variables|/Game/GD/ThirdPerson/Blueprints/BP_Diplome_First_Person_Project.BP_Diplome_First_Person_Project_C|GetCinematic_Camera _first_person_0) false false)
                (Components|Activation|SetActive (Variables|/Game/GD/ThirdPerson/Blueprints/BP_Diplome_First_Person_Project.BP_Diplome_First_Person_Project_C|GetFirst_Person_Camera _first_person_0) true false)
                (Variables|/Game/GD/ThirdPerson/Blueprints/BP_Diplome_First_Person_Project.BP_Diplome_First_Person_Project_C|SetInto_Minigame_? _first_person_0 false)
                (Input|DisableInput (Game|GetPlayerController 0))
                (Input|EnableInput _first_person_0_3 (Game|GetPlayerController 0))
                (Collision|SetCollisionProfileName (Variables|/Game/GD/ThirdPerson/Blueprints/BP_Diplome_First_Person_Project.BP_Diplome_First_Person_Project_C|GetHighlight_Detection _first_person_0_3) "OverlapAllDynamic" true :!class /Script/Engine.PrimitiveComponent)))))))))

(event Custom|Fourth_Wheel_Down
  (if (not (Variables|Default|GetFourth_Roulette_May_Turn_?))
    (Variables|Default|SetWheel_Turning (Variables|Default|GetCadenas_UE_Roulette_LP7))
    (Variables|Default|SetFourth_Roulette_May_Turn_? true)
    (Variables|Default|SetSide_To_Turn 4e+01)
    (if (< (- (Variables|Default|GetHow_Many_Time_Fourth_Roulettes_Rolled_?) 1.0) (Variables|Default|GetMin_Roulette))
      (Variables|Default|SetHow_Many_Time_Fourth_Roulettes_Rolled_? (Variables|Default|GetMax_Roulette))
      (else
        (Variables|Default|SetHow_Many_Time_Fourth_Roulettes_Rolled_? (- (Variables|Default|GetHow_Many_Time_Fourth_Roulettes_Rolled_?) 1.0))))
    (CallFunction|TurnAWheel)))

(event Custom|First_Wheel_Up
  (if (not (Variables|Default|GetFirst_Roulette_May_Turn_?))
    (Variables|Default|SetWheel_Turning (Variables|Default|GetCadenas_UE_Roulette_LP4))
    (Variables|Default|SetFirst_Roulette_May_Turn_? true)
    (Variables|Default|SetSide_To_Turn -4e+01)
    (if (> (+ (Variables|Default|GetHow_Many_Time_First_Roulettes_Rolled_?) 1.0) (Variables|Default|GetMax_Roulette))
      (Variables|Default|SetHow_Many_Time_First_Roulettes_Rolled_? (Variables|Default|GetMin_Roulette))
      (else
        (Variables|Default|SetHow_Many_Time_First_Roulettes_Rolled_? (+ (Variables|Default|GetHow_Many_Time_First_Roulettes_Rolled_?) 1.0))))
    (CallFunction|TurnAWheel)))

(event Custom|First_Wheel_Down
  (if (not (Variables|Default|GetFirst_Roulette_May_Turn_?))
    (Variables|Default|SetWheel_Turning (Variables|Default|GetCadenas_UE_Roulette_LP4))
    (Variables|Default|SetFirst_Roulette_May_Turn_? true)
    (Variables|Default|SetSide_To_Turn 4e+01)
    (if (< (- (Variables|Default|GetHow_Many_Time_First_Roulettes_Rolled_?) 1.0) (Variables|Default|GetMin_Roulette))
      (Variables|Default|SetHow_Many_Time_First_Roulettes_Rolled_? (Variables|Default|GetMax_Roulette))
      (else
        (Variables|Default|SetHow_Many_Time_First_Roulettes_Rolled_? (- (Variables|Default|GetHow_Many_Time_First_Roulettes_Rolled_?) 1.0))))
    (CallFunction|TurnAWheel)))

(event Custom|Third_Wheel_Up
  (if (not (Variables|Default|GetThird_Roulette_May_Turn_?))
    (Variables|Default|SetWheel_Turning (Variables|Default|GetCadenas_UE_Roulette_LP6))
    (Variables|Default|SetThird_Roulette_May_Turn_? true)
    (Variables|Default|SetSide_To_Turn -4e+01)
    (if (> (+ (Variables|Default|GetHow_Many_Time_Third_Roulettes_Rolled_?) 1.0) (Variables|Default|GetMax_Roulette))
      (Variables|Default|SetHow_Many_Time_Third_Roulettes_Rolled_? (Variables|Default|GetMin_Roulette))
      (else
        (Variables|Default|SetHow_Many_Time_Third_Roulettes_Rolled_? (+ (Variables|Default|GetHow_Many_Time_Third_Roulettes_Rolled_?) 1.0))))
    (CallFunction|TurnAWheel)))

(event Custom|Second_Wheel_Up
  (if (not (Variables|Default|GetSecond_Roulette_May_Turn_?))
    (Variables|Default|SetWheel_Turning (Variables|Default|GetCadenas_UE_Roulette_LP5))
    (Variables|Default|SetSecond_Roulette_May_Turn_? true)
    (Variables|Default|SetSide_To_Turn -4e+01)
    (if (> (+ (Variables|Default|GetHow_Many_Time_Second_Roulette_Rolled_?) 1.0) (Variables|Default|GetMax_Roulette))
      (Variables|Default|SetHow_Many_Time_Second_Roulette_Rolled_? (Variables|Default|GetMin_Roulette))
      (else
        (Variables|Default|SetHow_Many_Time_Second_Roulette_Rolled_? (+ (Variables|Default|GetHow_Many_Time_Second_Roulette_Rolled_?) 1.0))))
    (CallFunction|TurnAWheel)))

(event Custom|Second_Wheel_Down
  (if (not (Variables|Default|GetSecond_Roulette_May_Turn_?))
    (Variables|Default|SetWheel_Turning (Variables|Default|GetCadenas_UE_Roulette_LP5))
    (Variables|Default|SetSecond_Roulette_May_Turn_? true)
    (Variables|Default|SetSide_To_Turn 4e+01)
    (if (< (- (Variables|Default|GetHow_Many_Time_Second_Roulette_Rolled_?) 1.0) (Variables|Default|GetMin_Roulette))
      (Variables|Default|SetHow_Many_Time_Second_Roulette_Rolled_? (Variables|Default|GetMax_Roulette))
      (else
        (Variables|Default|SetHow_Many_Time_Second_Roulette_Rolled_? (- (Variables|Default|GetHow_Many_Time_Second_Roulette_Rolled_?) 1.0))))
    (CallFunction|TurnAWheel)))

(event Custom|Turn_A_Wheel
  (bind _wheel_turning (Variables|Default|GetWheel_Turning))
  (Variables|Default|SetOriginal_Relative_Rotation_From_Wheel_Which_Turn (Variables|/Script/Engine.SceneComponent|GetRelativeRotation (Variables|Default|GetWheel_Turning)))
  (bind _item_track (Timeline|Timeline_2 PlayFromStart)
    (:Update
      (Transformation|SetRelativeRotation (Variables|Default|GetWheel_Turning) (Math|Rotator|Lerp(Rotator) (Variables|Default|GetOriginal_Relative_Rotation_From_Wheel_Which_Turn) (Math|Rotator|MakeRotator (+ (.roll (Variables|Default|GetOriginal_Relative_Rotation_From_Wheel_Which_Turn)) (Variables|Default|GetSide_To_Turn)) (.pitch (Variables|Default|GetOriginal_Relative_Rotation_From_Wheel_Which_Turn)) (.yaw (Variables|Default|GetOriginal_Relative_Rotation_From_Wheel_Which_Turn))) _item_track) false false))
    (:Finished
      (CallFunction|GotRightCombination?)
      (if (== _wheel_turning (Variables|Default|GetCadenas_UE_Roulette_LP4))
        (Variables|Default|SetFirst_Roulette_May_Turn_? false)
        (elif (== _wheel_turning (Variables|Default|GetCadenas_UE_Roulette_LP5))
          (Variables|Default|SetSecond_Roulette_May_Turn_? false)
          (elif (== _wheel_turning (Variables|Default|GetCadenas_UE_Roulette_LP6))
            (Variables|Default|SetThird_Roulette_May_Turn_? false)
            (elif (== _wheel_turning (Variables|Default|GetCadenas_UE_Roulette_LP7))
              (Variables|Default|SetFourth_Roulette_May_Turn_? false))))))))

(event Custom|Third_Wheel_Down
  (if (not (Variables|Default|GetThird_Roulette_May_Turn_?))
    (Variables|Default|SetWheel_Turning (Variables|Default|GetCadenas_UE_Roulette_LP6))
    (Variables|Default|SetThird_Roulette_May_Turn_? true)
    (Variables|Default|SetSide_To_Turn 4e+01)
    (if (< (- (Variables|Default|GetHow_Many_Time_Third_Roulettes_Rolled_?) 1.0) (Variables|Default|GetMin_Roulette))
      (Variables|Default|SetHow_Many_Time_Third_Roulettes_Rolled_? (Variables|Default|GetMax_Roulette))
      (else
        (Variables|Default|SetHow_Many_Time_Third_Roulettes_Rolled_? (- (Variables|Default|GetHow_Many_Time_Third_Roulettes_Rolled_?) 1.0))))
    (CallFunction|TurnAWheel)))

(event Custom|Start_Piano
  (Variables|Default|SetCan_Be_Used_?_0 true))

(event Custom|All_Partitions_Gathered)

(event Custom|Fourth_Wheel_Up
  (if (not (Variables|Default|GetFourth_Roulette_May_Turn_?))
    (Variables|Default|SetWheel_Turning (Variables|Default|GetCadenas_UE_Roulette_LP7))
    (Variables|Default|SetFourth_Roulette_May_Turn_? true)
    (Variables|Default|SetSide_To_Turn -4e+01)
    (if (> (+ (Variables|Default|GetHow_Many_Time_Fourth_Roulettes_Rolled_?) 1.0) (Variables|Default|GetMax_Roulette))
      (Variables|Default|SetHow_Many_Time_Fourth_Roulettes_Rolled_? (Variables|Default|GetMin_Roulette))
      (else
        (Variables|Default|SetHow_Many_Time_Fourth_Roulettes_Rolled_? (+ (Variables|Default|GetHow_Many_Time_Fourth_Roulettes_Rolled_?) 1.0))))
    (CallFunction|TurnAWheel)))

(event EventBeginPlay
  (|CallParentFunction)
  (Transformation|AttachComponentToComponent (Variables|Default|GetArrow_Locker) 0 "None" "KeepWorld" "KeepWorld" "KeepWorld" true))

(event Collision|EventActorBeginOverlap
  (params (OtherActor :type Actor%20Object%20Reference))
  (|CallParentFunction OtherActor) ; This node is disabled and will not be called.\nDrag off pins to build functionality.
)

(event EventTick
  (params (DeltaSeconds :type Float%20%28single-precision%29))
  (|CallParentFunction DeltaSeconds) ; This node is disabled and will not be called.\nDrag off pins to build functionality.
)

(event EventPartHit
  (params (Hit_Component :type Primitive%20Component%20Object%20Reference) (Pawn :type Pawn%20Object%20Reference))
  (bind _asbp_diplome_first_person_project (Utilities|Casting|CastToBP_Diplome_First_Person_Project Pawn))
  (Utilities|IsValid (Variables|Default|GetFirst_Person_0)
    (:Is%20Valid
      _)
    (:Is%20Not%20Valid
      (Variables|Default|SetFirst_Person_0 _asbp_diplome_first_person_project)))
  (if (Variables|Default|GetCan_Be_Used_?_0)
    (if (== Hit_Component (Variables|Default|GetBox))
      (if (not (Variables|Default|GetUnlock_Ended_?))
        (Variables|Default|SetCan_Be_Used_? false)
        (Input|DisableInput (Variables|Default|GetFirst_Person_0) (Game|GetPlayerController 0))
        (Collision|SetCollisionProfileName (Variables|Default|GetBox) "NoCollision" true :!class /Script/Engine.PrimitiveComponent)
        (Variables|/Game/GD/ThirdPerson/Blueprints/BP_Diplome_First_Person_Project.BP_Diplome_First_Person_Project_C|SetInto_Minigame_? (Variables|Default|GetFirst_Person_0) true)
        (Variables|/Script/Engine.PlayerController|SetbShowMouseCursor (Game|GetPlayerController 0) true)
        (Collision|SetCollisionProfileName (Variables|Default|GetBox) "None" true :!class /Script/Engine.PrimitiveComponent)
        (Transformation|SetWorldTransform (Variables|/Game/GD/ThirdPerson/Blueprints/BP_Diplome_First_Person_Project.BP_Diplome_First_Person_Project_C|GetCinematic_Camera (Variables|Default|GetFirst_Person_0)) (Transformation|GetWorldTransform (Variables|/Game/GD/ThirdPerson/Blueprints/BP_Diplome_First_Person_Project.BP_Diplome_First_Person_Project_C|GetFirst_Person_Camera (Variables|Default|GetFirst_Person_0))) false false)
        (Variables|Default|SetFollow_Camera_Transform (Transformation|GetWorldTransform (Variables|/Game/GD/ThirdPerson/Blueprints/BP_Diplome_First_Person_Project.BP_Diplome_First_Person_Project_C|GetCinematic_Camera (Variables|Default|GetFirst_Person_0))))
        (Components|Activation|SetActive (Variables|/Game/GD/ThirdPerson/Blueprints/BP_Diplome_First_Person_Project.BP_Diplome_First_Person_Project_C|GetCinematic_Camera (Variables|Default|GetFirst_Person_0)) true false)
        (Components|Activation|SetActive (Variables|/Game/GD/ThirdPerson/Blueprints/BP_Diplome_First_Person_Project.BP_Diplome_First_Person_Project_C|GetFirst_Person_Camera (Variables|Default|GetFirst_Person_0)) false false)
        (bind _time_to_move_object (Timeline|Timeline_0 PlayFromStart)
          (:Update
            (Transformation|SetWorldTransform (Variables|/Game/GD/ThirdPerson/Blueprints/BP_Diplome_First_Person_Project.BP_Diplome_First_Person_Project_C|GetCinematic_Camera (Variables|Default|GetFirst_Person_0)) (Math|Transform|Lerp(Transform) (Variables|Default|GetFollow_Camera_Transform) (Transformation|GetWorldTransform (Variables|Default|GetCube6)) _time_to_move_object) false false))
          (:Finished
            (Variables|Default|SetFollow_Camera_Transform (Transformation|GetWorldTransform (Variables|/Game/GD/ThirdPerson/Blueprints/BP_Diplome_First_Person_Project.BP_Diplome_First_Person_Project_C|GetCinematic_Camera (Variables|Default|GetFirst_Person_0))))
            (Variables|Default|SetMay_Get_Out_Of_The_Minigame_? true)
            (Input|EnableInput (Game|GetPlayerController 0))
            (Collision|SetCollisionProfileName (Variables|Default|GetBox_Up_First_Roulette) "BlockAll" true :!class /Script/Engine.PrimitiveComponent)))
        (else
          (Default|CheckifAllPartition (Variables|Default|GetFirst_Person_0)))))
    (else
      (Default|TransmissDialogue (Variables|Default|GetFirst_Person_0) (Variables|Default|GetDialogue_If_Problem_?))
      (Utilities|FlowControl|Delay 2.0)
      (Default|EndDialogue (Variables|/Game/GD/ThirdPerson/Blueprints/BP_Diplome_First_Person_Project.BP_Diplome_First_Person_Project_C|GetHUD (Variables|Default|GetFirst_Person_0)))
      (Utilities|FlowControl|DoOnce false
        (:Completed
          (Utilities|FlowControl|DoOnce false
            (:Completed
              (Rendering|Components|TextRender|SetText (Variables|/Game/GD/Widget/HUD.HUD_C|GetHow_To_Show_Objective (Variables|/Game/GD/ThirdPerson/Blueprints/BP_Diplome_First_Person_Project.BP_Diplome_First_Person_Project_C|GetHUD (Variables|Default|GetFirst_Person_0))) "Objectif : Rappeler Cécile"))))))))

(event Input|MouseEvents|RightMouseButton
  (params (Key :type Key%20Structure :default "None"))
  (bind _first_person_0 (Variables|Default|GetFirst_Person_0))
  (bind _first_person_0_2 (Variables|Default|GetFirst_Person_0))
  (bind _first_person_0_3 (Variables|Default|GetFirst_Person_0))
  (:Pressed
    (if (Variables|Default|GetMay_Get_Out_Of_The_Minigame_?)
      (Variables|Default|SetMay_Get_Out_Of_The_Minigame_? false)
      (Variables|/Script/Engine.PlayerController|SetbShowMouseCursor (Game|GetPlayerController 0) false)
      (Variables|Default|SetCan_Be_Used_? false)
      (Collision|SetCollisionProfileName (Variables|Default|GetBox_Down_Fourth_Roulette) "NoCollision" true :!class /Script/Engine.PrimitiveComponent)
      (Collision|SetCollisionProfileName (Variables|Default|GetBox) "BlockAll" true :!class /Script/Engine.PrimitiveComponent)
      (bind _time_to_move_object (Timeline|Timeline_1 PlayFromStart)
        (:Update
          (Transformation|SetWorldTransform (Variables|/Game/GD/ThirdPerson/Blueprints/BP_Diplome_First_Person_Project.BP_Diplome_First_Person_Project_C|GetCinematic_Camera _first_person_0_3) (Math|Transform|Lerp(Transform) (Variables|Default|GetFollow_Camera_Transform) (Transformation|GetWorldTransform (Variables|/Game/GD/ThirdPerson/Blueprints/BP_Diplome_First_Person_Project.BP_Diplome_First_Person_Project_C|GetFirst_Person_Camera _first_person_0_3)) _time_to_move_object) false false))
        (:Finished
          (Components|Activation|SetActive (Variables|/Game/GD/ThirdPerson/Blueprints/BP_Diplome_First_Person_Project.BP_Diplome_First_Person_Project_C|GetCinematic_Camera _first_person_0) false false)
          (Components|Activation|SetActive (Variables|/Game/GD/ThirdPerson/Blueprints/BP_Diplome_First_Person_Project.BP_Diplome_First_Person_Project_C|GetFirst_Person_Camera _first_person_0) true false)
          (Variables|/Game/GD/ThirdPerson/Blueprints/BP_Diplome_First_Person_Project.BP_Diplome_First_Person_Project_C|SetInto_Minigame_? _first_person_0 false)
          (Input|DisableInput (Game|GetPlayerController 0))
          (Input|EnableInput _first_person_0_2 (Game|GetPlayerController 0))
          (Collision|SetCollisionProfileName (Variables|/Game/GD/ThirdPerson/Blueprints/BP_Diplome_First_Person_Project.BP_Diplome_First_Person_Project_C|GetHighlight_Detection _first_person_0_2) "OverlapAllDynamic" true :!class /Script/Engine.PrimitiveComponent))))))

(event Input|MouseEvents|LeftMouseButton
  (params (Key :type Key%20Structure :default "None"))
  (bind _returnvalue (Game|GetPlayerController 0))
  (bind _hitresult (Game|Player|GetHitResultUnderCursorbyChannel _returnvalue "TraceTypeQuery1" true))
  (bind _hitcomponent (Collision|BreakHitResult _hitresult))
  (:Released
    (if (== (Variables|Default|GetBox_Up_First_Roulette) _hitcomponent)
      (CallFunction|FirstWheelUp)
      (elif (== (Variables|Default|GetBox_Down_First_Roulette) _hitcomponent)
        (CallFunction|FirstWheelDown)
        (elif (== (Variables|Default|GetBox_Up_Second_Roulette) _hitcomponent)
          (CallFunction|SecondWheelUp)
          (elif (== (Variables|Default|GetBox_Down_Second_Roulette) _hitcomponent)
            (CallFunction|SecondWheelDown)
            (elif (== (Variables|Default|GetBox_Up_Third_Roulette) _hitcomponent)
              (CallFunction|ThirdWheelUp)
              (elif (== (Variables|Default|GetBox_Down_Third_Roulette) _hitcomponent)
                (CallFunction|ThirdWheelDown)
                (elif (== (Variables|Default|GetBox_Up_Fourth_Roulette) _hitcomponent)
                  (CallFunction|FourthWheelUp)
                  (elif (== (Variables|Default|GetBox_Down_Fourth_Roulette) _hitcomponent)
                    (CallFunction|FourthWheelDown)))))))))))

(fn ConstructionScript
  (|CallParentFunction))