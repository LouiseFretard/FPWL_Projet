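; Interactable drawer Blueprint that slides open and closed on alternate hits to its box, with a drawer sound.
; BeginPlay can swap the handle sphere for an item child actor and place a reward actor inside.
; A FlipFlop drives two timelines that lerp the Arrow component's relative location, enabling the reward's collision only while opening or open.
; Highlighting lazily creates an outline-material copy of the left-part mesh, then toggles its visibility.
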(event EventBeginPlay
  (bind _object_in_tiroir (Variables|Default|GetObject_In_Tiroir))
  (bind _reward (Variables|Default|GetReward))
  (|CallParentFunction)
  (if (and (== (Variables|Default|GetPoignee==Item_?) true) (== (Utilities|IsValidClass (Variables|Default|GetClass_Poignee)) true))
    (Development|SetHiddeninGame (Variables|Default|GetSphere) true false)
    (ChildActorComponent|SetChildActorClass (Variables|Default|GetItem_Poignee) (Variables|Default|GetClass_Poignee)))
  (if (Utilities|IsValidClass _reward)
    (ChildActorComponent|SetChildActorClass _object_in_tiroir _reward)
    (Collision|SetActorEnableCollision (Variables|/Script/Engine.ChildActorComponent|GetChildActor _object_in_tiroir) false)))

(event Collision|EventActorBeginOverlap
  (params (OtherActor :type Actor%20Object%20Reference))
  (|CallParentFunction OtherActor) ; This node is disabled and will not be called.\nDrag off pins to build functionality.
)

(event EventTick
  (params (DeltaSeconds :type Float%20%28single-precision%29))
  (|CallParentFunction DeltaSeconds) ; This node is disabled and will not be called.\nDrag off pins to build functionality.
)

(event EventPartHit
  (params (Hit_Component :type Primitive%20Component%20Object%20Reference) (Pawn :type Pawn%20Object%20Reference))
  (bind _object_in_tiroir (Variables|Default|GetObject_In_Tiroir))
  (bind _arrow (Variables|Default|GetArrow))
  (bind _object_in_tiroir_2 (Variables|Default|GetObject_In_Tiroir))
  (bind _childactor (Variables|/Script/Engine.ChildActorComponent|GetChildActor _object_in_tiroir_2))
  (bind _relativelocation (Variables|/Script/Engine.SceneComponent|GetRelativeLocation _arrow))
  (bind _childactor_2 (Variables|/Script/Engine.ChildActorComponent|GetChildActor _object_in_tiroir))
  (if (and (== Hit_Component (Variables|Default|GetBox)) (== (Variables|Default|GetIs_Moving_?) false))
    (Variables|Default|SetIs_Moving_? true)
    (Audio|SpawnSoundAttached "/Game/GD/Sound/Environment_Noise/SC_Drawer.SC_Drawer" (Variables|Default|GetArrow) "None" "0, 0, 0" "0, 0, 0" "SnapToTarget" false 1.0 1.0 0.0 0 0)
    (Utilities|FlowControl|FlipFlop
      (:A
        (Variables|Default|SetWhat_Direction_? "35.000000,0.000000, 0")
        (Utilities|IsValid _childactor_2
          (:Is%20Valid
            (Collision|SetActorEnableCollision _childactor_2 true)
            (bind _item_track (Timeline|Timeline_0 PlayFromStart)
              (:Update
                (Transformation|SetRelativeLocation _arrow (Math|Vector|Lerp(Vector) _relativelocation (Variables|Default|GetWhat_Direction_?) _item_track) false false))
              (:Finished
                (Variables|Default|SetIs_Moving_? false :!label _label))))
          (:Is%20Not%20Valid
            (Timeline|Timeline_0 PlayFromStart))))
      (:B
        (Variables|Default|SetWhat_Direction_? "-35.000000, 0, 0")
        (Utilities|IsValid _childactor
          (:Is%20Valid
            (Collision|SetActorEnableCollision _childactor false)
            (bind _item_track_2 (Timeline|Timeline_1 PlayFromStart)
              (:Update
                (Transformation|SetRelativeLocation _arrow (Math|Vector|Lerp(Vector) _relativelocation "0, 0, 0" _item_track_2) false false))
              (:Finished
                (goto _label))))
          (:Is%20Not%20Valid
            (Timeline|Timeline_1 PlayFromStart)))))))

(event EventOnHighlight
  (bind _tiroir_left_part (Variables|Default|GetTiroir_Left_Part))
  (Utilities|IsValid (Variables|Default|GetOutline_Mesh)
    (:Is%20Valid
      (Rendering|SetVisibility (Variables|Default|GetOutline_Mesh) true false))
    (:Is%20Not%20Valid
      (bind _returnvalue (AddComponent|AddStaticMeshComponent false (Math|Transform|MakeTransform (Variables|/Script/Engine.SceneComponent|GetRelativeLocation _tiroir_left_part) (Variables|/Script/Engine.SceneComponent|GetRelativeRotation _tiroir_left_part) (Transformation|GetWorldScale _tiroir_left_part))))
      (bind _output_get (Variables|Default|SetOutline_Mesh _returnvalue))
      (Components|StaticMesh|SetStaticMesh _output_get (Variables|/Script/Engine.StaticMeshComponent|GetStaticMesh _tiroir_left_part))
      (Rendering|Material|SetMaterial (Variables|Default|GetOutline_Mesh) 0 "/Game/GD/M_Test_Outline.M_Test_Outline")
      (Transformation|AttachComponentToComponent (Variables|Default|GetOutline_Mesh) _tiroir_left_part "None" "KeepWorld" "KeepWorld" "KeepWorld" true))))

(event EventStopHighlight
  (Utilities|IsValid (Variables|Default|GetOutline_Mesh)
    (:Is%20Valid
      (Rendering|SetVisibility (Variables|Default|GetOutline_Mesh) false false))))

(fn ConstructionScript
  (|CallParentFunction))