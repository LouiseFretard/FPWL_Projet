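; Combination-lock chest puzzle with five roulette dials that opens to give the player a reward.
; PartHit matches the hit component to a dial's up or down part, snaps that dial 45 degrees and wraps its counter between MinRoulette and MaxRoulette.
; Each turn checks a hard-coded combination; a match spawns Reward via a child actor, tilts the lid arrow open and disables collision.
; Timelines for smooth rotation exist but never run.
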(event Custom|Got_Right_Combination_?
  (bind _arrow_chest_open (Variables|Default|GetArrow_Chest_Open))
  (bind _relativerotation (Variables|/Script/Engine.SceneComponent|GetRelativeRotation _arrow_chest_open))
  (if (Math|Boolean|ANDBoolean (== (Variables|Default|GetHow_Many_Time_First_Roulettes_Rolled_?) 4.0) (== (Variables|Default|GetHow_Many_Time_Second_Roulette_Rolled_?) 0.0) (== (Variables|Default|GetHow_Many_Time_Third_Roulettes_Rolled_?) 2.0) (== (Variables|Default|GetHow_Many_Time_Fourth_Roulettes_Rolled_?) 5.0) (== (Variables|Default|GetHow_Many_Time_Fifth_Roulettes_Rolled_?) 5.0))
    (ChildActorComponent|SetChildActorClass (Variables|Default|GetReward_For_Player) (Variables|Default|GetReward))
    (Transformation|SetRelativeRotation _arrow_chest_open (Math|Rotator|MakeRotator (.roll _relativerotation) 45.0 (.yaw _relativerotation)) false false)
    (Collision|SetCollisionEnabled (Variables|Default|GetCube2) "NoCollision")))

(event EventBeginPlay
  (|CallParentFunction) ; This node is disabled and will not be called.\nDrag off pins to build functionality.
)

(event Collision|EventActorBeginOverlap
  (params (OtherActor :type Actor%20Object%20Reference))
  (|CallParentFunction OtherActor) ; This node is disabled and will not be called.\nDrag off pins to build functionality.
)

(event EventTick
  (params (DeltaSeconds :type Float%20%28single-precision%29))
  (|CallParentFunction DeltaSeconds) ; This node is disabled and will not be called.\nDrag off pins to build functionality.
)

(event EventPartHit
  (params (Hit_Component :type Primitive%20Component%20Object%20Reference))
  (bind _first_roulette (Variables|Default|GetFirst_Roulette))
  (bind _second_roulette (Variables|Default|GetSecond_Roulette))
  (bind _third_roulette (Variables|Default|GetThird_Roulette))
  (bind _second_roulette_2 (Variables|Default|GetSecond_Roulette))
  (bind _fifth_roulette (Variables|Default|GetFIfth_Roulette))
  (bind _fourth_roulette (Variables|Default|GetFourth_Roulette))
  (bind _third_roulette_2 (Variables|Default|GetThird_Roulette))
  (bind _fourth_roulette_2 (Variables|Default|GetFourth_Roulette))
  (bind _fifth_roulette_2 (Variables|Default|GetFIfth_Roulette))
  (bind _first_roulette_2 (Variables|Default|GetFirst_Roulette))
  (bind _relativerotation (Variables|/Script/Engine.SceneComponent|GetRelativeRotation _first_roulette))
  (bind _relativerotation_2 (Variables|/Script/Engine.SceneComponent|GetRelativeRotation _second_roulette_2))
  (bind _relativerotation_3 (Variables|/Script/Engine.SceneComponent|GetRelativeRotation _second_roulette))
  (bind _relativerotation_4 (Variables|/Script/Engine.SceneComponent|GetRelativeRotation _third_roulette_2))
  (bind _relativerotation_5 (Variables|/Script/Engine.SceneComponent|GetRelativeRotation _third_roulette))
  (bind _relativerotation_6 (Variables|/Script/Engine.SceneComponent|GetRelativeRotation _fourth_roulette_2))
  (bind _relativerotation_7 (Variables|/Script/Engine.SceneComponent|GetRelativeRotation _fourth_roulette))
  (bind _relativerotation_8 (Variables|/Script/Engine.SceneComponent|GetRelativeRotation _fifth_roulette_2))
  (bind _relativerotation_9 (Variables|/Script/Engine.SceneComponent|GetRelativeRotation _fifth_roulette))
  (bind _relativerotation_10 (Variables|/Script/Engine.SceneComponent|GetRelativeRotation _first_roulette_2))
  (if (and (== Hit_Component (Variables|Default|GetFirst_Roulette_Up)) (== (Variables|Default|GetFirst_Roulette_May_Turn_?) false))
    (Variables|Default|SetFirst_Roulette_May_Turn_? true)
    (if (> (+ (Variables|Default|GetHow_Many_Time_First_Roulettes_Rolled_?) 1.0) (Variables|Default|GetMax_Roulette))
      (Variables|Default|SetHow_Many_Time_First_Roulettes_Rolled_? (Variables|Default|GetMin_Roulette))
      (else
        (Variables|Default|SetHow_Many_Time_First_Roulettes_Rolled_? (+ (Variables|Default|GetHow_Many_Time_First_Roulettes_Rolled_?) 1.0))))
    (Transformation|SetRelativeRotation _first_roulette_2 (Math|Rotator|MakeRotator (+ (.roll _relativerotation_10) 45.0) (.pitch _relativerotation_10) (.yaw _relativerotation_10)) false false)
    (Variables|Default|SetFirst_Roulette_May_Turn_? false)
    (CallFunction|GotRightCombination?)
    (elif (and (== Hit_Component (Variables|Default|GetFirst_Roulette_Down)) (== (Variables|Default|GetFirst_Roulette_May_Turn_?) false))
      (Variables|Default|SetFirst_Roulette_May_Turn_? true)
      (if (< (- (Variables|Default|GetHow_Many_Time_First_Roulettes_Rolled_?) 1.0) (Variables|Default|GetMin_Roulette))
        (Variables|Default|SetHow_Many_Time_First_Roulettes_Rolled_? (Variables|Default|GetMax_Roulette))
        (else
          (Variables|Default|SetHow_Many_Time_First_Roulettes_Rolled_? (- (Variables|Default|GetHow_Many_Time_First_Roulettes_Rolled_?) 1.0))))
      (Transformation|SetRelativeRotation _first_roulette (Math|Rotator|MakeRotator (- (.roll _relativerotation) 45.0) (.pitch _relativerotation) (.yaw _relativerotation)) false false)
      (Variables|Default|SetFirst_Roulette_May_Turn_? false)
      (CallFunction|GotRightCombination?)
      (elif (and (== Hit_Component (Variables|Default|GetSecond_Roulette_Up)) (== (Variables|Default|GetSecond_Roulette_May_Turn_?) false))
        (Variables|Default|SetSecond_Roulette_May_Turn_? true)
        (if (> (+ (Variables|Default|GetHow_Many_Time_Second_Roulette_Rolled_?) 1.0) (Variables|Default|GetMax_Roulette))
          (Variables|Default|SetHow_Many_Time_Second_Roulette_Rolled_? (Variables|Default|GetMin_Roulette))
          (else
            (Variables|Default|SetHow_Many_Time_Second_Roulette_Rolled_? (+ (Variables|Default|GetHow_Many_Time_Second_Roulette_Rolled_?) 1.0))))
        (Transformation|SetRelativeRotation _second_roulette_2 (Math|Rotator|MakeRotator (+ (.roll _relativerotation_2) 45.0) (.pitch _relativerotation_2) (.yaw _relativerotation_2)) false false)
        (Variables|Default|SetSecond_Roulette_May_Turn_? false)
        (CallFunction|GotRightCombination?)
        (elif (and (== Hit_Component (Variables|Default|GetSecond_Roulette_Down)) (== (Variables|Default|GetSecond_Roulette_May_Turn_?) false))
          (Variables|Default|SetSecond_Roulette_May_Turn_? true)
          (if (< (- (Variables|Default|GetHow_Many_Time_Second_Roulette_Rolled_?) 1.0) (Variables|Default|GetMin_Roulette))
            (Variables|Default|SetHow_Many_Time_Second_Roulette_Rolled_? (Variables|Default|GetMax_Roulette))
            (else
              (Variables|Default|SetHow_Many_Time_Second_Roulette_Rolled_? (- (Variables|Default|GetHow_Many_Time_Second_Roulette_Rolled_?) 1.0))))
          (Transformation|SetRelativeRotation _second_roulette (Math|Rotator|MakeRotator (- (.roll _relativerotation_3) 45.0) (.pitch _relativerotation_3) (.yaw _relativerotation_3)) false false)
          (Variables|Default|SetSecond_Roulette_May_Turn_? false)
          (CallFunction|GotRightCombination?)
          (elif (and (== Hit_Component (Variables|Default|GetThird_Roulette_Up)) (== (Variables|Default|GetThird_Roulette_May_Turn_?) false))
            (Variables|Default|SetThird_Roulette_May_Turn_? true)
            (if (> (+ (Variables|Default|GetHow_Many_Time_Third_Roulettes_Rolled_?) 1.0) (Variables|Default|GetMax_Roulette))
              (Variables|Default|SetHow_Many_Time_Third_Roulettes_Rolled_? (Variables|Default|GetMin_Roulette))
              (else
                (Variables|Default|SetHow_Many_Time_Third_Roulettes_Rolled_? (+ (Variables|Default|GetHow_Many_Time_Third_Roulettes_Rolled_?) 1.0))))
            (Transformation|SetRelativeRotation _third_roulette_2 (Math|Rotator|MakeRotator (+ (.roll _relativerotation_4) 45.0) (.pitch _relativerotation_4) (.yaw _relativerotation_4)) false false)
            (Variables|Default|SetThird_Roulette_May_Turn_? false)
            (CallFunction|GotRightCombination?)
            (elif (and (== Hit_Component (Variables|Default|GetThird_Roulette_Down)) (== (Variables|Default|GetThird_Roulette_May_Turn_?) false))
              (Variables|Default|SetThird_Roulette_May_Turn_? true)
              (if (< (- (Variables|Default|GetHow_Many_Time_Third_Roulettes_Rolled_?) 1.0) (Variables|Default|GetMin_Roulette))
                (Variables|Default|SetHow_Many_Time_Third_Roulettes_Rolled_? (Variables|Default|GetMax_Roulette))
                (else
                  (Variables|Default|SetHow_Many_Time_Third_Roulettes_Rolled_? (- (Variables|Default|GetHow_Many_Time_Third_Roulettes_Rolled_?) 1.0))))
              (Transformation|SetRelativeRotation _third_roulette (Math|Rotator|MakeRotator (- (.roll _relativerotation_5) 45.0) (.pitch _relativerotation_5) (.yaw _relativerotation_5)) false false)
              (Variables|Default|SetThird_Roulette_May_Turn_? false)
              (CallFunction|GotRightCombination?)
              (elif (and (== Hit_Component (Variables|Default|GetFourth_Roulette_Up)) (== (Variables|Default|GetFourth_Roulette_May_Turn_?) false))
                (Variables|Default|SetFourth_Roulette_May_Turn_? true)
                (if (> (+ (Variables|Default|GetHow_Many_Time_Fourth_Roulettes_Rolled_?) 1.0) (Variables|Default|GetMax_Roulette))
                  (Variables|Default|SetHow_Many_Time_Fourth_Roulettes_Rolled_? (Variables|Default|GetMin_Roulette))
                  (else
                    (Variables|Default|SetHow_Many_Time_Fourth_Roulettes_Rolled_? (+ (Variables|Default|GetHow_Many_Time_Fourth_Roulettes_Rolled_?) 1.0))))
                (Transformation|SetRelativeRotation _fourth_roulette_2 (Math|Rotator|MakeRotator (+ (.roll _relativerotation_6) 45.0) (.pitch _relativerotation_6) (.yaw _relativerotation_6)) false false)
                (Variables|Default|SetFourth_Roulette_May_Turn_? false)
                (CallFunction|GotRightCombination?)
                (elif (and (== Hit_Component (Variables|Default|GetFourth_Roulette_Down)) (== (Variables|Default|GetFourth_Roulette_May_Turn_?) false))
                  (Variables|Default|SetFourth_Roulette_May_Turn_? true)
                  (if (< (- (Variables|Default|GetHow_Many_Time_Fourth_Roulettes_Rolled_?) 1.0) (Variables|Default|GetMin_Roulette))
                    (Variables|Default|SetHow_Many_Time_Fourth_Roulettes_Rolled_? (Variables|Default|GetMax_Roulette))
                    (else
                      (Variables|Default|SetHow_Many_Time_Fourth_Roulettes_Rolled_? (- (Variables|Default|GetHow_Many_Time_Fourth_Roulettes_Rolled_?) 1.0))))
                  (Transformation|SetRelativeRotation _fourth_roulette (Math|Rotator|MakeRotator (- (.roll _relativerotation_7) 45.0) (.pitch _relativerotation_7) (.yaw _relativerotation_7)) false false)
                  (Variables|Default|SetFourth_Roulette_May_Turn_? false)
                  (CallFunction|GotRightCombination?)
                  (elif (and (== Hit_Component (Variables|Default|GetFifth_Roulette_Up)) (== (Variables|Default|GetFifth_Roulette_May_Turn_?) false))
                    (Variables|Default|SetFifth_Roulette_May_Turn_? true)
                    (if (> (+ (Variables|Default|GetHow_Many_Time_Fifth_Roulettes_Rolled_?) 1.0) (Variables|Default|GetMax_Roulette))
                      (Variables|Default|SetHow_Many_Time_Fifth_Roulettes_Rolled_? (Variables|Default|GetMin_Roulette))
                      (else
                        (Variables|Default|SetHow_Many_Time_Fifth_Roulettes_Rolled_? (+ (Variables|Default|GetHow_Many_Time_Fifth_Roulettes_Rolled_?) 1.0))))
                    (Transformation|SetRelativeRotation _fifth_roulette_2 (Math|Rotator|MakeRotator (+ (.roll _relativerotation_8) 45.0) (.pitch _relativerotation_8) (.yaw _relativerotation_8)) false false)
                    (Variables|Default|SetFifth_Roulette_May_Turn_? false)
                    (CallFunction|GotRightCombination?)
                    (elif (and (== Hit_Component (Variables|Default|GetFifth_Roulette_Down)) (== (Variables|Default|GetFifth_Roulette_May_Turn_?) false))
                      (Variables|Default|SetFifth_Roulette_May_Turn_? true)
                      (if (< (- (Variables|Default|GetHow_Many_Time_Fifth_Roulettes_Rolled_?) 1.0) (Variables|Default|GetMin_Roulette))
                        (Variables|Default|SetHow_Many_Time_Fifth_Roulettes_Rolled_? (Variables|Default|GetMax_Roulette))
                        (else
                          (Variables|Default|SetHow_Many_Time_Fifth_Roulettes_Rolled_? (- (Variables|Default|GetHow_Many_Time_Fifth_Roulettes_Rolled_?) 1.0))))
                      (Transformation|SetRelativeRotation _fifth_roulette (Math|Rotator|MakeRotator (- (.roll _relativerotation_9) 45.0) (.pitch _relativerotation_9) (.yaw _relativerotation_9)) false false)
                      (Variables|Default|SetFifth_Roulette_May_Turn_? false)
                      (CallFunction|GotRightCombination?))))))))))))

(fn ConstructionScript
  (|CallParentFunction))