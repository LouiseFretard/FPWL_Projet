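; Interactable radio tuning minigame that, once solved, spawns a reward and starts the breakable statue.
; A hit blends the cinematic camera to the radio for mouse play; right-click exits.
; Two clickable knobs step an oscilloscope material's amplitude and frequency toward reference values, crossfading interference into music until both match.
; Start_Radio enables the initially inactive radio, while separate events sequence Morse letter sounds and highlight events toggle a material parameter.
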(event Custom|Got_Right_Combination_?
  (bind _returnvalue (Game|GetPlayerController 0))
  (bind _first_person_0 (Variables|Default|GetFirst_Person_0))
  (bind _dynamic_material (Variables|Default|GetDynamic_Material))
  (bind _first_person_0_2 (Variables|Default|GetFirst_Person_0))
  (bind _dynamic_material_2 (Variables|Default|GetDynamic_Material))
  (bind _returnvalue_2 (Rendering|Material|GetScalarParameterValue _dynamic_material_2 "Amplitude_Ref" :!class /Script/Engine.MaterialInstanceDynamic))
  (bind _returnvalue_3 (Rendering|Material|GetScalarParameterValue _dynamic_material_2 "Amplitude" :!class /Script/Engine.MaterialInstanceDynamic))
  (bind _returnvalue_4 (Rendering|Material|GetScalarParameterValue _dynamic_material "Frequence_Ref" :!class /Script/Engine.MaterialInstanceDynamic))
  (bind _returnvalue_5 (Rendering|Material|GetScalarParameterValue _dynamic_material "Frequence" :!class /Script/Engine.MaterialInstanceDynamic))
  (if (and (== (Math|Float|NearlyEqual(Float) _returnvalue_3 _returnvalue_2 1e-06) true) (== (Math|Float|NearlyEqual(Float) _returnvalue_5 _returnvalue_4 1e-06) true))
    (Audio|Components|Audio|Stop (Variables|Default|GetInterference_Sound))
    (Input|DisableInput (Game|GetPlayerController 0))
    (Audio|Components|Audio|SetVolumeMultiplier (Variables|Default|GetGood_Sound) 1.0 :!class /Script/Engine.AudioComponent)
    (ChildActorComponent|SetChildActorClass (Variables|Default|GetReward_For_Player) (Variables|Default|GetReward))
    (Collision|SetCollisionEnabled (Variables|Default|GetStaticMesh6) "NoCollision")
    (bind _time_to_move_object (Timeline|Timeline_2 PlayFromStart)
      (:Update
        (Transformation|SetRelativeLocation (Variables|Default|GetStaticMesh6) (Math|Vector|Lerp(Vector) "15.000000,-11.000000,-2.000000" "40.000000,-11.000000,-2.000000" _time_to_move_object) false false))
      (:Finished
        (Variables|Default|SetMay_Get_Out_Of_The_Minigame_? false)
        (Variables|/Script/Engine.PlayerController|SetbShowMouseCursor (Game|GetPlayerController 0) false)
        (Collision|SetActorEnableCollision self false)
        (bind _returnvalue_6 (Actor|GetActorOfClass "/Game/GD/Interactainable/Object_Interactable_But_Not_Inspectable_And_Need_Object/BP_Statue_Which_Will_Be_Broken_Child_INI.BP_Statue_Which_Will_Be_Broken_Child_INI_C"))
        (Default|StartStatue _returnvalue_6)
        (Collision|SetCollisionProfileName (Variables|Default|GetBox2) "NoCollision" true :!class /Script/Engine.PrimitiveComponent)
        (bind _time_to_move_object_2 (Timeline|Timeline_1 PlayFromStart)
          (:Update
            (Transformation|SetWorldTransform (Variables|/Game/GD/ThirdPerson/Blueprints/BP_Diplome_First_Person_Project.BP_Diplome_First_Person_Project_C|GetCinematic_Camera _first_person_0_2) (Math|Transform|Lerp(Transform) (Variables|Default|GetFollow_Camera_Transform) (Transformation|GetWorldTransform (Variables|/Game/GD/ThirdPerson/Blueprints/BP_Diplome_First_Person_Project.BP_Diplome_First_Person_Project_C|GetFirst_Person_Camera _first_person_0_2)) _time_to_move_object_2) false false))
          (:Finished
            (Components|Activation|SetActive (Variables|/Game/GD/ThirdPerson/Blueprints/BP_Diplome_First_Person_Project.BP_Diplome_First_Person_Project_C|GetCinematic_Camera _first_person_0) false false)
            (Components|Activation|SetActive (Variables|/Game/GD/ThirdPerson/Blueprints/BP_Diplome_First_Person_Project.BP_Diplome_First_Person_Project_C|GetFirst_Person_Camera _first_person_0) true false)
            (Variables|/Game/GD/ThirdPerson/Blueprints/BP_Diplome_First_Person_Project.BP_Diplome_First_Person_Project_C|SetInto_Minigame_? _first_person_0 false)
            (Input|DisableInput _returnvalue)
            (Input|EnableInput (Variables|Default|GetFirst_Person_0) _returnvalue)
            (Collision|SetCollisionProfileName (Variables|Default|GetBox) "BlockAll" true :!class /Script/Engine.PrimitiveComponent)))))
    (else
      (Variables|Default|SetFirst_Button_May_Turn_? false)
      (Variables|Default|SetSecond_Button_May_Turn_? false))))

(event Custom|Start_Radio
  (Audio|Components|Audio|SetVolumeMultiplier (Variables|Default|GetInterference_Sound) 1.0 :!class /Script/Engine.AudioComponent)
  (Collision|SetActorEnableCollision self true))

(event Custom|Fifth_Letter_Morse
  (Components|DestroyComponent (stale Custom|Fourth_Letter_Morse _returnvalue))
  (Utilities|FlowControl|Delay 0.2)
  (bind _returnvalue (Audio|SpawnSoundatLocation "/Game/GD/Sound/Environment_Noise/Morse_Sound/SC_Morse_S_Cue.SC_Morse_S_Cue" (Transformation|GetWorldLocation (Variables|Default|GetStaticMesh)) "0, 0, 0" 0.0 1.0 0.0 0 0 false)))

(event Custom|Sixth_Letter_Morse
  (Components|DestroyComponent (stale Custom|Fifth_Letter_Morse _returnvalue))
  (Utilities|FlowControl|Delay 0.2)
  (bind _returnvalue (Audio|SpawnSoundatLocation "/Game/GD/Sound/Cobra-DVD-Menu.Cobra-DVD-Menu" (Transformation|GetWorldLocation (Variables|Default|GetStaticMesh)) "0, 0, 0" 0.0 1.0 0.0 0 0 false)))

(event Custom|First_Button_Left
  (bind _interference_sound (Variables|Default|GetInterference_Sound))
  (bind _good_sound (Variables|Default|GetGood_Sound))
  (bind _interference_sound_2 (Variables|Default|GetInterference_Sound))
  (bind _good_sound_2 (Variables|Default|GetGood_Sound))
  (bind _returnvalue (Rendering|Material|GetScalarParameterValue (Variables|Default|GetDynamic_Material) "Amplitude" :!class /Script/Engine.MaterialInstanceDynamic))
  (Variables|Default|SetOriginal_Parameter_Value _returnvalue)
  (if (> _returnvalue 0.2)
    (if (not (Variables|Default|GetFirst_Button_May_Turn_?))
      (Variables|Default|SetFirst_Button_May_Turn_? true)
      (Variables|Default|SetFirst_Button_Relative_Rotation (Variables|/Script/Engine.SceneComponent|GetRelativeRotation (Variables|Default|GetFirst_Button)))
      (bind _item_track (Timeline|Timeline_4 PlayFromStart)
        (:Update
          (Rendering|Material|SetScalarParameterValue (Variables|Default|GetDynamic_Material) "Amplitude" (Math|Float|Lerp (Variables|Default|GetOriginal_Parameter_Value) (+ (Variables|Default|GetOriginal_Parameter_Value) -0.1) _item_track) :!class /Script/Engine.MaterialInstanceDynamic)
          (Transformation|SetRelativeRotation (Variables|Default|GetFirst_Button) (Math|Rotator|Lerp(Rotator) (Variables|Default|GetFirst_Button_Relative_Rotation) (Math|Rotator|CombineRotators (Variables|Default|GetFirst_Button_Relative_Rotation) (Math|Vector|RotatorfromAxisandAngle "1.000000, 0, 0" -36.0)) _item_track true) false false))
        (:Finished
          (bind _returnvalue_2 (Rendering|Material|GetScalarParameterValue (Variables|Default|GetDynamic_Material) "Amplitude_Ref" :!class /Script/Engine.MaterialInstanceDynamic))
          (if (>= _returnvalue _returnvalue_2)
            (Audio|Components|Audio|SetVolumeMultiplier _interference_sound (+ (Variables|/Script/Engine.AudioComponent|GetVolumeMultiplier _interference_sound) -0.0375) :!class /Script/Engine.AudioComponent)
            (Audio|Components|Audio|SetVolumeMultiplier _good_sound (+ (Variables|/Script/Engine.AudioComponent|GetVolumeMultiplier _good_sound) 0.0375) :!class /Script/Engine.AudioComponent)
            (else
              (Audio|Components|Audio|SetVolumeMultiplier _interference_sound_2 (+ (Variables|/Script/Engine.AudioComponent|GetVolumeMultiplier _interference_sound_2) 0.0375) :!class /Script/Engine.AudioComponent)
              (Audio|Components|Audio|SetVolumeMultiplier _good_sound_2 (+ (Variables|/Script/Engine.AudioComponent|GetVolumeMultiplier _good_sound_2) -0.0375) :!class /Script/Engine.AudioComponent)))
          (CallFunction|GotRightCombination?))))))

(event Custom|First_Button_Right
  (bind _good_sound (Variables|Default|GetGood_Sound))
  (bind _interference_sound (Variables|Default|GetInterference_Sound))
  (bind _interference_sound_2 (Variables|Default|GetInterference_Sound))
  (bind _good_sound_2 (Variables|Default|GetGood_Sound))
  (bind _returnvalue (Rendering|Material|GetScalarParameterValue (Variables|Default|GetDynamic_Material) "Amplitude" :!class /Script/Engine.MaterialInstanceDynamic))
  (Variables|Default|SetOriginal_Parameter_Value _returnvalue)
  (if (< _returnvalue 0.9)
    (Variables|Default|SetFirst_Button_Relative_Rotation (Variables|/Script/Engine.SceneComponent|GetRelativeRotation (Variables|Default|GetFirst_Button)))
    (if (not (Variables|Default|GetFirst_Button_May_Turn_?))
      (Variables|Default|SetFirst_Button_May_Turn_? true)
      (bind _item_track (Timeline|Timeline_3 PlayFromStart)
        (:Update
          (Rendering|Material|SetScalarParameterValue (Variables|Default|GetDynamic_Material) "Amplitude" (Math|Float|Lerp (Variables|Default|GetOriginal_Parameter_Value) (+ (Variables|Default|GetOriginal_Parameter_Value) 0.1) _item_track) :!class /Script/Engine.MaterialInstanceDynamic)
          (Transformation|SetRelativeRotation (Variables|Default|GetFirst_Button) (Math|Rotator|Lerp(Rotator) (Variables|Default|GetFirst_Button_Relative_Rotation) (Math|Rotator|CombineRotators (Variables|Default|GetFirst_Button_Relative_Rotation) (Math|Vector|RotatorfromAxisandAngle "1.000000, 0, 0" 36.0)) _item_track true) false false))
        (:Finished
          (bind _returnvalue_2 (Rendering|Material|GetScalarParameterValue (Variables|Default|GetDynamic_Material) "Amplitude_Ref" :!class /Script/Engine.MaterialInstanceDynamic))
          (if (<= _returnvalue _returnvalue_2)
            (Audio|Components|Audio|SetVolumeMultiplier _interference_sound_2 (+ (Variables|/Script/Engine.AudioComponent|GetVolumeMultiplier _interference_sound_2) -0.0375) :!class /Script/Engine.AudioComponent)
            (Audio|Components|Audio|SetVolumeMultiplier _good_sound_2 (+ (Variables|/Script/Engine.AudioComponent|GetVolumeMultiplier _good_sound_2) 0.0375) :!class /Script/Engine.AudioComponent)
            (else
              (Audio|Components|Audio|SetVolumeMultiplier _interference_sound (+ (Variables|/Script/Engine.AudioComponent|GetVolumeMultiplier _interference_sound) 0.0375) :!class /Script/Engine.AudioComponent)
              (Audio|Components|Audio|SetVolumeMultiplier _good_sound (+ (Variables|/Script/Engine.AudioComponent|GetVolumeMultiplier _good_sound) -0.0375) :!class /Script/Engine.AudioComponent)))
          (CallFunction|GotRightCombination?))))))

(event Custom|End_Morse
  (Components|DestroyComponent (stale Custom|Sixth_Letter_Morse _returnvalue)))

(event Custom|Second_Button_Left
  (bind _interference_sound (Variables|Default|GetInterference_Sound))
  (bind _good_sound (Variables|Default|GetGood_Sound))
  (bind _interference_sound_2 (Variables|Default|GetInterference_Sound))
  (bind _good_sound_2 (Variables|Default|GetGood_Sound))
  (bind _returnvalue (Rendering|Material|GetScalarParameterValue (Variables|Default|GetDynamic_Material) "Frequence" :!class /Script/Engine.MaterialInstanceDynamic))
  (Variables|Default|SetOriginal_Parameter_Value _returnvalue)
  (if (> _returnvalue 1.0)
    (Variables|Default|SetSecond_Button_Relative_Rotation (Variables|/Script/Engine.SceneComponent|GetRelativeRotation (Variables|Default|GetSecond_Button)))
    (if (not (Variables|Default|GetSecond_Button_May_Turn_?))
      (Variables|Default|SetSecond_Button_May_Turn_? true)
      (bind _item_track (Timeline|Timeline_6 PlayFromStart)
        (:Update
          (Rendering|Material|SetScalarParameterValue (Variables|Default|GetDynamic_Material) "Frequence" (Math|Float|Lerp (Variables|Default|GetOriginal_Parameter_Value) (+ (Variables|Default|GetOriginal_Parameter_Value) -0.1) _item_track) :!class /Script/Engine.MaterialInstanceDynamic)
          (Transformation|SetRelativeRotation (Variables|Default|GetSecond_Button) (Math|Rotator|Lerp(Rotator) (Variables|Default|GetSecond_Button_Relative_Rotation) (Math|Rotator|CombineRotators (Variables|Default|GetSecond_Button_Relative_Rotation) (Math|Vector|RotatorfromAxisandAngle "1.000000, 0, 0" -36.0)) _item_track true) false false))
        (:Finished
          (bind _returnvalue_2 (Rendering|Material|GetScalarParameterValue (Variables|Default|GetDynamic_Material) "Frequence_Ref" :!class /Script/Engine.MaterialInstanceDynamic))
          (if (>= _returnvalue _returnvalue_2)
            (Audio|Components|Audio|SetVolumeMultiplier _interference_sound (+ (Variables|/Script/Engine.AudioComponent|GetVolumeMultiplier _interference_sound) -0.0625) :!class /Script/Engine.AudioComponent)
            (Audio|Components|Audio|SetVolumeMultiplier _good_sound (+ (Variables|/Script/Engine.AudioComponent|GetVolumeMultiplier _good_sound) 0.0625) :!class /Script/Engine.AudioComponent)
            (else
              (Audio|Components|Audio|SetVolumeMultiplier _interference_sound_2 (+ (Variables|/Script/Engine.AudioComponent|GetVolumeMultiplier _interference_sound_2) 0.0625) :!class /Script/Engine.AudioComponent)
              (Audio|Components|Audio|SetVolumeMultiplier _good_sound_2 (+ (Variables|/Script/Engine.AudioComponent|GetVolumeMultiplier _good_sound_2) -0.0625) :!class /Script/Engine.AudioComponent)))
          (CallFunction|GotRightCombination?))))))

(event Custom|Second_Button_Right
  (bind _interference_sound (Variables|Default|GetInterference_Sound))
  (bind _good_sound (Variables|Default|GetGood_Sound))
  (bind _interference_sound_2 (Variables|Default|GetInterference_Sound))
  (bind _good_sound_2 (Variables|Default|GetGood_Sound))
  (bind _returnvalue (Rendering|Material|GetScalarParameterValue (Variables|Default|GetDynamic_Material) "Frequence" :!class /Script/Engine.MaterialInstanceDynamic))
  (Variables|Default|SetOriginal_Parameter_Value _returnvalue)
  (if (< _returnvalue 3.0)
    (Variables|Default|SetSecond_Button_Relative_Rotation (Variables|/Script/Engine.SceneComponent|GetRelativeRotation (Variables|Default|GetSecond_Button)))
    (if (not (Variables|Default|GetSecond_Button_May_Turn_?))
      (Variables|Default|SetSecond_Button_May_Turn_? true)
      (bind _item_track (Timeline|Timeline_5 PlayFromStart)
        (:Update
          (Rendering|Material|SetScalarParameterValue (Variables|Default|GetDynamic_Material) "Frequence" (Math|Float|Lerp (Variables|Default|GetOriginal_Parameter_Value) (+ (Variables|Default|GetOriginal_Parameter_Value) 0.1) _item_track) :!class /Script/Engine.MaterialInstanceDynamic)
          (Transformation|SetRelativeRotation (Variables|Default|GetSecond_Button) (Math|Rotator|Lerp(Rotator) (Variables|Default|GetSecond_Button_Relative_Rotation) (Math|Rotator|CombineRotators (Variables|Default|GetSecond_Button_Relative_Rotation) (Math|Vector|RotatorfromAxisandAngle "1.000000, 0, 0" 36.0)) _item_track true) false false))
        (:Finished
          (bind _returnvalue_2 (Rendering|Material|GetScalarParameterValue (Variables|Default|GetDynamic_Material) "Frequence_Ref" :!class /Script/Engine.MaterialInstanceDynamic))
          (if (<= _returnvalue _returnvalue_2)
            (Audio|Components|Audio|SetVolumeMultiplier _interference_sound (+ (Variables|/Script/Engine.AudioComponent|GetVolumeMultiplier _interference_sound) -0.0625) :!class /Script/Engine.AudioComponent)
            (Audio|Components|Audio|SetVolumeMultiplier _good_sound (+ (Variables|/Script/Engine.AudioComponent|GetVolumeMultiplier _good_sound) 0.0625) :!class /Script/Engine.AudioComponent)
            (else
              (Audio|Components|Audio|SetVolumeMultiplier _interference_sound_2 (+ (Variables|/Script/Engine.AudioComponent|GetVolumeMultiplier _interference_sound_2) 0.0625) :!class /Script/Engine.AudioComponent)
              (Audio|Components|Audio|SetVolumeMultiplier _good_sound_2 (+ (Variables|/Script/Engine.AudioComponent|GetVolumeMultiplier _good_sound_2) -0.0625) :!class /Script/Engine.AudioComponent)))
          (CallFunction|GotRightCombination?))))))

(event Custom|Turn_A_Wheel)

(event Custom|Start_Morse
  (Audio|Components|Audio|SetVolumeMultiplier (Variables|Default|GetGood_Sound) 0.0 :!class /Script/Engine.AudioComponent)
  (bind _returnvalue (Audio|SpawnSoundatLocation "/Game/GD/Sound/Environment_Noise/Morse_Sound/SC_Morse_U_Cue.SC_Morse_U_Cue" (Transformation|GetWorldLocation (Variables|Default|GetStaticMesh)) "0, 0, 0" 0.0 1.0 0.0 0 0 false)))

(event Custom|Second_Letter_Morse
  (Components|DestroyComponent (stale Custom|Start_Morse _returnvalue))
  (Utilities|FlowControl|Delay 0.2)
  (bind _returnvalue (Audio|SpawnSoundatLocation "/Game/GD/Sound/Environment_Noise/Morse_Sound/Sc_Morse_L_Cue.Sc_Morse_L_Cue" (Transformation|GetWorldLocation (Variables|Default|GetStaticMesh)) "0, 0, 0" 0.0 1.0 0.0 0 0 false)))

(event Custom|Third_Letter_Morse
  (Components|DestroyComponent (stale Custom|Second_Letter_Morse _returnvalue))
  (Utilities|FlowControl|Delay 0.2)
  (bind _returnvalue (Audio|SpawnSoundatLocation "/Game/GD/Sound/Environment_Noise/Morse_Sound/SC_Morse_Y_Cue.SC_Morse_Y_Cue" (Transformation|GetWorldLocation (Variables|Default|GetStaticMesh)) "0, 0, 0" 0.0 1.0 0.0 0 0 false)))

(event Custom|Fourth_Letter_Morse
  (Components|DestroyComponent (stale Custom|Third_Letter_Morse _returnvalue))
  (Utilities|FlowControl|Delay 0.2)
  (bind _returnvalue (Audio|SpawnSoundatLocation "/Game/GD/Sound/Environment_Noise/Morse_Sound/SC_Morse_S_Cue.SC_Morse_S_Cue" (Transformation|GetWorldLocation (Variables|Default|GetStaticMesh)) "0, 0, 0" 0.0 1.0 0.0 0 0 false)))

(event EventStopHighlight
  (Rendering|Material|SetScalarParameterValue (Variables|Default|GetM_inst) "Activate" 0.0 :!class /Script/Engine.MaterialInstanceDynamic))

(event Collision|EventActorBeginOverlap
  (params (OtherActor :type Actor%20Object%20Reference))
  (|CallParentFunction OtherActor) ; This node is disabled and will not be called.\nDrag off pins to build functionality.
)

(event EventOnHighlight
  (Rendering|Material|SetScalarParameterValue (Variables|Default|GetM_inst) "Activate" 1.0 :!class /Script/Engine.MaterialInstanceDynamic))

(event EventPartHit
  (params (Hit_Component :type Primitive%20Component%20Object%20Reference) (Pawn :type Pawn%20Object%20Reference))
  (bind _asbp_diplome_first_person_project (Utilities|Casting|CastToBP_Diplome_First_Person_Project Pawn))
  (Utilities|IsValid (Variables|Default|GetFirst_Person_0)
    (:Is%20Valid
      _)
    (:Is%20Not%20Valid
      (Variables|Default|SetFirst_Person_0 _asbp_diplome_first_person_project)))
  (if (== Hit_Component (Variables|Default|GetBox))
    (Input|DisableInput (Variables|Default|GetFirst_Person_0) (Game|GetPlayerController 0))
    (Collision|SetCollisionProfileName (Variables|Default|GetBox) "NoCollision" true :!class /Script/Engine.PrimitiveComponent)
    (Variables|/Game/GD/ThirdPerson/Blueprints/BP_Diplome_First_Person_Project.BP_Diplome_First_Person_Project_C|SetInto_Minigame_? (Variables|Default|GetFirst_Person_0) true)
    (Variables|/Script/Engine.PlayerController|SetbShowMouseCursor (Game|GetPlayerController 0) true)
    (Collision|SetCollisionProfileName (Variables|Default|GetBox) "None" true :!class /Script/Engine.PrimitiveComponent)
    (Transformation|SetWorldTransform (Variables|/Game/GD/ThirdPerson/Blueprints/BP_Diplome_First_Person_Project.BP_Diplome_First_Person_Project_C|GetCinematic_Camera (Variables|Default|GetFirst_Person_0)) (Transformation|GetWorldTransform (Variables|/Game/GD/ThirdPerson/Blueprints/BP_Diplome_First_Person_Project.BP_Diplome_First_Person_Project_C|GetFirst_Person_Camera (Variables|Default|GetFirst_Person_0))) false false)
    (Variables|Default|SetFollow_Camera_Transform (Transformation|GetWorldTransform (Variables|/Game/GD/ThirdPerson/Blueprints/BP_Diplome_First_Person_Project.BP_Diplome_First_Person_Project_C|GetCinematic_Camera (Variables|Default|GetFirst_Person_0))))
    (Components|Activation|SetActive (Variables|/Game/GD/ThirdPerson/Blueprints/BP_Diplome_First_Person_Project.BP_Diplome_First_Person_Project_C|GetCinematic_Camera (Variables|Default|GetFirst_Person_0)) true false)
    (Components|Activation|SetActive (Variables|/Game/GD/ThirdPerson/Blueprints/BP_Diplome_First_Person_Project.BP_Diplome_First_Person_Project_C|GetFirst_Person_Camera (Variables|Default|GetFirst_Person_0)) false false)
    (bind _time_to_move_object (Timeline|Timeline_0 PlayFromStart)
      (:Update
        (Transformation|SetWorldTransform (Variables|/Game/GD/ThirdPerson/Blueprints/BP_Diplome_First_Person_Project.BP_Diplome_First_Person_Project_C|GetCinematic_Camera (Variables|Default|GetFirst_Person_0)) (Math|Transform|Lerp(Transform) (Variables|Default|GetFollow_Camera_Transform) (Transformation|GetWorldTransform (Variables|Default|GetCube6)) _time_to_move_object) false false))
      (:Finished
        (Variables|Default|SetFollow_Camera_Transform (Transformation|GetWorldTransform (Variables|/Game/GD/ThirdPerson/Blueprints/BP_Diplome_First_Person_Project.BP_Diplome_First_Person_Project_C|GetCinematic_Camera (Variables|Default|GetFirst_Person_0))))
        (Variables|Default|SetMay_Get_Out_Of_The_Minigame_? true)
        (Input|EnableInput (Game|GetPlayerController 0))
        (Collision|SetCollisionProfileName (Variables|Default|GetBox2) "BlockAll" true :!class /Script/Engine.PrimitiveComponent)))))

(event EventBeginPlay
  (bind _staticmesh (Variables|Default|GetStaticMesh))
  (bind _returnvalue (Rendering|Material|CreateDynamicMaterialInstance "/Game/TA/Materials/Gameplay/Maison/Radio.Radio" "None" "None" :!class /Script/Engine.KismetMaterialLibrary))
  (bind _output_get (Variables|Default|SetM_inst _returnvalue))
  (Rendering|Material|SetMaterial (Variables|Default|GetStaticMesh) 0 _output_get)
  (Rendering|Material|SetScalarParameterValue (Variables|Default|GetM_inst) "Activate" 0.0 :!class /Script/Engine.MaterialInstanceDynamic)
  (Variables|Default|SetFirst_Button_Relative_Rotation (Variables|/Script/Engine.SceneComponent|GetRelativeRotation (Variables|Default|GetFirst_Button)))
  (Variables|Default|SetSecond_Button_Relative_Rotation (Variables|/Script/Engine.SceneComponent|GetRelativeRotation (Variables|Default|GetSecond_Button)))
  (Collision|SetActorEnableCollision self false)
  (bind _returnvalue_2 (Audio|SpawnSoundatLocation "/Game/GD/Sound/Environment_Noise/SC_Radio_Interference_Cue.SC_Radio_Interference_Cue" (Transformation|GetWorldLocation (Variables|Default|GetStaticMesh)) "0, 0, 0" 0.0 1.0 0.0 0 0 false))
  (Variables|Default|SetInterference_Sound _returnvalue_2)
  (bind _returnvalue_3 (Audio|SpawnSoundatLocation "/Game/GD/Sound/Music_Noise/SC_Game_Theme_Radio_Cue.SC_Game_Theme_Radio_Cue" (Transformation|GetWorldLocation (Variables|Default|GetStaticMesh)) "0, 0, 0" 0.0 1.0 0.0 0 0 false))
  (bind _output_get_2 (Variables|Default|SetGood_Sound _returnvalue_3))
  (Audio|Components|Audio|Play _output_get_2 0.0)
  (bind _returnvalue_4 (Rendering|Material|CreateDynamicMaterialInstance _staticmesh 1 (Rendering|Material|GetMaterial _staticmesh 1) "None" :!class /Script/Engine.PrimitiveComponent))
  (bind _output_get_3 (Variables|Default|SetDynamic_Material _returnvalue_4))
  (Rendering|Material|SetMaterial _staticmesh 1 _output_get_3))

(event EventTick
  (params (DeltaSeconds :type Float%20%28single-precision%29)))

(event Input|MouseEvents|RightMouseButton
  (params (Key :type Key%20Structure :default "None"))
  (bind _returnvalue (Game|GetPlayerController 0))
  (bind _first_person_0 (Variables|Default|GetFirst_Person_0))
  (bind _first_person_0_2 (Variables|Default|GetFirst_Person_0))
  (:Pressed
    (if (Variables|Default|GetMay_Get_Out_Of_The_Minigame_?)
      (Input|DisableInput (Game|GetPlayerController 0))
      (Variables|Default|SetMay_Get_Out_Of_The_Minigame_? false)
      (Variables|/Script/Engine.PlayerController|SetbShowMouseCursor (Game|GetPlayerController 0) false)
      (Collision|SetCollisionProfileName (Variables|Default|GetBox) "BlockAll" true :!class /Script/Engine.PrimitiveComponent)
      (Collision|SetCollisionProfileName (Variables|Default|GetBox2) "NoCollision" true :!class /Script/Engine.PrimitiveComponent)
      (bind _time_to_move_object (Timeline|Timeline_1 PlayFromStart)
        (:Update
          (Transformation|SetWorldTransform (Variables|/Game/GD/ThirdPerson/Blueprints/BP_Diplome_First_Person_Project.BP_Diplome_First_Person_Project_C|GetCinematic_Camera _first_person_0_2) (Math|Transform|Lerp(Transform) (Variables|Default|GetFollow_Camera_Transform) (Transformation|GetWorldTransform (Variables|/Game/GD/ThirdPerson/Blueprints/BP_Diplome_First_Person_Project.BP_Diplome_First_Person_Project_C|GetFirst_Person_Camera _first_person_0_2)) _time_to_move_object) false false))
        (:Finished
          (Components|Activation|SetActive (Variables|/Game/GD/ThirdPerson/Blueprints/BP_Diplome_First_Person_Project.BP_Diplome_First_Person_Project_C|GetCinematic_Camera _first_person_0) false false)
          (Components|Activation|SetActive (Variables|/Game/GD/ThirdPerson/Blueprints/BP_Diplome_First_Person_Project.BP_Diplome_First_Person_Project_C|GetFirst_Person_Camera _first_person_0) true false)
          (Variables|/Game/GD/ThirdPerson/Blueprints/BP_Diplome_First_Person_Project.BP_Diplome_First_Person_Project_C|SetInto_Minigame_? _first_person_0 false)
          (Input|DisableInput _returnvalue)
          (Input|EnableInput (Variables|Default|GetFirst_Person_0) _returnvalue)
          (Collision|SetCollisionProfileName (Variables|Default|GetBox) "BlockAll" true :!class /Script/Engine.PrimitiveComponent))))))

(event Input|MouseEvents|LeftMouseButton
  (params (Key :type Key%20Structure :default "None"))
  (bind _returnvalue (Game|GetPlayerController 0))
  (bind _hitresult (Game|Player|GetHitResultUnderCursorbyChannel _returnvalue "TraceTypeQuery1" true))
  (bind _hitcomponent (Collision|BreakHitResult _hitresult))
  (:Released
    (if (== (Variables|Default|GetBox1) _hitcomponent)
      (CallFunction|FirstButtonLeft)
      (elif (== (Variables|Default|GetBox2) _hitcomponent)
        (CallFunction|FirstButtonRight)
        (elif (== (Variables|Default|GetBox3) _hitcomponent)
          (CallFunction|SecondButtonLeft)
          (elif (== (Variables|Default|GetBox4) _hitcomponent)
            (CallFunction|SecondButtonRight)))))))

(fn ConstructionScript
  (|CallParentFunction))