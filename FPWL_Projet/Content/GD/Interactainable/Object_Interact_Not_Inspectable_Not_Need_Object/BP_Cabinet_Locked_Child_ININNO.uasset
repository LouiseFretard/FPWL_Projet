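; Interactable locked cabinet with a three-wheel combination padlock minigame that gives the player a reward when solved.
; Hitting its box disables player input and blends the cinematic camera to the lock, where cursor clicks on hitboxes turn wheels and right-click exits.
; Each turn checks a hard-coded combination; success restores the view, then chained timelines open padlock and door around spawning the Reward child actor.
; Dynamic material instances toggle the highlight.
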(event Custom|Got_Right_Combination_?
  (bind _returnvalue (Game|GetPlayerController 0))
  (bind _first_person_0 (Variables|Default|GetFirst_Person_0))
  (bind _first_person_0_2 (Variables|Default|GetFirst_Person_0))
  (bind _first_person_0_3 (Variables|Default|GetFirst_Person_0))
  ;[1 1 1] Check_Combination_+_What_To_Do_If_Right_Combination
  (if (Math|Boolean|ANDBoolean (== (Variables|Default|GetHow_Many_Time_First_Roulettes_Rolled_?) 1.0) (== (Variables|Default|GetHow_Many_Time_Second_Roulette_Rolled_?) 6.0) (== (Variables|Default|GetHow_Many_Time_Third_Roulettes_Rolled_?) 8.0))
    (Collision|SetCollisionEnabled (Variables|Default|GetBox) "NoCollision")
    (Input|DisableInput (Game|GetPlayerController 0))
    (Variables|Default|SetMay_Get_Out_Of_The_Minigame_? false)
    (Variables|/Script/Engine.PlayerController|SetbShowMouseCursor (Game|GetPlayerController 0) false)
    (Collision|SetCollisionProfileName (Variables|Default|GetBox) "NoCollision" true :!class /Script/Engine.PrimitiveComponent)
    (bind _time_to_move_object (Timeline|Timeline_3 PlayFromStart)
      (:Update
        (Transformation|SetWorldTransform (Variables|/Game/GD/ThirdPerson/Blueprints/BP_Diplome_First_Person_Project.BP_Diplome_First_Person_Project_C|GetCinematic_Camera _first_person_0_2) (Math|Transform|Lerp(Transform) (Variables|Default|GetFollow_Camera_Transform) (Transformation|GetWorldTransform (Variables|/Game/GD/ThirdPerson/Blueprints/BP_Diplome_First_Person_Project.BP_Diplome_First_Person_Project_C|GetFirst_Person_Camera _first_person_0_2)) _time_to_move_object) false false))
      (:Finished
        (Components|Activation|SetActive (Variables|/Game/GD/ThirdPerson/Blueprints/BP_Diplome_First_Person_Project.BP_Diplome_First_Person_Project_C|GetCinematic_Camera _first_person_0_3) false false)
        (Components|Activation|SetActive (Variables|/Game/GD/ThirdPerson/Blueprints/BP_Diplome_First_Person_Project.BP_Diplome_First_Person_Project_C|GetFirst_Person_Camera _first_person_0_3) true false)
        (Variables|/Game/GD/ThirdPerson/Blueprints/BP_Diplome_First_Person_Project.BP_Diplome_First_Person_Project_C|SetInto_Minigame_? _first_person_0_3 false)
        (Variables|Default|SetOriginal_Relative_Rotation_Locker_Wheel_Part_Arrow (Variables|/Script/Engine.SceneComponent|GetRelativeRotation (Variables|Default|GetArrow1)))
        (Variables|Default|SetOriginal_Relative_Rotation_Locker_Opening_Part_Arrow (Variables|/Script/Engine.SceneComponent|GetRelativeRotation (Variables|Default|GetCadenas_UE_Ouverture2_LP)))
        (bind _time_to_move_object_2 (Timeline|Timeline_4 PlayFromStart)
          (:Update
            (Transformation|SetRelativeRotation (Variables|Default|GetArrow1) (Math|Rotator|Lerp(Rotator) (Variables|Default|GetOriginal_Relative_Rotation_Locker_Wheel_Part_Arrow) (Math|Rotator|CombineRotators (Variables|Default|GetOriginal_Relative_Rotation_Locker_Wheel_Part_Arrow) (Math|Vector|RotatorfromAxisandAngle "1.000000,0.000000, 0" 5e+01)) _time_to_move_object_2) false false)
            (Transformation|SetRelativeRotation (Variables|Default|GetCadenas_UE_Ouverture2_LP) (Math|Rotator|Lerp(Rotator) (Variables|Default|GetOriginal_Relative_Rotation_Locker_Opening_Part_Arrow) (Math|Rotator|CombineRotators (Variables|Default|GetOriginal_Relative_Rotation_Locker_Opening_Part_Arrow) (Math|Vector|RotatorfromAxisandAngle "1.000000,0.000000, 0" -2e+01)) _time_to_move_object_2) false false))
          (:Finished
            (ChildActorComponent|SetChildActorClass (Variables|Default|GetReward_For_Player) (Variables|Default|GetReward))
            (Collision|SetCollisionProfileName (Variables|Default|GetBox_Up_First_Roulette) "NoCollision" true :!class /Script/Engine.PrimitiveComponent)
            (Variables|Default|SetOriginal_Relative_Rotation_Locker_Arrow (Variables|/Script/Engine.SceneComponent|GetRelativeRotation (Variables|Default|GetArrow2)))
            (bind _time_to_move_object_3 (Timeline|Timeline_5 PlayFromStart)
              (:Update
                (Transformation|SetRelativeRotation (Variables|Default|GetArrow2) (Math|Rotator|Lerp(Rotator) (Variables|Default|GetOriginal_Relative_Rotation_Locker_Arrow) (Math|Rotator|CombineRotators (Variables|Default|GetOriginal_Relative_Rotation_Locker_Arrow) (Math|Vector|RotatorfromAxisandAngle "1.000000,0.000000, 0" 2e+01)) _time_to_move_object_3) false false))
              (:Finished
                (Variables|Default|SetOriginal_Relative_Rotation_Door (Variables|/Script/Engine.SceneComponent|GetRelativeRotation (Variables|Default|GetDoor)))
                (bind _time_to_move_object_4 (Timeline|Timeline_6 PlayFromStart)
                  (:Update
                    (Transformation|SetRelativeRotation (Variables|Default|GetDoor) (Math|Rotator|Lerp(Rotator) (Variables|Default|GetOriginal_Relative_Rotation_Door) (Math|Rotator|CombineRotators (Variables|Default|GetOriginal_Relative_Rotation_Door) (Math|Vector|RotatorfromAxisandAngle "0.000000,0.000000,1.000000" 2e+02)) _time_to_move_object_4) false false))
                  (:Finished
                    (Variables|Default|SetCan_Be_Used_? false)
                    ;[1 1 1] Get_Out_Of_This_Minigame
                    (bind _time_to_move_object_5 (Timeline|Timeline_1 PlayFromStart)
                      (:Update
                        (Transformation|SetWorldTransform (Variables|/Game/GD/ThirdPerson/Blueprints/BP_Diplome_First_Person_Project.BP_Diplome_First_Person_Project_C|GetCinematic_Camera (Variables|Default|GetFirst_Person_0)) (Math|Transform|Lerp(Transform) (Variables|Default|GetFollow_Camera_Transform) (Transformation|GetWorldTransform (Variables|/Game/GD/ThirdPerson/Blueprints/BP_Diplome_First_Person_Project.BP_Diplome_First_Person_Project_C|GetFirst_Person_Camera (Variables|Default|GetFirst_Person_0))) _time_to_move_object_5) false false))
                      (:Finished
                        (Components|Activation|SetActive (Variables|/Game/GD/ThirdPerson/Blueprints/BP_Diplome_First_Person_Project.BP_Diplome_First_Person_Project_C|GetCinematic_Camera _first_person_0) false false)
                        (Components|Activation|SetActive (Variables|/Game/GD/ThirdPerson/Blueprints/BP_Diplome_First_Person_Project.BP_Diplome_First_Person_Project_C|GetFirst_Person_Camera _first_person_0) true false)
                        (Variables|/Game/GD/ThirdPerson/Blueprints/BP_Diplome_First_Person_Project.BP_Diplome_First_Person_Project_C|SetInto_Minigame_? (Variables|Default|GetFirst_Person_0) false)
                        (Input|EnableInput (Variables|Default|GetFirst_Person_0) (Game|GetPlayerController 0))
                        (Input|DisableInput _returnvalue)
                        (Input|EnableInput (Variables|Default|GetFirst_Person_0) _returnvalue)
                        (Collision|SetCollisionProfileName (Variables|/Game/GD/ThirdPerson/Blueprints/BP_Diplome_First_Person_Project.BP_Diplome_First_Person_Project_C|GetHighlight_Detection (Variables|Default|GetFirst_Person_0)) "OverlapAllDynamic" true :!class /Script/Engine.PrimitiveComponent)))))))))))))

(event Custom|Third_Wheel_Down
  ;[1 1 1] What_To_Do_When_A_Hitbox_Is_Hit
  (if (not (Variables|Default|GetThird_Roulette_May_Turn_?))
    (Variables|Default|SetWheel_Which_Turn_V_2 (Variables|Default|GetCadenas_UE_Roulette2_LP2))
    (Variables|Default|SetThird_Roulette_May_Turn_? true)
    (Variables|Default|SetSide_To_Turn 4e+01)
    (if (< (- (Variables|Default|GetHow_Many_Time_Third_Roulettes_Rolled_?) 1.0) (Variables|Default|GetMin_Roulette))
      (Variables|Default|SetHow_Many_Time_Third_Roulettes_Rolled_? (Variables|Default|GetMax_Roulette))
      (else
        (Variables|Default|SetHow_Many_Time_Third_Roulettes_Rolled_? (- (Variables|Default|GetHow_Many_Time_Third_Roulettes_Rolled_?) 1.0))))
    (CallFunction|TurnAWheel)))

(event Custom|First_Wheel_Up
  ;[1 1 1] What_To_Do_When_A_Hitbox_Is_Hit
  (if (not (Variables|Default|GetFirst_Roulette_May_Turn_?))
    (Variables|Default|SetWheel_Which_Turn_V_2 (Variables|Default|GetCadenas_UE_Roulette2_LP1))
    (Variables|Default|SetFirst_Roulette_May_Turn_? true)
    (Variables|Default|SetSide_To_Turn -4e+01)
    (if (> (+ (Variables|Default|GetHow_Many_Time_First_Roulettes_Rolled_?) 1.0) (Variables|Default|GetMax_Roulette))
      (Variables|Default|SetHow_Many_Time_First_Roulettes_Rolled_? (Variables|Default|GetMin_Roulette))
      (else
        (Variables|Default|SetHow_Many_Time_First_Roulettes_Rolled_? (+ (Variables|Default|GetHow_Many_Time_First_Roulettes_Rolled_?) 1.0))))
    (CallFunction|TurnAWheel)))

(event Custom|First_Wheel_Down
  ;[1 1 1] What_To_Do_When_A_Hitbox_Is_Hit
  (if (not (Variables|Default|GetFirst_Roulette_May_Turn_?))
    (Variables|Default|SetWheel_Which_Turn_V_2 (Variables|Default|GetCadenas_UE_Roulette2_LP1))
    (Variables|Default|SetFirst_Roulette_May_Turn_? true)
    (Variables|Default|SetSide_To_Turn 4e+01)
    (if (< (- (Variables|Default|GetHow_Many_Time_First_Roulettes_Rolled_?) 1.0) (Variables|Default|GetMin_Roulette))
      (Variables|Default|SetHow_Many_Time_First_Roulettes_Rolled_? (Variables|Default|GetMax_Roulette))
      (else
        (Variables|Default|SetHow_Many_Time_First_Roulettes_Rolled_? (- (Variables|Default|GetHow_Many_Time_First_Roulettes_Rolled_?) 1.0))))
    (CallFunction|TurnAWheel)))

(event Custom|Second_Wheel_Up
  ;[1 1 1] What_To_Do_When_A_Hitbox_Is_Hit
  (if (not (Variables|Default|GetSecond_Roulette_May_Turn_?))
    (Variables|Default|SetWheel_Which_Turn_V_2 (Variables|Default|GetCadenas_UE_Roulette2_LP))
    (Variables|Default|SetSecond_Roulette_May_Turn_? true)
    (Variables|Default|SetSide_To_Turn -4e+01)
    (if (> (+ (Variables|Default|GetHow_Many_Time_Second_Roulette_Rolled_?) 1.0) (Variables|Default|GetMax_Roulette))
      (Variables|Default|SetHow_Many_Time_Second_Roulette_Rolled_? (Variables|Default|GetMin_Roulette))
      (else
        (Variables|Default|SetHow_Many_Time_Second_Roulette_Rolled_? (+ (Variables|Default|GetHow_Many_Time_Second_Roulette_Rolled_?) 1.0))))
    (CallFunction|TurnAWheel)))

(event Custom|Second_Wheel_Down
  ;[1 1 1] What_To_Do_When_A_Hitbox_Is_Hit
  (if (not (Variables|Default|GetSecond_Roulette_May_Turn_?))
    (Variables|Default|SetWheel_Which_Turn_V_2 (Variables|Default|GetCadenas_UE_Roulette2_LP))
    (Variables|Default|SetSecond_Roulette_May_Turn_? true)
    (Variables|Default|SetSide_To_Turn 4e+01)
    (if (< (- (Variables|Default|GetHow_Many_Time_Second_Roulette_Rolled_?) 1.0) (Variables|Default|GetMin_Roulette))
      (Variables|Default|SetHow_Many_Time_Second_Roulette_Rolled_? (Variables|Default|GetMax_Roulette))
      (else
        (Variables|Default|SetHow_Many_Time_Second_Roulette_Rolled_? (- (Variables|Default|GetHow_Many_Time_Second_Roulette_Rolled_?) 1.0))))
    (CallFunction|TurnAWheel)))

(event Custom|Turn_A_Wheel
  (bind _wheel_which_turn_v_2 (Variables|Default|GetWheel_Which_Turn_V_2))
  ;[1 1 1] Turn a Wheel
  (Variables|Default|SetOriginal_Relative_Rotation_From_Wheel_Which_Turn (Variables|/Script/Engine.SceneComponent|GetRelativeRotation (Variables|Default|GetWheel_Which_Turn_V_2)))
  (bind _item_track (Timeline|Timeline_2 PlayFromStart)
    (:Update
      (Transformation|SetRelativeRotation (Variables|Default|GetWheel_Which_Turn_V_2) (Math|Rotator|Lerp(Rotator) (Variables|Default|GetOriginal_Relative_Rotation_From_Wheel_Which_Turn) (Math|Rotator|MakeRotator (+ (.roll (Variables|Default|GetOriginal_Relative_Rotation_From_Wheel_Which_Turn)) (Variables|Default|GetSide_To_Turn)) (.pitch (Variables|Default|GetOriginal_Relative_Rotation_From_Wheel_Which_Turn)) (.yaw (Variables|Default|GetOriginal_Relative_Rotation_From_Wheel_Which_Turn))) _item_track) false false))
    (:Finished
      (CallFunction|GotRightCombination?)
      (if (== (Variables|Default|GetWheel_Which_Turn_V_2) (Variables|Default|GetCadenas_UE_Roulette2_LP1))
        (Variables|Default|SetFirst_Roulette_May_Turn_? false)
        (elif (== _wheel_which_turn_v_2 (Variables|Default|GetCadenas_UE_Roulette2_LP))
          (Variables|Default|SetSecond_Roulette_May_Turn_? false)
          (elif (== _wheel_which_turn_v_2 (Variables|Default|GetCadenas_UE_Roulette2_LP2))
            (Variables|Default|SetThird_Roulette_May_Turn_? false)))))))

(event Custom|Third_Wheel_Up
  ;[1 1 1] What_To_Do_When_A_Hitbox_Is_Hit
  (if (not (Variables|Default|GetThird_Roulette_May_Turn_?))
    (Variables|Default|SetWheel_Which_Turn_V_2 (Variables|Default|GetCadenas_UE_Roulette2_LP2))
    (Variables|Default|SetThird_Roulette_May_Turn_? true)
    (Variables|Default|SetSide_To_Turn -4e+01)
    (if (> (+ (Variables|Default|GetHow_Many_Time_Third_Roulettes_Rolled_?) 1.0) (Variables|Default|GetMax_Roulette))
      (Variables|Default|SetHow_Many_Time_Third_Roulettes_Rolled_? (Variables|Default|GetMin_Roulette))
      (else
        (Variables|Default|SetHow_Many_Time_Third_Roulettes_Rolled_? (+ (Variables|Default|GetHow_Many_Time_Third_Roulettes_Rolled_?) 1.0))))
    (CallFunction|TurnAWheel)))

(event EventBeginPlay
  (|CallParentFunction)
  (bind _returnvalue (Rendering|Material|CreateDynamicMaterialInstance "/Game/TA/Materials/Gameplay/Maison/BoiteClés.BoiteClés" "None" "None" :!class /Script/Engine.KismetMaterialLibrary))
  (bind _output_get (Variables|Default|SetM_inst _returnvalue))
  (Rendering|Material|SetMaterial (Variables|Default|GetStaticMesh6) 0 _output_get)
  (Rendering|Material|SetScalarParameterValue (Variables|Default|GetM_inst) "Activate" 0.0 :!class /Script/Engine.MaterialInstanceDynamic)
  (bind _returnvalue_2 (Rendering|Material|CreateDynamicMaterialInstance "/Game/TA/Materials/Gameplay/Maison/Cadenas.Cadenas" "None" "None" :!class /Script/Engine.KismetMaterialLibrary))
  (bind _output_get_2 (Variables|Default|SetM_inst2 _returnvalue_2))
  (Rendering|Material|SetMaterial (Variables|Default|GetCadenas_UE_Main2_LP) 0 _output_get_2)
  (Rendering|Material|SetScalarParameterValue _output_get_2 "Activate" 0.0 :!class /Script/Engine.MaterialInstanceDynamic))

(event Collision|EventActorBeginOverlap
  (params (OtherActor :type Actor%20Object%20Reference))
  (|CallParentFunction OtherActor) ; This node is disabled and will not be called.\nDrag off pins to build functionality.
)

(event EventTick
  (params (DeltaSeconds :type Float%20%28single-precision%29))
  (|CallParentFunction DeltaSeconds) ; This node is disabled and will not be called.\nDrag off pins to build functionality.
)

(event EventPartHit
  (params (Hit_Component :type Primitive%20Component%20Object%20Reference) (Pawn :type Pawn%20Object%20Reference))
  (bind _asbp_diplome_first_person_project (Utilities|Casting|CastToBP_Diplome_First_Person_Project Pawn))
  (Utilities|IsValid (Variables|Default|GetFirst_Person_0)
    (:Is%20Valid
      _)
    (:Is%20Not%20Valid
      (Variables|Default|SetFirst_Person_0 _asbp_diplome_first_person_project)))
  (if (== Hit_Component (Variables|Default|GetBox))
    (Variables|Default|SetCan_Be_Used_? false)
    (Variables|/Game/GD/ThirdPerson/Blueprints/BP_Diplome_First_Person_Project.BP_Diplome_First_Person_Project_C|SetInto_Minigame_? (Variables|Default|GetFirst_Person_0) true)
    (Variables|/Script/Engine.PlayerController|SetbShowMouseCursor (Game|GetPlayerController 0) true)
    (Collision|SetCollisionProfileName (Variables|Default|GetBox) "None" true :!class /Script/Engine.PrimitiveComponent)
    (Input|DisableInput (Variables|Default|GetFirst_Person_0) (Game|GetPlayerController 0))
    (Collision|SetCollisionProfileName (Variables|Default|GetBox) "NoCollision" true :!class /Script/Engine.PrimitiveComponent)
    (Transformation|SetWorldTransform (Variables|/Game/GD/ThirdPerson/Blueprints/BP_Diplome_First_Person_Project.BP_Diplome_First_Person_Project_C|GetCinematic_Camera (Variables|Default|GetFirst_Person_0)) (Transformation|GetWorldTransform (Variables|/Game/GD/ThirdPerson/Blueprints/BP_Diplome_First_Person_Project.BP_Diplome_First_Person_Project_C|GetFirst_Person_Camera (Variables|Default|GetFirst_Person_0))) false false)
    (Variables|Default|SetFollow_Camera_Transform (Transformation|GetWorldTransform (Variables|/Game/GD/ThirdPerson/Blueprints/BP_Diplome_First_Person_Project.BP_Diplome_First_Person_Project_C|GetCinematic_Camera (Variables|Default|GetFirst_Person_0))))
    (Components|Activation|SetActive (Variables|/Game/GD/ThirdPerson/Blueprints/BP_Diplome_First_Person_Project.BP_Diplome_First_Person_Project_C|GetCinematic_Camera (Variables|Default|GetFirst_Person_0)) true false)
    (Components|Activation|SetActive (Variables|/Game/GD/ThirdPerson/Blueprints/BP_Diplome_First_Person_Project.BP_Diplome_First_Person_Project_C|GetFirst_Person_Camera (Variables|Default|GetFirst_Person_0)) false false)
    (bind _time_to_move_object (Timeline|Timeline_0 PlayFromStart)
      (:Update
        (Transformation|SetWorldTransform (Variables|/Game/GD/ThirdPerson/Blueprints/BP_Diplome_First_Person_Project.BP_Diplome_First_Person_Project_C|GetCinematic_Camera (Variables|Default|GetFirst_Person_0)) (Math|Transform|Lerp(Transform) (Variables|Default|GetFollow_Camera_Transform) (Transformation|GetWorldTransform (Variables|Default|GetCube6)) _time_to_move_object) false false))
      (:Finished
        (Variables|Default|SetFollow_Camera_Transform (Transformation|GetWorldTransform (Variables|/Game/GD/ThirdPerson/Blueprints/BP_Diplome_First_Person_Project.BP_Diplome_First_Person_Project_C|GetCinematic_Camera (Variables|Default|GetFirst_Person_0))))
        (Variables|Default|SetMay_Get_Out_Of_The_Minigame_? true)
        (Input|EnableInput (Game|GetPlayerController 0))
        (Collision|SetCollisionProfileName (Variables|Default|GetBox_Up_First_Roulette) "BlockAll" true :!class /Script/Engine.PrimitiveComponent)))))

(event EventOnHighlight
  (Rendering|Material|SetScalarParameterValue (Variables|Default|GetM_inst) "Activate" 1.0 :!class /Script/Engine.MaterialInstanceDynamic)
  (Rendering|Material|SetScalarParameterValue (Variables|Default|GetM_inst2) "Activate" 1.0 :!class /Script/Engine.MaterialInstanceDynamic))

(event EventStopHighlight
  (Rendering|Material|SetScalarParameterValue (Variables|Default|GetM_inst) "Activate" 0.0 :!class /Script/Engine.MaterialInstanceDynamic)
  (Rendering|Material|SetScalarParameterValue (Variables|Default|GetM_inst2) "Activate" 0.0 :!class /Script/Engine.MaterialInstanceDynamic))

(event Input|MouseEvents|RightMouseButton
  (params (Key :type Key%20Structure :default "None"))
  (bind _returnvalue (Game|GetPlayerController 0))
  (bind _first_person_0 (Variables|Default|GetFirst_Person_0))
  ;[1 1 1] Get_Out_Of_This_Minigame
  (:Released
    (if (Variables|Default|GetMay_Get_Out_Of_The_Minigame_?)
      (Input|DisableInput (Game|GetPlayerController 0))
      (Variables|Default|SetMay_Get_Out_Of_The_Minigame_? false)
      (Variables|/Script/Engine.PlayerController|SetbShowMouseCursor (Game|GetPlayerController 0) false)
      (Collision|SetCollisionProfileName (Variables|Default|GetBox) "BlockAll" true :!class /Script/Engine.PrimitiveComponent)
      (Variables|Default|SetCan_Be_Used_? true)
      (bind _time_to_move_object (Timeline|Timeline_1 PlayFromStart)
        (:Update
          (Transformation|SetWorldTransform (Variables|/Game/GD/ThirdPerson/Blueprints/BP_Diplome_First_Person_Project.BP_Diplome_First_Person_Project_C|GetCinematic_Camera (Variables|Default|GetFirst_Person_0)) (Math|Transform|Lerp(Transform) (Variables|Default|GetFollow_Camera_Transform) (Transformation|GetWorldTransform (Variables|/Game/GD/ThirdPerson/Blueprints/BP_Diplome_First_Person_Project.BP_Diplome_First_Person_Project_C|GetFirst_Person_Camera (Variables|Default|GetFirst_Person_0))) _time_to_move_object) false false))
        (:Finished
          (Components|Activation|SetActive (Variables|/Game/GD/ThirdPerson/Blueprints/BP_Diplome_First_Person_Project.BP_Diplome_First_Person_Project_C|GetCinematic_Camera _first_person_0) false false)
          (Components|Activation|SetActive (Variables|/Game/GD/ThirdPerson/Blueprints/BP_Diplome_First_Person_Project.BP_Diplome_First_Person_Project_C|GetFirst_Person_Camera _first_person_0) true false)
          (Variables|/Game/GD/ThirdPerson/Blueprints/BP_Diplome_First_Person_Project.BP_Diplome_First_Person_Project_C|SetInto_Minigame_? (Variables|Default|GetFirst_Person_0) false)
          (Input|EnableInput (Variables|Default|GetFirst_Person_0) (Game|GetPlayerController 0))
          (Input|DisableInput _returnvalue)
          (Input|EnableInput (Variables|Default|GetFirst_Person_0) _returnvalue)
          (Collision|SetCollisionProfileName (Variables|/Game/GD/ThirdPerson/Blueprints/BP_Diplome_First_Person_Project.BP_Diplome_First_Person_Project_C|GetHighlight_Detection (Variables|Default|GetFirst_Person_0)) "OverlapAllDynamic" true :!class /Script/Engine.PrimitiveComponent))))))

(event Input|MouseEvents|LeftMouseButton
  (params (Key :type Key%20Structure :default "None"))
  (bind _returnvalue (Game|GetPlayerController 0))
  (bind _hitresult (Game|Player|GetHitResultUnderCursorbyChannel _returnvalue "TraceTypeQuery1" true))
  (bind _hitcomponent (Collision|BreakHitResult _hitresult))
  ;[1 1 1] What_Hitbox_Is_hit
  (:Released
    (if (== (Variables|Default|GetBox_Up_First_Roulette) _hitcomponent)
      (CallFunction|FirstWheelUp)
      (elif (== (Variables|Default|GetBox_Down_First_Roulette) _hitcomponent)
        (CallFunction|FirstWheelDown)
        (elif (== (Variables|Default|GetBox_Up_Second_Roulette) _hitcomponent)
          (CallFunction|SecondWheelUp)
          (elif (== (Variables|Default|GetBox_Down_Second_Roulette) _hitcomponent)
            (CallFunction|SecondWheelDown)
            (elif (== (Variables|Default|GetBox_Up_Third_Roulette) _hitcomponent)
              (CallFunction|ThirdWheelUp)
              (elif (== (Variables|Default|GetBox_Down_Third_Roulette) _hitcomponent)
                (CallFunction|ThirdWheelDown)))))))))

(fn ConstructionScript
  (|CallParentFunction))