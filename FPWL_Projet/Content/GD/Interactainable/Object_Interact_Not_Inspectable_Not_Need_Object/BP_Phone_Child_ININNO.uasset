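; Interactable phone that lets the player switch between two first-person characters, with a scripted Raymond and Cécile call.
; BeginPlay moves the second phone mesh, spawns and briefly possesses a second pawn there, then repossesses the first.
; HitSucces shows restore-power or explore objectives until both are done, then plays the delay-chained dialogue and an FOV-zoom possession swap.
; Later hits alternate possession by FlipFlop, indexing GetAllActorsOfClass; sphere overlap logic is disconnected.
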(event OnComponentBeginOverlap(Sphere)
  (params (OverlappedComponent :type Primitive%20Component%20Object%20Reference) (OtherActor :type Actor%20Object%20Reference) (OtherComp :type Primitive%20Component%20Object%20Reference) (OtherBodyIndex :type Integer) (bFromSweep :type Boolean) (SweepResult :type Hit%20Result%20Structure%20%28by%20ref%29)))

(event OnComponentEndOverlap(Sphere)
  (params (OverlappedComponent :type Primitive%20Component%20Object%20Reference) (OtherActor :type Actor%20Object%20Reference) (OtherComp :type Primitive%20Component%20Object%20Reference) (OtherBodyIndex :type Integer)))

(event OnComponentBeginOverlap(Sphere1)
  (params (OverlappedComponent :type Primitive%20Component%20Object%20Reference) (OtherActor :type Actor%20Object%20Reference) (OtherComp :type Primitive%20Component%20Object%20Reference) (OtherBodyIndex :type Integer) (bFromSweep :type Boolean) (SweepResult :type Hit%20Result%20Structure%20%28by%20ref%29)))

(event OnComponentEndOverlap(Sphere1)
  (params (OverlappedComponent :type Primitive%20Component%20Object%20Reference) (OtherActor :type Actor%20Object%20Reference) (OtherComp :type Primitive%20Component%20Object%20Reference) (OtherBodyIndex :type Integer)))

(event EventBeginPlay
  (bind _returnvalue (Game|GetPlayerController 0))
  (|CallParentFunction)
  (Transformation|SetWorldLocation (Variables|Default|GetStaticMesh1) (Variables|Default|GetLocation_Second_Phone) false false)
  (Variables|Default|SetProblem_? true)
  (bind _returnvalue_2 (Game|SpawnActorfromClass "/Game/GD/ThirdPerson/Blueprints/BP_Diplome_First_Person_Project.BP_Diplome_First_Person_Project_C" (Math|Transform|MakeTransform (Variables|Default|GetLocation_Second_Phone) "0, 0, 0" "1.000000,1.000000,1.000000") "Undefined" 0 0))
  (bind _asbp_diplome_first_person_project (Utilities|Casting|CastToBP_Diplome_First_Person_Project _returnvalue_2))
  (bind _output_get (Variables|Default|Set2nd_First_Person _asbp_diplome_first_person_project))
  (Pawn|Possess _returnvalue _output_get)
  (Input|EnableInput _output_get _returnvalue)
  (Default|BlackScreenOff (Variables|/Game/GD/ThirdPerson/Blueprints/BP_Diplome_First_Person_Project.BP_Diplome_First_Person_Project_C|GetHUD _output_get))
  (Variables|/Game/GD/ThirdPerson/Blueprints/BP_Diplome_First_Person_Project.BP_Diplome_First_Person_Project_C|SetBriquet_Activé_Une_Fois_? _output_get true)
  (bind _outactors (Actor|GetAllActorsOfClass "/Game/GD/ThirdPerson/Blueprints/BP_Diplome_First_Person_Project.BP_Diplome_First_Person_Project_C"))
  (Pawn|Possess (Game|GetPlayerController 0) (Utilities|Array|Get(acopy) _outactors)))

(event Collision|EventActorBeginOverlap
  (params (OtherActor :type Actor%20Object%20Reference))
  (|CallParentFunction OtherActor) ; This node is disabled and will not be called.\nDrag off pins to build functionality.
)

(event EventTick
  (params (DeltaSeconds :type Float%20%28single-precision%29))
  (|CallParentFunction DeltaSeconds) ; This node is disabled and will not be called.\nDrag off pins to build functionality.
)

(event EventHitSucces
  (bind _returnvalue (Game|GetPlayerController 0))
  (bind _dialogue_if_problem__ (Variables|Default|GetDialogue_If_Problem_?))
  (bind _dialogue (Variables|Default|GetDialogue))
  (bind _first_person (Variables|Default|GetFirst_Person))
  (bind _first_person_2 (Variables|Default|GetFirst_Person))
  (bind _first_person_3 (Variables|Default|GetFirst_Person))
  (bind _first_person_4 (Variables|Default|GetFirst_Person))
  (bind _first_person_5 (Variables|Default|GetFirst_Person))
  (bind _first_person_6 (Variables|Default|GetFirst_Person))
  (bind _first_person_7 (Variables|Default|GetFirst_Person))
  (bind _first_person_8 (Variables|Default|GetFirst_Person))
  (bind _first_person_9 (Variables|Default|GetFirst_Person))
  (bind _first_person_10 (Variables|Default|GetFirst_Person))
  (bind _first_person_11 (Variables|Default|GetFirst_Person))
  (bind _first_person_12 (Variables|Default|GetFirst_Person))
  (bind _first_person_13 (Variables|Default|GetFirst_Person))
  (bind _first_person_14 (Variables|Default|GetFirst_Person))
  (bind _first_person_15 (Variables|Default|GetFirst_Person))
  (bind _first_person_16 (Variables|Default|GetFirst_Person))
  (bind _first_person_17 (Variables|Default|GetFirst_Person))
  (bind _first_person_18 (Variables|Default|GetFirst_Person))
  (bind _first_person_19 (Variables|Default|GetFirst_Person))
  (bind _first_person_20 (Variables|Default|GetFirst_Person))
  (bind _first_person_21 (Variables|Default|GetFirst_Person))
  (bind _first_person_22 (Variables|Default|GetFirst_Person))
  (bind _first_person_23 (Variables|Default|GetFirst_Person))
  (bind _hud (Variables|/Game/GD/ThirdPerson/Blueprints/BP_Diplome_First_Person_Project.BP_Diplome_First_Person_Project_C|GetHUD _first_person_23))
  (bind _hud_2 (Variables|/Game/GD/ThirdPerson/Blueprints/BP_Diplome_First_Person_Project.BP_Diplome_First_Person_Project_C|GetHUD _first_person_7))
  (if (Variables|Default|GetProblem_?)
    (if (not (Utilities|Enum|Equal(Enum) _dialogue_if_problem__ ""))
      (Default|TransmissDialogue _first_person_23 _dialogue_if_problem__)
      (Utilities|FlowControl|Delay 2.0))
    (Default|EndDialogue _hud)
    (Widget|SetRenderOpacity (Variables|/Game/GD/Widget/HUD.HUD_C|GetBorder_Objective _hud) 1.0)
    (Rendering|Components|TextRender|SetText (Variables|/Game/GD/Widget/HUD.HUD_C|GetHow_To_Show_Objective _hud) "Objectif : Rétablir le courant")
    (elif (not (Variables|Default|GetExploration_Terminée_?))
      (if (not (Utilities|Enum|Equal(Enum) _dialogue ""))
        (Default|TransmissDialogue _first_person_7 _dialogue)
        (Utilities|FlowControl|Delay 2.0))
      (Default|EndDialogue _hud_2)
      (Widget|SetRenderOpacity (Variables|/Game/GD/Widget/HUD.HUD_C|GetBorder_Objective _hud_2) 1.0)
      (Rendering|Components|TextRender|SetText (Variables|/Game/GD/Widget/HUD.HUD_C|GetHow_To_Show_Objective _hud_2) "Objectif : Explorer")
      (elif (Variables|Default|GetExploration_Terminée_?)
        (if (Variables|Default|GetFirst_Switch_Done_?)
          (Utilities|FlowControl|FlipFlop
            (:A
              (bind _outactors (Actor|GetAllActorsOfClass "/Game/GD/ThirdPerson/Blueprints/BP_Diplome_First_Person_Project.BP_Diplome_First_Person_Project_C"))
              (Pawn|Possess (Game|GetPlayerController 0) (Utilities|Array|Get(acopy) _outactors)))
            (:B
              (bind _outactors_2 (Actor|GetAllActorsOfClass "/Game/GD/ThirdPerson/Blueprints/BP_Diplome_First_Person_Project.BP_Diplome_First_Person_Project_C"))
              (Pawn|Possess (Game|GetPlayerController 0) (Utilities|Array|Get(acopy) _outactors_2 1))))
          (else
            (Input|DisableInput _first_person_2 (Game|GetPlayerController 0))
            ;[1 1 1] LES DIALOGUES DU PREMIER CHANGEMENT
            (Default|TransmissDialogue _first_person_2 "\"Bonjour\"")
            (Utilities|FlowControl|Delay 2.0)
            (Default|EndDialogue (Variables|/Game/GD/ThirdPerson/Blueprints/BP_Diplome_First_Person_Project.BP_Diplome_First_Person_Project_C|GetHUD _first_person_2))
            (Default|TransmissDialogue _first_person_11 "Raymond : \"Bonjour. Mettez moi en lien avec la maison au passage des Lilas à Auvillar\"")
            (Utilities|FlowControl|Delay 5.0)
            (Default|EndDialogue (Variables|/Game/GD/ThirdPerson/Blueprints/BP_Diplome_First_Person_Project.BP_Diplome_First_Person_Project_C|GetHUD _first_person_11))
            (Default|TransmissDialogue _first_person_18 "Un instant s’il vous plaît.")
            (Utilities|FlowControl|Delay 2.0)
            (Default|EndDialogue (Variables|/Game/GD/ThirdPerson/Blueprints/BP_Diplome_First_Person_Project.BP_Diplome_First_Person_Project_C|GetHUD _first_person_18))
            (Default|TransmissDialogue _first_person_12 "Cécile : “Raymond ?”")
            (Utilities|FlowControl|Delay 2.0)
            (Default|EndDialogue (Variables|/Game/GD/ThirdPerson/Blueprints/BP_Diplome_First_Person_Project.BP_Diplome_First_Person_Project_C|GetHUD _first_person_12))
            (Default|TransmissDialogue _first_person_13 "Raymon : “Oui Cécile, c’est moi. Je suis chez Lucien ..il n’y a personne.”")
            (Utilities|FlowControl|Delay 5.0)
            (Default|EndDialogue (Variables|/Game/GD/ThirdPerson/Blueprints/BP_Diplome_First_Person_Project.BP_Diplome_First_Person_Project_C|GetHUD _first_person_13))
            (Default|TransmissDialogue _first_person_17 "Cécile :“Et bien ?”")
            (Utilities|FlowControl|Delay 2.0)
            (Default|EndDialogue (Variables|/Game/GD/ThirdPerson/Blueprints/BP_Diplome_First_Person_Project.BP_Diplome_First_Person_Project_C|GetHUD _first_person_17))
            (Default|TransmissDialogue _first_person_14 "Raymond : “Et bien il n’y a personne !  
L’appartement est inhabité et pas franchement chaleureux.”")
            (Utilities|FlowControl|Delay 5.0)
            (Default|EndDialogue (Variables|/Game/GD/ThirdPerson/Blueprints/BP_Diplome_First_Person_Project.BP_Diplome_First_Person_Project_C|GetHUD _first_person_14))
            (Default|TransmissDialogue _first_person_15 "Cécile : “ ”")
            (Utilities|FlowControl|Delay 2.0)
            (Default|EndDialogue (Variables|/Game/GD/ThirdPerson/Blueprints/BP_Diplome_First_Person_Project.BP_Diplome_First_Person_Project_C|GetHUD _first_person_15))
            (Default|TransmissDialogue _first_person_16 "Raymond : “Cécile ?”")
            (Utilities|FlowControl|Delay 2.0)
            (Default|EndDialogue (Variables|/Game/GD/ThirdPerson/Blueprints/BP_Diplome_First_Person_Project.BP_Diplome_First_Person_Project_C|GetHUD _first_person_16))
            (Default|TransmissDialogue _first_person_8 "Cécile : “J’aurais dû savoir que ce ne serait pas si facile.”")
            (Utilities|FlowControl|Delay 2.0)
            (Default|EndDialogue (Variables|/Game/GD/ThirdPerson/Blueprints/BP_Diplome_First_Person_Project.BP_Diplome_First_Person_Project_C|GetHUD _first_person_8))
            (Default|TransmissDialogue _first_person_10 "Raymond : “Que quoi soit facile ? Cécile, vous vous rendez compte de la situation ?  
Vous m’avez traverser Paris pour fouiller dans les affaires d’un homme mort.”")
            (Utilities|FlowControl|Delay 8.0)
            (Default|EndDialogue (Variables|/Game/GD/ThirdPerson/Blueprints/BP_Diplome_First_Person_Project.BP_Diplome_First_Person_Project_C|GetHUD _first_person_10))
            (Default|TransmissDialogue _first_person_20 "Cécile : “..Ses affaires sont encore là ?” 
")
            (Utilities|FlowControl|Delay 2.0)
            (Default|EndDialogue (Variables|/Game/GD/ThirdPerson/Blueprints/BP_Diplome_First_Person_Project.BP_Diplome_First_Person_Project_C|GetHUD _first_person_20))
            (Default|TransmissDialogue _first_person_4 "Raymond : “Oui, et ça ne me rappelle pas de si bons souvenirs, donc si on pouvait en finir…”")
            (Utilities|FlowControl|Delay 2.0)
            (Default|EndDialogue (Variables|/Game/GD/ThirdPerson/Blueprints/BP_Diplome_First_Person_Project.BP_Diplome_First_Person_Project_C|GetHUD _first_person_4))
            (Default|TransmissDialogue _first_person_9 "Cécile : “Très bien ; Je ne vais pas tourner autour du pot : Je pense que Jeanne va mettre fin à ses jours.”")
            (Utilities|FlowControl|Delay 5.0)
            (Default|EndDialogue (Variables|/Game/GD/ThirdPerson/Blueprints/BP_Diplome_First_Person_Project.BP_Diplome_First_Person_Project_C|GetHUD _first_person_9))
            (Default|TransmissDialogue _first_person_19 "Raymond : “Comment ?”")
            (Utilities|FlowControl|Delay 2.0)
            (Default|EndDialogue (Variables|/Game/GD/ThirdPerson/Blueprints/BP_Diplome_First_Person_Project.BP_Diplome_First_Person_Project_C|GetHUD _first_person_19))
            (Default|TransmissDialogue _first_person_3 "Cécile :“Elle a quitté l'hôpital où elle était soignée avant-hier.  
Je me suis rendue chez elle pour essayer de la trouver, mais je n’ai rien trouvé à part une lettre.., un poème, adressé à Lucien.” 
")
            (Utilities|FlowControl|Delay 8.0)
            (Default|EndDialogue (Variables|/Game/GD/ThirdPerson/Blueprints/BP_Diplome_First_Person_Project.BP_Diplome_First_Person_Project_C|GetHUD _first_person_3))
            (Default|TransmissDialogue _first_person_5 "Raymond : “Vous lui aviez parlé récemment ?”")
            (Utilities|FlowControl|Delay 2.0)
            (Default|EndDialogue (Variables|/Game/GD/ThirdPerson/Blueprints/BP_Diplome_First_Person_Project.BP_Diplome_First_Person_Project_C|GetHUD _first_person_5))
            (Default|TransmissDialogue _first_person_22 "Cécile : “Pas vraiment, je devais lui rendre visite.. Attendez. J’entends quelque chose.. ”")
            (Utilities|FlowControl|Delay 5.0)
            (Default|EndDialogue (Variables|/Game/GD/ThirdPerson/Blueprints/BP_Diplome_First_Person_Project.BP_Diplome_First_Person_Project_C|GetHUD _first_person_22))
            (Default|TransmissDialogue _first_person_21 "Raymond : “.....Cécile ?”")
            (Utilities|FlowControl|Delay 2.0)
            (Default|EndDialogue (Variables|/Game/GD/ThirdPerson/Blueprints/BP_Diplome_First_Person_Project.BP_Diplome_First_Person_Project_C|GetHUD _first_person_21))
            (Default|TransmissDialogue _first_person_6 "Cécile : “Je vous rappelle. ”")
            (Utilities|FlowControl|Delay 2.0)
            (Default|EndDialogue (Variables|/Game/GD/ThirdPerson/Blueprints/BP_Diplome_First_Person_Project.BP_Diplome_First_Person_Project_C|GetHUD _first_person_6))
            (Default|TransmissDialogue _first_person "Raymond : “Non. Cécile, attendez !”")
            (Utilities|FlowControl|Delay 2.0)
            (Default|EndDialogue (Variables|/Game/GD/ThirdPerson/Blueprints/BP_Diplome_First_Person_Project.BP_Diplome_First_Person_Project_C|GetHUD _first_person))
            (bind _item_track (Timeline|Timeline_0 PlayFromStart)
              (:Update
                (Camera|SetFieldOfView (Variables|/Game/GD/ThirdPerson/Blueprints/BP_Diplome_First_Person_Project.BP_Diplome_First_Person_Project_C|GetFirst_Person_Camera (Variables|Default|GetFirst_Person)) (Math|Float|Lerp 9e+01 7e+01 _item_track)))
              (:Finished
                (Variables|Default|SetFirst_Switch_Done_? true)
                (bind _outactors_3 (Actor|GetAllActorsOfClass "/Game/GD/ThirdPerson/Blueprints/BP_Diplome_First_Person_Project.BP_Diplome_First_Person_Project_C"))
                (Pawn|Possess _returnvalue (Utilities|Array|Get(acopy) _outactors_3 1))
                (Input|DisableInput (Utilities|Array|Get(acopy) _outactors_3 1) _returnvalue)
                (bind _item_track_2 (Timeline|Timeline_1 PlayFromStart)
                  (:Update
                    (Camera|SetFieldOfView (Variables|/Game/GD/ThirdPerson/Blueprints/BP_Diplome_First_Person_Project.BP_Diplome_First_Person_Project_C|GetFirst_Person_Camera (Utilities|Array|Get(acopy) _outactors_3 1)) (Math|Float|Lerp 7e+01 9e+01 _item_track_2)))
                  (:Finished
                    (Input|EnableInput (Utilities|Array|Get(acopy) _outactors_3 1) (Game|GetPlayerController 0))))))))))))

(fn ConstructionScript
  (|CallParentFunction))