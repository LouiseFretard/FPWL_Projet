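; Library interactable, a child of the not-inspectable, no-item-needed interaction object, with a hidden-button style mechanism that works once.
; On BeginPlay it sets the classes of two Photo child actors from variables.
; When PartHit reports the Box, chained timelines press it in and back out with click and furniture-moving sounds, then slide the Arrow component along local Y, presumably moving the furniture attached to it.
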(event OnComponentHit(Box)
  (params (HitComponent :type Primitive%20Component%20Object%20Reference) (OtherActor :type Actor%20Object%20Reference) (OtherComp :type Primitive%20Component%20Object%20Reference) (NormalImpulse :type Vector :default "0, 0, 0") (Hit :type Hit%20Result%20Structure%20%28by%20ref%29)))

(event OnClicked(Box)
  (params (TouchedComponent :type Primitive%20Component%20Object%20Reference) (ButtonPressed :type Key%20Structure :default "None")))

(event EventBeginPlay
  (|CallParentFunction)
  (ChildActorComponent|SetChildActorClass (Variables|Default|GetPhoto) (Variables|Default|GetIn%20Class))
  (ChildActorComponent|SetChildActorClass (Variables|Default|GetPhoto1) (Variables|Default|GetIn%20Class_0)))

(event Collision|EventActorBeginOverlap
  (params (OtherActor :type Actor%20Object%20Reference))
  (|CallParentFunction OtherActor) ; This node is disabled and will not be called.\nDrag off pins to build functionality.
)

(event EventTick
  (params (DeltaSeconds :type Float%20%28single-precision%29))
  (|CallParentFunction DeltaSeconds) ; This node is disabled and will not be called.\nDrag off pins to build functionality.
)

(event EventPartHit
  (params (Hit_Component :type Primitive%20Component%20Object%20Reference) (Pawn :type Pawn%20Object%20Reference))
  (if (== Hit_Component (Variables|Default|GetBox))
    (Utilities|FlowControl|DoOnce false
      (:Completed
        (Variables|Default|SetArrow_Relative_Location (Variables|/Script/Engine.SceneComponent|GetRelativeLocation (Variables|Default|GetArrow)))
        (Variables|Default|SetBox_Relative_Location (Variables|/Script/Engine.SceneComponent|GetRelativeLocation (Variables|Default|GetBox)))
        (Audio|PlaySound2D "/Game/GD/Sound/Environment_Noise/SC_Button_Click_Cue.SC_Button_Click_Cue" 1.0 1.0 0.0 0 0)
        (bind _item_track (Timeline|Timeline_1 PlayFromStart)
          (:Update
            (Transformation|SetRelativeLocation (Variables|Default|GetBox) (Math|Vector|Lerp(Vector) (Variables|Default|GetBox_Relative_Location) (Math|Vector|MakeVector (.x (Variables|Default|GetBox_Relative_Location)) (+ (.y (Variables|Default|GetBox_Relative_Location)) -3.0) (.z (Variables|Default|GetBox_Relative_Location))) _item_track) false false))
          (:Finished
            (Variables|Default|SetBox_Relative_Location (Variables|/Script/Engine.SceneComponent|GetRelativeLocation (Variables|Default|GetBox)))
            (Audio|PlaySound2D "/Game/GD/Sound/Environment_Noise/SC_Moving_Furniture_Cue.SC_Moving_Furniture_Cue" 1.0 1.0 1.5 0 0)
            (bind _item_track_2 (Timeline|Timeline_2 PlayFromStart)
              (:Update
                (Transformation|SetRelativeLocation (Variables|Default|GetBox) (Math|Vector|Lerp(Vector) (Variables|Default|GetBox_Relative_Location) (Math|Vector|MakeVector (.x (Variables|Default|GetBox_Relative_Location)) (+ (.y (Variables|Default|GetBox_Relative_Location)) 3.0) (.z (Variables|Default|GetBox_Relative_Location))) _item_track_2) false false))
              (:Finished
                (bind _item_track_3 (Timeline|Timeline_0 PlayFromStart)
                  (:Update
                    (Transformation|SetRelativeLocation (Variables|Default|GetArrow) (Math|Vector|Lerp(Vector) (Variables|Default|GetArrow_Relative_Location) (Math|Vector|MakeVector 0.0 (+ (.y (Variables|Default|GetArrow_Relative_Location)) -1.8e+02) (.z (Variables|Default|GetArrow_Relative_Location))) _item_track_3) false false)))))))))))

(fn ConstructionScript
  (|CallParentFunction))