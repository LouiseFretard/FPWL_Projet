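; Interactable window Blueprint that, going by its name, draws the player's attention by flapping while it is flagged as chaotic.
; On BeginPlay a Delay loop swings Arrow1 and Arrow2 back and forth in opposite yaw directions for as long as ChaoticWindow is true.
; A PartHit on BoxFrontCollision clears the flag, so the loop exits at its next check and snaps both arrows to fixed resting yaws.
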(event EventBeginPlay
  (bind _arrow2 (Variables|Default|GetArrow2))
  (bind _arrow1 (Variables|Default|GetArrow1))
  (bind _arrow1_2 (Variables|Default|GetArrow1))
  (bind _arrow2_2 (Variables|Default|GetArrow2))
  (bind _arrow2_3 (Variables|Default|GetArrow2))
  (bind _arrow1_3 (Variables|Default|GetArrow1))
  (bind _relativerotation (Variables|/Script/Engine.SceneComponent|GetRelativeRotation _arrow1))
  (bind _relativerotation_2 (Variables|/Script/Engine.SceneComponent|GetRelativeRotation _arrow2_2))
  (bind _relativerotation_3 (Variables|/Script/Engine.SceneComponent|GetRelativeRotation _arrow1_2))
  (bind _relativerotation_4 (Variables|/Script/Engine.SceneComponent|GetRelativeRotation _arrow2_3))
  (bind _relativerotation_5 (Variables|/Script/Engine.SceneComponent|GetRelativeRotation _arrow1_3))
  (bind _relativerotation_6 (Variables|/Script/Engine.SceneComponent|GetRelativeRotation _arrow2))
  (|CallParentFunction)
  (if (Variables|Default|GetChaotic_Window_?)
    (Utilities|FlowControl|Delay 0.2 :!label _label)
    (Transformation|SetRelativeRotation _arrow1_3 (Math|Rotator|MakeRotator (.roll _relativerotation_5) (.pitch _relativerotation_5) (+ (.yaw _relativerotation_5) 45.0)) false false)
    (Transformation|SetRelativeRotation _arrow2 (Math|Rotator|MakeRotator (.roll _relativerotation_6) (.pitch _relativerotation_6) (+ (.yaw _relativerotation_6) -45.0)) false false)
    (Utilities|FlowControl|Delay 0.2)
    (if (Variables|Default|GetChaotic_Window_?)
      (Transformation|SetRelativeRotation _arrow1 (Math|Rotator|MakeRotator (.roll _relativerotation) (.pitch _relativerotation) (+ (.yaw _relativerotation) -45.0)) false false)
      (Transformation|SetRelativeRotation _arrow2_2 (Math|Rotator|MakeRotator (.roll _relativerotation_2) (.pitch _relativerotation_2) (+ (.yaw _relativerotation_2) 45.0)) false false)
      (goto _label)
      (else
        _)))
  (Transformation|SetRelativeRotation _arrow1_2 (Math|Rotator|MakeRotator (.roll _relativerotation_3) (.pitch _relativerotation_3) 1.8e+02) false false)
  (Transformation|SetRelativeRotation _arrow2_3 (Math|Rotator|MakeRotator (.roll _relativerotation_4) (.pitch _relativerotation_4) 25.0) false false))

(event Collision|EventActorBeginOverlap
  (params (OtherActor :type Actor%20Object%20Reference))
  (|CallParentFunction OtherActor) ; This node is disabled and will not be called.\nDrag off pins to build functionality.
)

(event EventTick
  (params (DeltaSeconds :type Float%20%28single-precision%29))
  (|CallParentFunction DeltaSeconds) ; This node is disabled and will not be called.\nDrag off pins to build functionality.
)

(event EventPartHit
  (params (Hit_Component :type Primitive%20Component%20Object%20Reference))
  (if (== Hit_Component (Variables|Default|GetBox_Front_Collision))
    (Variables|Default|SetChaotic_Window_? false)))

(fn ConstructionScript
  (|CallParentFunction))