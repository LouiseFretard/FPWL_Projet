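; Interactable kitchen book that plays dialogue and makes a reward available to the player the first time its box is hit.
; On BeginPlay it spawns the Reward class through a child actor component with collision disabled.
; A one-time PartHit on the box sends Dialogue to the player character, flips Arrow1's pitch by 180 degrees, enables reward collision and disables the box's collision.
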(event EventBeginPlay
  (bind _reward_for_player (Variables|Default|GetReward_For_Player))
  (|CallParentFunction)
  (ChildActorComponent|SetChildActorClass _reward_for_player (Variables|Default|GetReward))
  (Collision|SetActorEnableCollision (Variables|/Script/Engine.ChildActorComponent|GetChildActor _reward_for_player) false))

(event Collision|EventActorBeginOverlap
  (params (OtherActor :type Actor%20Object%20Reference))
  (|CallParentFunction OtherActor) ; This node is disabled and will not be called.\nDrag off pins to build functionality.
)

(event EventTick
  (params (DeltaSeconds :type Float%20%28single-precision%29))
  (|CallParentFunction DeltaSeconds) ; This node is disabled and will not be called.\nDrag off pins to build functionality.
)

(event EventPartHit
  (params (Hit_Component :type Primitive%20Component%20Object%20Reference))
  (bind _arrow1 (Variables|Default|GetArrow1))
  (bind _relativerotation (Variables|/Script/Engine.SceneComponent|GetRelativeRotation _arrow1))
  (if (and (== Hit_Component (Variables|Default|GetBox)) (== (Variables|Default|GetOnce) false))
    (bind _asbp_diplome_first_person_project (Utilities|Casting|CastToBP_Diplome_First_Person_Project (Game|GetPlayerCharacter 0)))
    (Default|TransmissDialogue _asbp_diplome_first_person_project (Variables|Default|GetDialogue))
    (Transformation|SetRelativeRotation _arrow1 (Math|Rotator|MakeRotator (.roll _relativerotation) (+ (.pitch _relativerotation) 1.8e+02) (.yaw _relativerotation)) false false)
    (Variables|Default|SetOnce true)
    (Collision|SetActorEnableCollision (Variables|/Script/Engine.ChildActorComponent|GetChildActor (Variables|Default|GetReward_For_Player)) true)
    (Collision|SetCollisionEnabled (Variables|Default|GetBox) "NoCollision")))

(fn ConstructionScript
  (|CallParentFunction))