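; Music box puzzle interactable where the player presses four buttons in the right order to earn a reward.
; Once enabled, interacting blends the player's cinematic camera to a close-up and hands mouse input to the box.
; Cursor hit tests drive timeline-animated presses recorded in an array and compared to the target combination.
; A match rotates the opening arrow and spawns the reward child actor; four wrong presses reset, and right-click exits.
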(event Custom|Got_Right_Combination_?
  (if (== (Utilities|Array|Identical (Variables|Default|GetCombination_To_Do) (Variables|Default|GetCombination_Done)) true)
    (Collision|SetCollisionEnabled (Variables|Default|GetBox) "NoCollision")
    (Input|DisableInput (Game|GetPlayerController 0))
    (Variables|Default|SetMay_Get_Out_Of_The_Minigame_? false)
    (Variables|/Script/Engine.PlayerController|SetbShowMouseCursor (Game|GetPlayerController 0) false)
    (Collision|SetCollisionProfileName (Variables|Default|GetBox) "NoCollision" true :!class /Script/Engine.PrimitiveComponent)
    (Variables|Default|SetOriginal_Relative_Rotation_Opening_Arrow (Variables|/Script/Engine.SceneComponent|GetRelativeRotation (Variables|Default|GetOpening_Arrow)))
    (ChildActorComponent|SetChildActorClass (Variables|Default|GetReward_For_Player) (Variables|Default|GetReward))
    (bind _time_to_move_object (Timeline|Timeline_4 PlayFromStart)
      (:Update
        (Transformation|SetRelativeRotation (Variables|Default|GetOpening_Arrow) (Math|Rotator|Lerp(Rotator) (Variables|Default|GetOriginal_Relative_Rotation_Opening_Arrow) (Math|Rotator|CombineRotators (Variables|Default|GetOriginal_Relative_Rotation_Opening_Arrow) (Math|Vector|RotatorfromAxisandAngle "0.000000,1.000000, 0" 2.6e+02)) _time_to_move_object true) false false)))
    (elif (Math|Boolean|ANDBoolean (== (Variables|Default|GetLeft_Up_Button_May_Be_Pushed) true) (== (Variables|Default|GetLeft_Down_Button_May_Be_Pushed) true) (== (Variables|Default|GetRight_Up_Button_May_Be_Pushed) true) (== (Variables|Default|GetRight_Down_Button_May_Be_Pushed_?) true))
      (Variables|Default|SetCombination_Index 0)
      (Variables|Default|SetLeft_Up_Relative_Location (Variables|/Script/Engine.SceneComponent|GetRelativeLocation (Variables|Default|GetLeft_Up_Button)))
      (Variables|Default|SetLeft_Down_Relative_Location (Variables|/Script/Engine.SceneComponent|GetRelativeLocation (Variables|Default|GetLeft_Down_Button)))
      (Variables|Default|SetRight_Up_Relative_Location (Variables|/Script/Engine.SceneComponent|GetRelativeLocation (Variables|Default|GetRight_Up_Button)))
      (Variables|Default|SetRight_Down_Relative_Location (Variables|/Script/Engine.SceneComponent|GetRelativeLocation (Variables|Default|GetRight_Down_Button)))
      (bind _item_track (Timeline|Timeline_5 PlayFromStart)
        (:Update
          (Transformation|SetRelativeLocation (Variables|Default|GetLeft_Up_Button) (Math|Vector|Lerp(Vector) (Variables|Default|GetLeft_Up_Relative_Location) (Math|Vector|MakeVector (+ (.X (Math|Vector|BreakVector (Variables|Default|GetLeft_Up_Relative_Location))) 5.0) (.Y (Math|Vector|BreakVector (Variables|Default|GetLeft_Up_Relative_Location))) (.Z (Math|Vector|BreakVector (Variables|Default|GetLeft_Up_Relative_Location)))) _item_track) false false)
          (Transformation|SetRelativeLocation (Variables|Default|GetLeft_Down_Button) (Math|Vector|Lerp(Vector) (Variables|Default|GetLeft_Down_Relative_Location) (Math|Vector|MakeVector (+ (.X (Math|Vector|BreakVector (Variables|Default|GetLeft_Down_Relative_Location))) 5.0) (.Y (Math|Vector|BreakVector (Variables|Default|GetLeft_Down_Relative_Location))) (.Z (Math|Vector|BreakVector (Variables|Default|GetLeft_Down_Relative_Location)))) _item_track) false false)
          (Transformation|SetRelativeLocation (Variables|Default|GetRight_Up_Button) (Math|Vector|Lerp(Vector) (Variables|Default|GetRight_Up_Relative_Location) (Math|Vector|MakeVector (+ (.X (Math|Vector|BreakVector (Variables|Default|GetRight_Up_Relative_Location))) 5.0) (.Y (Math|Vector|BreakVector (Variables|Default|GetRight_Up_Relative_Location))) (.Z (Math|Vector|BreakVector (Variables|Default|GetRight_Up_Relative_Location)))) _item_track) false false)
          (Transformation|SetRelativeLocation (Variables|Default|GetRight_Down_Button) (Math|Vector|Lerp(Vector) (Variables|Default|GetRight_Down_Relative_Location) (Math|Vector|MakeVector (+ (.X (Math|Vector|BreakVector (Variables|Default|GetRight_Down_Relative_Location))) 5.0) (.Y (Math|Vector|BreakVector (Variables|Default|GetRight_Down_Relative_Location))) (.Z (Math|Vector|BreakVector (Variables|Default|GetRight_Down_Relative_Location)))) _item_track) false false))
        (:Finished
          (Variables|Default|SetLeft_Up_Button_May_Be_Pushed false)
          (Variables|Default|SetLeft_Down_Button_May_Be_Pushed false)
          (Variables|Default|SetRight_Up_Button_May_Be_Pushed false)
          (Variables|Default|SetRight_Down_Button_May_Be_Pushed_? false)
          (for _index (range 0 3)
            (Utilities|Array|SetArrayElem (Variables|Default|GetCombination_Done) _index 4)))))))

(event Custom|Start_Music_Box
  (Variables|Default|SetCan_Be_Used_?_0 true))

(event Custom|Left_Up_Button_Push
  (if (not (Variables|Default|GetLeft_Up_Button_May_Be_Pushed))
    (Variables|Default|SetButton_Which_Move (Variables|Default|GetLeft_Up_Button))
    (Variables|Default|SetLeft_Up_Button_May_Be_Pushed true)
    (if (== (Variables|Default|GetButton_Which_Move) (Variables|Default|GetLeft_Up_Button))
      (Utilities|Array|SetArrayElem (Variables|Default|GetCombination_Done) (Variables|Default|GetCombination_Index) 0)
      (CallFunction|MoveAButton)
      (Variables|Default|SetCombination_Index (+ (Variables|Default|GetCombination_Index) 1)))))

(event Custom|Left_Down_Button_Push
  (if (not (Variables|Default|GetLeft_Down_Button_May_Be_Pushed))
    (Variables|Default|SetButton_Which_Move (Variables|Default|GetLeft_Down_Button))
    (Variables|Default|SetLeft_Down_Button_May_Be_Pushed true)
    (if (== (Variables|Default|GetButton_Which_Move) (Variables|Default|GetLeft_Down_Button))
      (Utilities|Array|SetArrayElem (Variables|Default|GetCombination_Done) (Variables|Default|GetCombination_Index) 1)
      (CallFunction|MoveAButton)
      (Variables|Default|SetCombination_Index (+ (Variables|Default|GetCombination_Index) 1)))))

(event Custom|Right_Up_Button_Push
  (if (not (Variables|Default|GetRight_Up_Button_May_Be_Pushed))
    (Variables|Default|SetButton_Which_Move (Variables|Default|GetRight_Up_Button))
    (Variables|Default|SetRight_Up_Button_May_Be_Pushed true)
    (if (== (Variables|Default|GetButton_Which_Move) (Variables|Default|GetRight_Up_Button))
      (Utilities|Array|SetArrayElem (Variables|Default|GetCombination_Done) (Variables|Default|GetCombination_Index) 2)
      (CallFunction|MoveAButton)
      (Variables|Default|SetCombination_Index (+ (Variables|Default|GetCombination_Index) 1)))))

(event Custom|Right_Down_Button_Push
  (if (not (Variables|Default|GetRight_Down_Button_May_Be_Pushed_?))
    (Variables|Default|SetButton_Which_Move (Variables|Default|GetRight_Down_Button))
    (Variables|Default|SetRight_Down_Button_May_Be_Pushed_? true)
    (if (== (Variables|Default|GetButton_Which_Move) (Variables|Default|GetRight_Down_Button))
      (Utilities|Array|SetArrayElem (Variables|Default|GetCombination_Done) (Variables|Default|GetCombination_Index) 3)
      (CallFunction|MoveAButton)
      (Variables|Default|SetCombination_Index (+ (Variables|Default|GetCombination_Index) 1)))))

(event Custom|Move_A_Button
  (Variables|Default|SetButton_Which_Move_Original_Relative_Location (Variables|/Script/Engine.SceneComponent|GetRelativeLocation (Variables|Default|GetButton_Which_Move)))
  (bind _item_track (Timeline|Timeline_2 PlayFromStart)
    (:Update
      (Transformation|SetRelativeLocation (Variables|Default|GetButton_Which_Move) (Math|Vector|Lerp(Vector) (Variables|Default|GetButton_Which_Move_Original_Relative_Location) (Math|Vector|MakeVector (+ (.X (Math|Vector|BreakVector (Variables|Default|GetButton_Which_Move_Original_Relative_Location))) -5.0) (.Y (Math|Vector|BreakVector (Variables|Default|GetButton_Which_Move_Original_Relative_Location))) (.Z (Math|Vector|BreakVector (Variables|Default|GetButton_Which_Move_Original_Relative_Location)))) _item_track) false false))
    (:Finished
      (CallFunction|GotRightCombination?))))

(event EventBeginPlay
  (|CallParentFunction) ; This node is disabled and will not be called.\nDrag off pins to build functionality.
)

(event Collision|EventActorBeginOverlap
  (params (OtherActor :type Actor%20Object%20Reference))
  (|CallParentFunction OtherActor) ; This node is disabled and will not be called.\nDrag off pins to build functionality.
)

(event EventTick
  (params (DeltaSeconds :type Float%20%28single-precision%29))
  (|CallParentFunction DeltaSeconds) ; This node is disabled and will not be called.\nDrag off pins to build functionality.
)

(event EventPartHit
  (params (Hit_Component :type Primitive%20Component%20Object%20Reference) (Pawn :type Pawn%20Object%20Reference))
  (bind _asbp_diplome_first_person_project (Utilities|Casting|CastToBP_Diplome_First_Person_Project Pawn))
  (Utilities|IsValid (Variables|Default|GetFirst_Person_0)
    (:Is%20Valid
      _)
    (:Is%20Not%20Valid
      (Variables|Default|SetFirst_Person_0 _asbp_diplome_first_person_project)))
  (if (== Hit_Component (Variables|Default|GetBox))
    (if (Variables|Default|GetCan_Be_Used_?_0)
      (Variables|/Game/GD/ThirdPerson/Blueprints/BP_Diplome_First_Person_Project.BP_Diplome_First_Person_Project_C|SetInto_Minigame_? (Variables|Default|GetFirst_Person_0) true)
      (Variables|/Script/Engine.PlayerController|SetbShowMouseCursor (Game|GetPlayerController 0) true)
      (Collision|SetCollisionProfileName (Variables|Default|GetBox) "None" true :!class /Script/Engine.PrimitiveComponent)
      (Input|DisableInput (Variables|Default|GetFirst_Person_0) (Game|GetPlayerController 0))
      (Collision|SetCollisionProfileName (Variables|Default|GetBox) "NoCollision" true :!class /Script/Engine.PrimitiveComponent)
      (Transformation|SetWorldTransform (Variables|/Game/GD/ThirdPerson/Blueprints/BP_Diplome_First_Person_Project.BP_Diplome_First_Person_Project_C|GetCinematic_Camera (Variables|Default|GetFirst_Person_0)) (Transformation|GetWorldTransform (Variables|/Game/GD/ThirdPerson/Blueprints/BP_Diplome_First_Person_Project.BP_Diplome_First_Person_Project_C|GetFirst_Person_Camera (Variables|Default|GetFirst_Person_0))) false false)
      (Variables|Default|SetFollow_Camera_Transform (Transformation|GetWorldTransform (Variables|/Game/GD/ThirdPerson/Blueprints/BP_Diplome_First_Person_Project.BP_Diplome_First_Person_Project_C|GetCinematic_Camera (Variables|Default|GetFirst_Person_0))))
      (Components|Activation|SetActive (Variables|/Game/GD/ThirdPerson/Blueprints/BP_Diplome_First_Person_Project.BP_Diplome_First_Person_Project_C|GetCinematic_Camera (Variables|Default|GetFirst_Person_0)) true false)
      (Components|Activation|SetActive (Variables|/Game/GD/ThirdPerson/Blueprints/BP_Diplome_First_Person_Project.BP_Diplome_First_Person_Project_C|GetFirst_Person_Camera (Variables|Default|GetFirst_Person_0)) false false)
      (bind _time_to_move_object (Timeline|Timeline_0 PlayFromStart)
        (:Update
          (Transformation|SetWorldTransform (Variables|/Game/GD/ThirdPerson/Blueprints/BP_Diplome_First_Person_Project.BP_Diplome_First_Person_Project_C|GetCinematic_Camera (Variables|Default|GetFirst_Person_0)) (Math|Transform|Lerp(Transform) (Variables|Default|GetFollow_Camera_Transform) (Transformation|GetWorldTransform (Variables|Default|GetCube6)) _time_to_move_object) false false))
        (:Finished
          (Variables|Default|SetFollow_Camera_Transform (Transformation|GetWorldTransform (Variables|/Game/GD/ThirdPerson/Blueprints/BP_Diplome_First_Person_Project.BP_Diplome_First_Person_Project_C|GetCinematic_Camera (Variables|Default|GetFirst_Person_0))))
          (Variables|Default|SetMay_Get_Out_Of_The_Minigame_? true)
          (Input|EnableInput (Game|GetPlayerController 0))
          (Collision|SetCollisionProfileName (Variables|Default|GetLeft_Up_Button) "BlockAll" true :!class /Script/Engine.PrimitiveComponent))))))

(event Input|MouseEvents|RightMouseButton
  (params (Key :type Key%20Structure :default "None"))
  (bind _returnvalue (Game|GetPlayerController 0))
  (bind _first_person_0 (Variables|Default|GetFirst_Person_0))
  (bind _first_person_0_2 (Variables|Default|GetFirst_Person_0))
  (:Pressed
    (if (Variables|Default|GetMay_Get_Out_Of_The_Minigame_?)
      (Input|DisableInput (Game|GetPlayerController 0))
      (Variables|Default|SetMay_Get_Out_Of_The_Minigame_? false)
      (Variables|/Script/Engine.PlayerController|SetbShowMouseCursor (Game|GetPlayerController 0) false)
      (Collision|SetCollisionProfileName (Variables|Default|GetBox) "BlockAll" true :!class /Script/Engine.PrimitiveComponent)
      (bind _time_to_move_object (Timeline|Timeline_1 PlayFromStart)
        (:Update
          (Transformation|SetWorldTransform (Variables|/Game/GD/ThirdPerson/Blueprints/BP_Diplome_First_Person_Project.BP_Diplome_First_Person_Project_C|GetCinematic_Camera _first_person_0_2) (Math|Transform|Lerp(Transform) (Variables|Default|GetFollow_Camera_Transform) (Transformation|GetWorldTransform (Variables|/Game/GD/ThirdPerson/Blueprints/BP_Diplome_First_Person_Project.BP_Diplome_First_Person_Project_C|GetFirst_Person_Camera _first_person_0_2)) _time_to_move_object) false false))
        (:Finished
          (Components|Activation|SetActive (Variables|/Game/GD/ThirdPerson/Blueprints/BP_Diplome_First_Person_Project.BP_Diplome_First_Person_Project_C|GetCinematic_Camera _first_person_0) false false)
          (Components|Activation|SetActive (Variables|/Game/GD/ThirdPerson/Blueprints/BP_Diplome_First_Person_Project.BP_Diplome_First_Person_Project_C|GetFirst_Person_Camera _first_person_0) true false)
          (Variables|/Game/GD/ThirdPerson/Blueprints/BP_Diplome_First_Person_Project.BP_Diplome_First_Person_Project_C|SetInto_Minigame_? _first_person_0 false)
          (Input|DisableInput _returnvalue)
          (Input|EnableInput (Variables|Default|GetFirst_Person_0) _returnvalue)
          (Collision|SetCollisionProfileName (Variables|Default|GetBox) "BlockAll" true :!class /Script/Engine.PrimitiveComponent)
          (Collision|SetCollisionProfileName (Variables|/Game/GD/ThirdPerson/Blueprints/BP_Diplome_First_Person_Project.BP_Diplome_First_Person_Project_C|GetHighlight_Detection (Variables|Default|GetFirst_Person_0)) "OverlapAllDynamic" true :!class /Script/Engine.PrimitiveComponent)
          (Collision|SetCollisionProfileName (Variables|Default|GetLeft_Up_Button) "BlockAll" true :!class /Script/Engine.PrimitiveComponent))))))

(event Input|MouseEvents|LeftMouseButton
  (params (Key :type Key%20Structure :default "None"))
  (bind _returnvalue (Game|GetPlayerController 0))
  (bind _hitresult (Game|Player|GetHitResultUnderCursorbyChannel _returnvalue "TraceTypeQuery1" true))
  (bind _hitcomponent (Collision|BreakHitResult _hitresult))
  (:Released
    (if (== (Variables|Default|GetLeft_Up_Button) _hitcomponent)
      (CallFunction|LeftUpButtonPush)
      (elif (== (Variables|Default|GetLeft_Down_Button) _hitcomponent)
        (CallFunction|LeftDownButtonPush)
        (elif (== (Variables|Default|GetRight_Up_Button) _hitcomponent)
          (CallFunction|RightUpButtonPush)
          (elif (== (Variables|Default|GetRight_Down_Button) _hitcomponent)
            (CallFunction|RightDownButtonPush)))))))

(fn ConstructionScript
  (|CallParentFunction))