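; Match inventory item that animates striking a match and using it to light a fireplace.
; Left click nudges the match out and back; P capsule-traces forward and calls SetFireToMatch if the fireplace can be lit.
; Set_Fire_To_Match chains timelines through step markers, ramping up the point light, then moves the match to the hit fireplace's BoxToBurn, calls SwitchOnFire and destroys the match components.
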(event Custom|Set_Fire_To_Match
  (params (Hit_Actor :type Actor%20Object%20Reference))
  (bind _time_to_move_object (Timeline|Timeline_1 PlayFromStart)
    (:Update
      (Transformation|SetRelativeLocation (Variables|Default|GetMatch) (Math|Vector|Lerp(Vector) (Variables|/Script/Engine.SceneComponent|GetRelativeLocation (Variables|Default|GetCube2)) (Variables|/Script/Engine.SceneComponent|GetRelativeLocation (Variables|Default|Get1st_Step)) _time_to_move_object) false false))
    (:Finished
      (bind _time_to_move_object_2 (Timeline|Timeline_2 PlayFromStart)
        (:Update
          (Transformation|SetRelativeLocation (Variables|Default|GetMatch) (Math|Vector|Lerp(Vector) (Variables|/Script/Engine.SceneComponent|GetRelativeLocation (Variables|Default|Get1st_Step)) (Variables|/Script/Engine.SceneComponent|GetRelativeLocation (Variables|Default|Get2nd_Step)) _time_to_move_object_2) false false))
        (:Finished
          (bind _time_to_move_object_3 (Timeline|Timeline_3 PlayFromStart)
            (:Update
              (Transformation|SetRelativeLocation (Variables|Default|GetMatch) (Math|Vector|Lerp(Vector) (Variables|/Script/Engine.SceneComponent|GetRelativeLocation (Variables|Default|Get2nd_Step)) (Variables|/Script/Engine.SceneComponent|GetRelativeLocation (Variables|Default|Get3rd_Step)) _time_to_move_object_3) false false))
            (:Finished
              (bind _time_to_move_object_4 (Timeline|Timeline_4 PlayFromStart)
                (:Update
                  (Transformation|SetRelativeLocation (Variables|Default|GetMatch) (Math|Vector|Lerp(Vector) (Variables|/Script/Engine.SceneComponent|GetRelativeLocation (Variables|Default|Get3rd_Step)) (Variables|/Script/Engine.SceneComponent|GetRelativeLocation (Variables|Default|Get4th_Step)) _time_to_move_object_4) false false)
                  (Rendering|Components|Light|SetIntensity (Variables|Default|GetPointLight) (Math|Float|Lerp 0.0 5e+03 _time_to_move_object_4)))
                (:Finished
                  (Development|PrintString (Utilities|GetDisplayName Hit_Actor))
                  (bind _asbp_fireplace_child_ini (Utilities|Casting|CastToBp_Fireplace_Child_INI Hit_Actor)
                    (:then
                      (bind _time_to_move_object_5 (Timeline|Timeline_5 PlayFromStart)
                        (:Update
                          (Transformation|SetWorldLocation (Variables|Default|GetMatch) (Math|Vector|Lerp(Vector) (Transformation|GetWorldLocation (Variables|Default|Get4th_Step)) (Transformation|GetWorldLocation (Variables|/Game/GD/Interactainable/Object_Interactable_But_Not_Inspectable/Bp_Fireplace_Child_INI.Bp_Fireplace_Child_INI_C|GetBox_To_Burn _asbp_fireplace_child_ini)) _time_to_move_object_5) false false))
                        (:Finished
                          (Default|SwitchonFire _asbp_fireplace_child_ini)
                          (Components|DestroyComponent (Variables|Default|GetMatch)))))
                    (:CastFailed
                      (Development|PrintString "FAIL"))))))))))))

(event Collision|EventActorBeginOverlap
  (params (OtherActor :type Actor%20Object%20Reference))
  (|CallParentFunction OtherActor) ; This node is disabled and will not be called.\nDrag off pins to build functionality.
)

(event EventTick
  (params (DeltaSeconds :type Float%20%28single-precision%29))
  (|CallParentFunction DeltaSeconds) ; This node is disabled and will not be called.\nDrag off pins to build functionality.
)

(event EventBeginPlay)

(event Input|KeyboardEvents|M
  (params (Key :type Key%20Structure :default "None")))

(event Input|KeyboardEvents|P
  (params (Key :type Key%20Structure :default "None"))
  (bind _arrow1 (Variables|Default|GetArrow1))
  (bind _returnvalue (Transformation|GetWorldLocation _arrow1))
  (:Pressed
    (bind _outhit (Collision|CapsuleTraceByChannel _returnvalue (+ _returnvalue (* (Math|Vector|GetForwardVector _arrow1) 2.5e+02)) 2e+01 2e+01 "TraceTypeQuery1" false 0 "ForDuration"))
    (Development|PrintString (Utilities|GetDisplayName (.HitActor (Collision|BreakHitResult _outhit))))
    (bind _asbp_fireplace_child_ini (Utilities|Casting|CastToBp_Fireplace_Child_INI (.HitActor (Collision|BreakHitResult _outhit))))
    (if (Variables|/Game/GD/Interactainable/Object_Interactable_But_Not_Inspectable/Bp_Fireplace_Child_INI.Bp_Fireplace_Child_INI_C|GetCan_Set_Fire_? _asbp_fireplace_child_ini)
      (CallFunction|SetFiretoMatch))))

(event Input|MouseEvents|LeftMouseButton
  (params (Key :type Key%20Structure :default "None"))
  (:Pressed
    (Utilities|FlowControl|Sequence
      (:then_0
        (bind _time_to_move_object (Timeline|Timeline_0 PlayFromStart)
          (:Update
            (Transformation|SetRelativeLocation (Variables|Default|GetMatch) (Math|Vector|Lerp(Vector) (Variables|/Script/Engine.SceneComponent|GetRelativeLocation (Variables|Default|GetCube2)) (Variables|/Script/Engine.SceneComponent|GetRelativeLocation (Variables|Default|Get1st_Step)) _time_to_move_object) false false))))
      (:then_1
        (Utilities|FlowControl|Delay 1.0)
        (Timeline|Timeline_0 ReverseFromEnd)))))

(fn ConstructionScript
  (|CallParentFunction))