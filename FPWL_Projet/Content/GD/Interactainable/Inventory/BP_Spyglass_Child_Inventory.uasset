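; Spyglass child Blueprint, apparently an inventory variant of an interactable spyglass, that extends its parent's BeginPlay and construction script.
; Custom events switch collision between BlockAll and NoCollision to allow or block taking it, and Active sets inspection and zoom flags.
; A large timeline-driven zoom graph (FOV lerp, cinematic camera swap, arrow-based rotation with pitch clamp) remains but is disconnected and never runs.
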(event Custom|Active
  (Variables|Default|SetActivity_Into_Inspection_But_Finished_? true)
  (Variables|Default|SetZoomed_? true))

(event Custom|May_Take_Spyglass
  (Collision|SetCollisionProfileName (Variables|Default|GetBox) "BlockAll" true :!class /Script/Engine.PrimitiveComponent))

(event Custom|Can't_Take_Spyglass
  (Collision|SetCollisionProfileName (Variables|Default|GetBox) "NoCollision" true :!class /Script/Engine.PrimitiveComponent))

(event EventBeginPlay
  (|CallParentFunction)
  (Collision|SetCollisionProfileName (Variables|Default|GetBox) "BlockAll" true :!class /Script/Engine.PrimitiveComponent))

(event Collision|EventActorBeginOverlap
  (params (OtherActor :type Actor%20Object%20Reference))
  (|CallParentFunction OtherActor) ; This node is disabled and will not be called.\nDrag off pins to build functionality.
)

(event EventTick
  (params (DeltaSeconds :type Float%20%28single-precision%29)))

(event Input|MouseEvents|LeftMouseButton
  (params (Key :type Key%20Structure :default "None")))

(event Input|MouseEvents|RightMouseButton
  (params (Key :type Key%20Structure :default "None")))

(fn ConstructionScript
  (|CallParentFunction))