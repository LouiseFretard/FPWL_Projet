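; BP_Briquet is a lighter inventory item that toggles on and off with a sound, an animated pivot, flame and lights.
; Switch_On_Off uses a FlipFlop, ignoring calls while an animation runs.
; Switching on shows the fire and swings Arrow1 90 degrees in pitch, then a second timeline ramps up both lights.
; Switching off hides the fire and plays both timelines backwards in reverse order, steered by a Reversed flag.
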(event Custom|Switch_On_Off
  (bind _relative_rotation (Variables|Default|GetRelative%20Rotation))
  (if (not (Variables|Default|GetAnimation_Going_?))
    (Variables|Default|SetAnimation_Going_? true)
    (Audio|PlaySound2D "/Game/GD/Sound/Environment_Noise/SC_Lighter_Switch_On_Cue.SC_Lighter_Switch_On_Cue" 1.0 1.0 0.0 0 0)
    (Utilities|FlowControl|FlipFlop
      (:A
        (Rendering|SetVisibility (Variables|Default|GetFire) true false)
        (bind _item_track (Timeline|Timeline_0 PlayFromStart)
          (:Update
            (Transformation|SetRelativeRotation (Variables|Default|GetArrow1) (Math|Rotator|Lerp(Rotator) (Variables|Default|GetRelative%20Rotation) (Math|Rotator|MakeRotator (.roll _relative_rotation) (+ (.pitch _relative_rotation) 9e+01) (.yaw _relative_rotation)) _item_track) false false))
          (:Finished
            (if (Variables|Default|GetReversed_?)
              (Variables|Default|SetReversed_? false)
              (Variables|Default|SetAnimation_Going_? false)
              (else
                (bind _item_track_2 (Timeline|Timeline_1 PlayFromStart)
                  (:Update
                    (Rendering|Components|Light|SetIntensity (Variables|Default|GetPointLight) (Math|Float|Lerp 0.0 (Variables|Default|GetMax_Intensity) _item_track_2))
                    (Rendering|Components|Light|SetIntensity (Variables|Default|GetAdditional) (Math|Float|Lerp 0.0 5e+01 _item_track_2))
                    (Effects|Components|ParticleSystem|SetEmitterEnable (Variables|Default|GetFire) "None" true))
                  (:Finished
                    (if (Variables|Default|GetReversed_?)
                      (Timeline|Timeline_0 ReverseFromEnd)
                      (else
                        (Variables|Default|SetAnimation_Going_? false))))))))))
      (:B
        (Rendering|SetVisibility (Variables|Default|GetFire) false false)
        (Variables|Default|SetReversed_? true)
        (Timeline|Timeline_1 ReverseFromEnd)))))

(event EventBeginPlay
  (|CallParentFunction)
  (Variables|Default|SetRelative%20Rotation (Variables|/Script/Engine.SceneComponent|GetRelativeRotation (Variables|Default|GetArrow1))))

(event Collision|EventActorBeginOverlap
  (params (OtherActor :type Actor%20Object%20Reference))
  (|CallParentFunction OtherActor) ; This node is disabled and will not be called.\nDrag off pins to build functionality.
)

(event EventTick
  (params (DeltaSeconds :type Float%20%28single-precision%29))
  (|CallParentFunction DeltaSeconds) ; This node is disabled and will not be called.\nDrag off pins to build functionality.
)

(fn ConstructionScript
  (|CallParentFunction))