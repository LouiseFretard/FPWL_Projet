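; BP_Actor_To_Save is an actor that exercises a BP_Save_Levels save object when the player touches its Cube.
; BeginPlay creates a fresh save object and keeps it in memory, with no saving to or loading from a slot.
; Cube overlap and hit share one check for BP_Diplome_First_Person_Project: it fills the Phrase field if empty, otherwise prints it.
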(event OnComponentBeginOverlap(Cube)
  (params (OverlappedComponent :type Primitive%20Component%20Object%20Reference) (OtherActor :type Actor%20Object%20Reference) (OtherComp :type Primitive%20Component%20Object%20Reference) (OtherBodyIndex :type Integer) (bFromSweep :type Boolean) (SweepResult :type Hit%20Result%20Structure%20%28by%20ref%29))
  (bind _newvar_0 (Variables|Default|GetNewVar_0))
  (if (== (Utilities|GetClass (stale OnComponentHit(Cube) OtherActor)) "/Game/GD/ThirdPerson/Blueprints/BP_Diplome_First_Person_Project.BP_Diplome_First_Person_Project_C")
    (if (Utilities|Enum|Equal(Enum) (Variables|/Game/GD/Maps/BP_Save_Levels.BP_Save_Levels_C|GetPhrase _newvar_0) "")
      (Variables|/Game/GD/Maps/BP_Save_Levels.BP_Save_Levels_C|SetPhrase _newvar_0 "Oskur")
      (else
        (Development|PrintString (Variables|/Game/GD/Maps/BP_Save_Levels.BP_Save_Levels_C|GetPhrase _newvar_0))))))

(event OnComponentHit(Cube)
  (params (HitComponent :type Primitive%20Component%20Object%20Reference) (OtherActor :type Actor%20Object%20Reference) (OtherComp :type Primitive%20Component%20Object%20Reference) (NormalImpulse :type Vector :default "0, 0, 0") (Hit :type Hit%20Result%20Structure%20%28by%20ref%29))
  (bind _newvar_0 (Variables|Default|GetNewVar_0))
  (if (== (Utilities|GetClass OtherActor) "/Game/GD/ThirdPerson/Blueprints/BP_Diplome_First_Person_Project.BP_Diplome_First_Person_Project_C")
    (if (Utilities|Enum|Equal(Enum) (Variables|/Game/GD/Maps/BP_Save_Levels.BP_Save_Levels_C|GetPhrase _newvar_0) "")
      (Variables|/Game/GD/Maps/BP_Save_Levels.BP_Save_Levels_C|SetPhrase _newvar_0 "Oskur")
      (else
        (Development|PrintString (Variables|/Game/GD/Maps/BP_Save_Levels.BP_Save_Levels_C|GetPhrase _newvar_0))))))

(event EventBeginPlay
  (bind _returnvalue (SaveGame|CreateSaveGameObject "/Game/GD/Maps/BP_Save_Levels.BP_Save_Levels_C"))
  (Variables|Default|SetNewVar_0 _returnvalue))

(event Collision|EventActorBeginOverlap
  (params (OtherActor :type Actor%20Object%20Reference)))

(event EventTick
  (params (DeltaSeconds :type Float%20%28single-precision%29)))

(fn ConstructionScript)