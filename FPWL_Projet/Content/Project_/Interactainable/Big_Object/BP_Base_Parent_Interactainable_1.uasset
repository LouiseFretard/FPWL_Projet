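; Base parent for big interactable objects that the first-person player can inspect and rotate.
; Start_Inspect moves input from the player to the object after a short delay, and the interact key hands it back once TimeToGetRewardFinished is true.
; Mouse axes rotate the Arrow component unless text is shown, which Space toggles on objects that have text.
; Item-check and completion events are empty stubs.
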(event Custom|Start_Inspect
  (params (Inspector :type Pawn%20Object%20Reference) (Enigmes_Accomplie_? :type Boolean))
  (bind _returnvalue (Game|GetPlayerController 0))
  ;[1 1 1] Change_Input_When_Inspect_And_End_Of_Inspection
  (bind _asbp_diplome_first_person_project (Utilities|Casting|CastToBP_Diplome_First_Person_Project Inspector))
  (Variables|Default|SetFirst_Person _asbp_diplome_first_person_project)
  (Variables|/Game/Project_/ThirdPerson/Blueprints/BP_Diplome_First_Person_Project.BP_Diplome_First_Person_Project_C|SetShow_Text_? _asbp_diplome_first_person_project false)
  (Input|DisableInput Inspector _returnvalue)
  (Utilities|FlowControl|Delay 0.6)
  (Input|EnableInput _returnvalue))

(event Custom|Set_If_Finished)

(event Custom|Does_The_Player_Have_The_Right_Item_?)

(event EventBeginPlay)

(event Collision|EventActorBeginOverlap
  (params (OtherActor :type Actor%20Object%20Reference)))

(event Input|ActionEvents|InputActionInteraction_With_Actor
  (params (Key :type Key%20Structure))
  (bind _returnvalue (Game|GetPlayerController 0))
  ;[1 1 1] Change_Input_When_Inspect_And_End_Of_Inspection
  (:Pressed
    (if (Variables|Default|GetTime_To_Get_Reward_Finished_?)
      (Variables|/Game/Project_/ThirdPerson/Blueprints/BP_Diplome_First_Person_Project.BP_Diplome_First_Person_Project_C|SetShow_Text_? (stale Custom|Start_Inspect _asbp_diplome_first_person_project) false)
      (Input|DisableInput _returnvalue)
      (Input|EnableInput (stale Custom|Start_Inspect Inspector) _returnvalue)
      (bind _asbp_diplome_first_person_project (Utilities|Casting|CastToBP_Diplome_First_Person_Project (stale Custom|Start_Inspect Inspector)))
      (Default|Inspect _asbp_diplome_first_person_project false))))

(event Input|MouseEvents|MouseX
  (params (AxisValue :type Float%20%28single-precision%29))
  ;[1 1 1] How_To_Move_Actor_Depending_If_Text_Is_Shown
  (if (not (Variables|/Game/Project_/ThirdPerson/Blueprints/BP_Diplome_First_Person_Project.BP_Diplome_First_Person_Project_C|GetShow_Text_? (Variables|Default|GetFirst_Person)))
    (Transformation|SetRelativeRotation (Variables|Default|GetArrow) (Math|Rotator|CombineRotators (Variables|/Script/Engine.SceneComponent|GetRelativeRotation (Variables|Default|GetArrow)) (Math|Rotator|MakeRotator (* AxisValue -1.0) 0.0 0.0)) false false)))

(event Input|MouseEvents|MouseY
  (params (AxisValue :type Float%20%28single-precision%29))
  ;[1 1 1] How_To_Move_Actor_Depending_If_Text_Is_Shown
  (if (not (Variables|/Game/Project_/ThirdPerson/Blueprints/BP_Diplome_First_Person_Project.BP_Diplome_First_Person_Project_C|GetShow_Text_? (Variables|Default|GetFirst_Person)))
    (Transformation|SetRelativeRotation (Variables|Default|GetArrow) (Math|Rotator|CombineRotators (Variables|/Script/Engine.SceneComponent|GetRelativeRotation (Variables|Default|GetArrow)) (Math|Rotator|MakeRotator 0.0 (* AxisValue -1.0) 0.0)) false false)))

(event Input|KeyboardEvents|SpaceBar
  (params (Key :type Key%20Structure))
  (bind _first_person (Variables|Default|GetFirst_Person))
  ;[1 1 1] Show_Text_Or_Not
  (:Pressed
    (if (Variables|Default|GetGot_An_Text_?)
      (Utilities|FlowControl|FlipFlop
        (:A
          (Variables|/Game/Project_/ThirdPerson/Blueprints/BP_Diplome_First_Person_Project.BP_Diplome_First_Person_Project_C|SetShow_Text_? _first_person true))
        (:B
          (Variables|/Game/Project_/ThirdPerson/Blueprints/BP_Diplome_First_Person_Project.BP_Diplome_First_Person_Project_C|SetShow_Text_? _first_person false))))))

(fn ConstructionScript)