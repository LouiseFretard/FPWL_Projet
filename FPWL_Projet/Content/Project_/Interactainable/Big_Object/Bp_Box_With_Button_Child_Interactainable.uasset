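; Interactable puzzle box with four side buttons that must be pressed in the right order to release a reward.
; A left-click camera trace finds an unpressed button, slides it with a timeline and records its number in the attempted combination.
; After four presses, a match raises the reward holder and spawns a letter or item child actor, while a mismatch resets the buttons.
; SetifFinished snaps buttons and reward holder to their solved positions.
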(event EventBeginPlay
  ;[1 1 1] Get_Importants_Variables
  (|CallParentFunction)
  (CallFunction|SetOriginalLocationOfButton (Variables|/Script/Engine.SceneComponent|GetRelativeLocation (Variables|Default|GetFront_Button)) (Variables|/Script/Engine.SceneComponent|GetRelativeLocation (Variables|Default|GetLeft_Button)) (Variables|/Script/Engine.SceneComponent|GetRelativeLocation (Variables|Default|GetBack_Button)) (Variables|/Script/Engine.SceneComponent|GetRelativeLocation (Variables|Default|GetRight_Button))))

(event Collision|EventActorBeginOverlap
  (params (OtherActor :type Actor%20Object%20Reference))
  (|CallParentFunction OtherActor) ; This node is disabled and will not be called.\nDrag off pins to build functionality.
)

(event EventTick
  (params (DeltaSeconds :type Float%20%28single-precision%29)))

(event EventSetifFinished
  (bind _front_button (Variables|Default|GetFront_Button))
  (bind _left_button (Variables|Default|GetLeft_Button))
  (bind _back_button (Variables|Default|GetBack_Button))
  (bind _right_button (Variables|Default|GetRight_Button))
  (bind _place_for_reward (Variables|Default|GetPlace_For_Reward))
  ;[1 1 1] If_Succesfuly_Finished_Set_Postion_Of_Buttons_And_Reward
  (CallFunction|SetLocationOfButtonifRiddleFinished _front_button _left_button _back_button _right_button _place_for_reward (Variables|/Script/Engine.SceneComponent|GetRelativeLocation _front_button) (Variables|/Script/Engine.SceneComponent|GetRelativeLocation _left_button) (Variables|/Script/Engine.SceneComponent|GetRelativeLocation _back_button) (Variables|/Script/Engine.SceneComponent|GetRelativeLocation _right_button) (Variables|/Script/Engine.SceneComponent|GetRelativeLocation _place_for_reward)))

(event EventDoesthePlayerHavetheRightItem?)

(event Input|MouseEvents|LeftMouseButton
  (params (Key :type Key%20Structure :default "None"))
  (bind _reward (Variables|Default|GetReward))
  (bind _front_button (Variables|Default|GetFront_Button))
  (bind _front_button_2 (Variables|Default|GetFront_Button))
  (bind _left_button (Variables|Default|GetLeft_Button))
  (bind _back_button (Variables|Default|GetBack_Button))
  (bind _right_button (Variables|Default|GetRight_Button))
  (bind _back_button_2 (Variables|Default|GetBack_Button))
  (bind _left_button_2 (Variables|Default|GetLeft_Button))
  (bind _reward_2 (Variables|Default|GetReward))
  (bind _right_button_2 (Variables|Default|GetRight_Button))
  (bind _place_for_reward (Variables|Default|GetPlace_For_Reward))
  (bind _relativelocation (Variables|/Script/Engine.SceneComponent|GetRelativeLocation _front_button_2))
  (bind _relativelocation_2 (Variables|/Script/Engine.SceneComponent|GetRelativeLocation _left_button))
  (bind _relativelocation_3 (Variables|/Script/Engine.SceneComponent|GetRelativeLocation _back_button))
  (bind _relativelocation_4 (Variables|/Script/Engine.SceneComponent|GetRelativeLocation _right_button))
  (bind _relativelocation_5 (Variables|/Script/Engine.SceneComponent|GetRelativeLocation _place_for_reward))
  (bind _childactor (Variables|/Script/Engine.ChildActorComponent|GetChildActor _reward))
  ;[1 1 1] Ray_To_Hit_Button
  (:Pressed
    (bind _outhit (CallFunction|PushButton))
    ;[1 1 1] What_Button_Is_Hit_And_Only_Allow_One_Hit_By_Button_By_Try
    (bind _returnvalue (CallFunction|CheckWhatButtonIsPushedandifItsAlreadyBeenPushed (.HitComponent (Collision|BreakHitResult _outhit)) (Variables|Default|GetFront_Box) (Variables|Default|GetFront_Button_Activated_?)))
    (if _returnvalue
      ;[1 1 1] Move_Button_Forbid_Them_To_Move_Until_New_Try_And_Assign_Them_A_Number_For_Check_If_Sucess
      (Variables|Default|SetFront_Button_Activated_? true)
      (bind _complete_button_movement (Timeline|Timeline_5 PlayFromStart)
        (:Update
          (CallFunction|TrajectforAActorinATime _relativelocation (+ _relativelocation "1.000000,0,0") _complete_button_movement _front_button_2))
        (:Finished
          (Utilities|Array|SetArrayElem (Variables|Default|GetCombination_Actual) (Variables|Default|GetIndex) 1)
          ;[1 1 1] Change_of_Index_And_Verification_If_Player_Succesfuly_Find_The_Right_Combination
          (if (> (+ (Variables|Default|GetIndex) 1) 3) :!label _label
            (Variables|Default|SetIndex 0)
            (if (Utilities|Array|Identical (Variables|Default|GetCombination_To_Get) (Variables|Default|GetCombination_Actual))
              (Variables|Default|SetTime_To_Get_Reward_Finished_? false)
              ;[1 1 1] What_To_Do_If_Good_Combination
              (Variables|Default|SetRiddle_Ended_? true)
              (bind _complete_button_movement_2 (Timeline|Timeline_3 PlayFromStart)
                (:Update
                  (CallFunction|TrajectforAActorinATime _relativelocation_5 (+ _relativelocation_5 "0,0,1.000000") _complete_button_movement_2 _place_for_reward)
                  (Utilities|FlowControl|Delay 0.6)
                  (ChildActorComponent|SetChildActorClass (Variables|Default|GetReward) (Variables|Default|GetGet_Reward_Class_V_2))
                  (bind _complete_button_movement_3 (Timeline|Timeline_6 PlayFromStart)
                    (:Update
                      (CallFunction|TrajectforAActorinATime (Variables|/Script/Engine.SceneComponent|GetRelativeLocation _reward_2) (Variables|/Script/Engine.SceneComponent|GetRelativeLocation (Variables|Default|GetSee_Reward)) _complete_button_movement_3 _reward_2))
                    (:Finished
                      (Utilities|Casting|CastToBP_Base_Parent_Interactainable_Letter _childactor
                        (:then
                          (Variables|Default|SetItem_To_Finish_This_Actor_Is_1_Letter_2_Item 1.0)
                          (Game|SetGamePaused true)
                          (Utilities|FlowControl|Delay 2.0)
                          (Game|SetGamePaused false)
                          (ChildActorComponent|SetChildActorClass (Variables|Default|GetReward) 0))
                        (:CastFailed
                          (Utilities|Casting|CastToBP_Base_Parent_Inventory_Item _childactor)
                          (Variables|Default|SetItem_To_Finish_This_Actor_Is_1_Letter_2_Item 2.0)
                          (Game|SetGamePaused true)
                          (Utilities|FlowControl|Delay 2.0)
                          (Game|SetGamePaused false)
                          (ChildActorComponent|SetChildActorClass (Variables|Default|GetReward) 0)))
                      (Variables|Default|SetTime_To_Get_Reward_Finished_? true)))))
              (else
                ;[1 1 1] What_To_Do_If_Bad_Combination
                (bind _complete_button_movement_4 (Timeline|Timeline_4 PlayFromStart)
                  (:Update
                    (CallFunction|TrajectforAActorinATime (Variables|/Script/Engine.SceneComponent|GetRelativeLocation _left_button_2) (Variables|Default|GetOriginal_Relative_Location_Left_Button) _complete_button_movement_4 _left_button_2)
                    (CallFunction|TrajectforAActorinATime (Variables|/Script/Engine.SceneComponent|GetRelativeLocation _front_button) (Variables|Default|GetOriginal_Relative_Location_Front_Button) _complete_button_movement_4 _front_button)
                    (CallFunction|TrajectforAActorinATime (Variables|/Script/Engine.SceneComponent|GetRelativeLocation _back_button_2) (Variables|Default|GetOriginal_Relative_Location_Back_Button) _complete_button_movement_4 _back_button_2)
                    (CallFunction|TrajectforAActorinATime (Variables|/Script/Engine.SceneComponent|GetRelativeLocation _right_button_2) (Variables|Default|GetOriginal_Relative_Location_Right_Button) _complete_button_movement_4 _right_button_2))
                  (:Finished
                    (CallFunction|ResetButtonActivationifCombinationFailed)))))
            (else
              (Variables|Default|SetIndex (+ (Variables|Default|GetIndex) 1))))))
      (else
        (bind _returnvalue_2 (CallFunction|CheckWhatButtonIsPushedandifItsAlreadyBeenPushed (.HitComponent (Collision|BreakHitResult _outhit)) (Variables|Default|GetLeft_Box) (Variables|Default|GetLeft_Button_Activated_?)))
        (if _returnvalue_2
          (Variables|Default|SetLeft_Button_Activated_? true)
          (bind _complete_button_movement_5 (Timeline|Timeline_0 PlayFromStart)
            (:Update
              (CallFunction|TrajectforAActorinATime _relativelocation_2 (+ _relativelocation_2 "0.000000,1.000000,0") _complete_button_movement_5 _left_button))
            (:Finished
              (Utilities|Array|SetArrayElem (Variables|Default|GetCombination_Actual) (Variables|Default|GetIndex) 2)
              (goto _label)))
          (else
            (bind _returnvalue_3 (CallFunction|CheckWhatButtonIsPushedandifItsAlreadyBeenPushed (.HitComponent (Collision|BreakHitResult _outhit)) (Variables|Default|GetBack_Box) (Variables|Default|GetBack_Button_Activated_?)))
            (if _returnvalue_3
              (Variables|Default|SetBack_Button_Activated_? true)
              (bind _complete_button_movement_6 (Timeline|Timeline_1 PlayFromStart)
                (:Update
                  (CallFunction|TrajectforAActorinATime _relativelocation_3 (+ _relativelocation_3 "-1.000000,0,0") _complete_button_movement_6 _back_button))
                (:Finished
                  (Utilities|Array|SetArrayElem (Variables|Default|GetCombination_Actual) (Variables|Default|GetIndex) 3)
                  (goto _label)))
              (else
                (bind _returnvalue_4 (CallFunction|CheckWhatButtonIsPushedandifItsAlreadyBeenPushed (.HitComponent (Collision|BreakHitResult _outhit)) (Variables|Default|GetRight_Box) (Variables|Default|GetRight_Button_Activated_?)))
                (if _returnvalue_4
                  (Variables|Default|SetRight_Button_Activated_? true)
                  (bind _complete_button_movement_7 (Timeline|Timeline_2 PlayFromStart)
                    (:Update
                      (CallFunction|TrajectforAActorinATime _relativelocation_4 (+ _relativelocation_4 "0.000000,-1.000000,0") _complete_button_movement_7 _right_button))
                    (:Finished
                      (Utilities|Array|SetArrayElem (Variables|Default|GetCombination_Actual) (Variables|Default|GetIndex) 4)
                      (goto _label))))))))))))

(fn ConstructionScript
  (|CallParentFunction))

(fn PushButton
  (bind _camera (Variables|Default|GetCamera))
  (bind _returnvalue (Transformation|GetWorldLocation _camera))
  (if (not (Variables|Default|GetRiddle_Ended_?))
    (bind _outhit (Collision|LineTraceByChannel _returnvalue (+ _returnvalue (* (Math|Vector|GetForwardVector _camera) 2.5e+02)) "TraceTypeQuery1" false 0 "None" false))
    (return _outhit)))

(fn CheckWhatButtonIsPushedandifItsAlreadyBeenPushed
  (params (Component_Hit :type Object%20Object%20Reference) (Get_Box :type Object%20Object%20Reference) (Button_Activated_? :type Boolean))
  (return (and (== Component_Hit Get_Box) (== Button_Activated_? false))))

(fn SetOriginalLocationOfButton
  (params (Original_Relative_Location_Front_Button :type Vector) (Original_Relative_Location_Left_Button :type Vector) (Original_Relative_Location_Back_Button :type Vector) (Original_Relative_Location_Right_Button :type Vector))
  (Variables|Default|SetOriginal_Relative_Location_Front_Button Original_Relative_Location_Front_Button)
  (Variables|Default|SetOriginal_Relative_Location_Left_Button Original_Relative_Location_Left_Button)
  (Variables|Default|SetOriginal_Relative_Location_Back_Button Original_Relative_Location_Back_Button)
  (Variables|Default|SetOriginal_Relative_Location_Right_Button Original_Relative_Location_Right_Button))

(fn SetLocationOfButtonifRiddleFinished
  (params (Front_Button :type Scene%20Component%20Object%20Reference) (Left_Button :type Scene%20Component%20Object%20Reference) (Back_Button :type Scene%20Component%20Object%20Reference) (Right_Button :type Scene%20Component%20Object%20Reference) (Place_For_Reward :type Scene%20Component%20Object%20Reference) (Front_Relative_Location :type Vector) (Left_Relative_Location :type Vector) (Back_Relative_Location :type Vector) (Right_Relative_Location :type Vector) (Place_For_Reward_Relative_Location :type Vector))
  (Transformation|SetRelativeLocation Front_Button (+ Front_Relative_Location "100.000000,0,0") false false)
  (Transformation|SetRelativeLocation Left_Button (+ Left_Relative_Location "0.000000,100.000000,0") false false)
  (Transformation|SetRelativeLocation Back_Button (+ Back_Relative_Location "-100.000000,0,0") false false)
  (Transformation|SetRelativeLocation Right_Button (+ Right_Relative_Location "0.000000,-100.000000,0") false false)
  (Transformation|SetRelativeLocation Place_For_Reward (+ Place_For_Reward_Relative_Location "0,0.000000,15.000000") false false))

(fn TrajectforAActorinATime
  (params (Original_Location :type Vector) (New_Location :type Vector) (Complete_Button_Movement :type Float%20%28single-precision%29) (Actor :type Scene%20Component%20Object%20Reference))
  (Transformation|SetRelativeLocation Actor (Math|Vector|Lerp(Vector) Original_Location New_Location Complete_Button_Movement) false false))

(fn ResetButtonActivationifCombinationFailed
  (Variables|Default|SetFront_Button_Activated_? false)
  (Variables|Default|SetBack_Button_Activated_? false)
  (Variables|Default|SetLeft_Button_Activated_? false)
  (Variables|Default|SetRight_Button_Activated_? false))