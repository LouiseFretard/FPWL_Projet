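; Base parent actor for inventory items that the first-person player can inspect, such as readable letters.
; Start_Inspect moves input from the player to the item, where mouse movement rotates its Arrow component unless text is shown.
; Space toggles the player's ShowText flag and the mouse wheel forwards to ChangeLetter.
; R or E returns input and calls Inspect(false), or GetOutOfInventoryLetter when the game is paused.
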(event Custom|Start_Inspect
  (params (Inspector :type Pawn%20Object%20Reference) (Enigmes_Accomplie_? :type Boolean))
  (bind _returnvalue (Game|GetPlayerController 0))
  (bind _asbp_diplome_first_person_project (Utilities|Casting|CastToBP_Diplome_First_Person_Project Inspector))
  (Variables|Default|SetFirst_Person _asbp_diplome_first_person_project)
  (Input|DisableInput Inspector _returnvalue)
  (Input|EnableInput _returnvalue))

(event EventBeginPlay)

(event Collision|EventActorBeginOverlap
  (params (OtherActor :type Actor%20Object%20Reference)))

(event EventTick
  (params (DeltaSeconds :type Float%20%28single-precision%29)))

(event Input|MouseEvents|MouseX
  (params (AxisValue :type Float%20%28single-precision%29))
  ;[1 1 1] How_To_Move_Actor_Depending_If_Text_Is_Shown
  (if (not (Variables|/Game/Project_/ThirdPerson/Blueprints/BP_Diplome_First_Person_Project.BP_Diplome_First_Person_Project_C|GetShow_Text_? (Variables|Default|GetFirst_Person)))
    (Transformation|SetRelativeRotation (Variables|Default|GetArrow) (Math|Rotator|CombineRotators (Variables|/Script/Engine.SceneComponent|GetRelativeRotation (Variables|Default|GetArrow)) (Math|Rotator|MakeRotator (* AxisValue -1.0) 0.0 0.0)) false false)))

(event Input|MouseEvents|MouseY
  (params (AxisValue :type Float%20%28single-precision%29))
  ;[1 1 1] How_To_Move_Actor_Depending_If_Text_Is_Shown
  (if (not (Variables|/Game/Project_/ThirdPerson/Blueprints/BP_Diplome_First_Person_Project.BP_Diplome_First_Person_Project_C|GetShow_Text_? (Variables|Default|GetFirst_Person)))
    (Transformation|SetRelativeRotation (Variables|Default|GetArrow) (Math|Rotator|CombineRotators (Variables|/Script/Engine.SceneComponent|GetRelativeRotation (Variables|Default|GetArrow)) (Math|Rotator|MakeRotator 0.0 (* AxisValue -1.0) 0.0)) false false)))

(event Input|KeyboardEvents|E
  (params (Key :type Key%20Structure))
  (bind _returnvalue (Game|GetPlayerController 0))
  (:Pressed
    (Input|DisableInput _returnvalue)
    (Input|EnableInput (stale Custom|Start_Inspect Inspector) _returnvalue)
    (bind _asbp_diplome_first_person_project (Utilities|Casting|CastToBP_Diplome_First_Person_Project (stale Custom|Start_Inspect Inspector)))
    (if (not (Game|IsGamePaused))
      (Default|Inspect _asbp_diplome_first_person_project false)
      (else
        (Default|GetOutOfInventoryLetter _asbp_diplome_first_person_project)))))

(event Input|KeyboardEvents|SpaceBar
  (params (Key :type Key%20Structure))
  ;[1 1 1] Show_Text_Or_Not
  (:Pressed
    (bind _asbp_diplome_first_person_project (Utilities|Casting|CastToBP_Diplome_First_Person_Project (stale Custom|Start_Inspect Inspector)))
    (Utilities|FlowControl|FlipFlop
      (:A
        (Variables|/Game/Project_/ThirdPerson/Blueprints/BP_Diplome_First_Person_Project.BP_Diplome_First_Person_Project_C|SetShow_Text_? _asbp_diplome_first_person_project true))
      (:B
        (Variables|/Game/Project_/ThirdPerson/Blueprints/BP_Diplome_First_Person_Project.BP_Diplome_First_Person_Project_C|SetShow_Text_? _asbp_diplome_first_person_project false)))))

(event Input|KeyboardEvents|R
  (params (Key :type Key%20Structure))
  (bind _returnvalue (Game|GetPlayerController 0))
  (:Pressed
    (Input|DisableInput _returnvalue)
    (Input|EnableInput (stale Custom|Start_Inspect Inspector) _returnvalue)
    (bind _asbp_diplome_first_person_project (Utilities|Casting|CastToBP_Diplome_First_Person_Project (stale Custom|Start_Inspect Inspector)))
    (if (not (Game|IsGamePaused))
      (Default|Inspect _asbp_diplome_first_person_project false)
      (else
        (Default|GetOutOfInventoryLetter _asbp_diplome_first_person_project)))))

(event Input|MouseEvents|MouseWheelDown
  (params (Key :type Key%20Structure))
  ;[1 1 1] Change_Of_Letter
  (:Pressed
    (bind _asbp_diplome_first_person_project (Utilities|Casting|CastToBP_Diplome_First_Person_Project (stale Custom|Start_Inspect Inspector)))
    (if (== (stale Input|MouseEvents|MouseWheelUp Key) "MouseScrollUp")
      (Default|ChangeLetter _asbp_diplome_first_person_project (stale Input|MouseEvents|MouseWheelUp Key))
      (else
        (Default|ChangeLetter _asbp_diplome_first_person_project Key)))))

(event Input|MouseEvents|MouseWheelUp
  (params (Key :type Key%20Structure))
  ;[1 1 1] Change_Of_Letter
  (:Pressed
    (bind _asbp_diplome_first_person_project (Utilities|Casting|CastToBP_Diplome_First_Person_Project (stale Custom|Start_Inspect Inspector)))
    (if (== Key "MouseScrollUp")
      (Default|ChangeLetter _asbp_diplome_first_person_project Key)
      (else
        (Default|ChangeLetter _asbp_diplome_first_person_project (stale Input|MouseEvents|MouseWheelDown Key))))))

(fn ConstructionScript)