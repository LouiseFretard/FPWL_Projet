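; Base inventory item actor that the first-person player can inspect, with a proximity clue on how to get it.
; Start_Inspect shows the HUD and moves input to the item, so mouse axes rotate its Arrow unless text is shown.
; Right click exits inspection, or the inventory letter when paused.
; Collision overlaps toggle the clue, which Tick aligns to the player camera from first overlap onward.
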(event OnComponentBeginOverlap(Collision_To_Show_Clue)
  (params (OverlappedComponent :type Primitive%20Component%20Object%20Reference) (OtherActor :type Actor%20Object%20Reference) (OtherComp :type Primitive%20Component%20Object%20Reference) (OtherBodyIndex :type Integer) (bFromSweep :type Boolean) (SweepResult :type Hit%20Result%20Structure%20%28by%20ref%29))
  (Utilities|Casting|CastToBP_Diplome_First_Person_Project OtherActor)
  (Variables|Default|SetCan_Turn_With_Player_? true)
  (Development|SetHiddeninGame (Variables|Default|GetClue_To_How_Get_Item) false false))

(event OnComponentEndOverlap(Collision_To_Show_Clue)
  (params (OverlappedComponent :type Primitive%20Component%20Object%20Reference) (OtherActor :type Actor%20Object%20Reference) (OtherComp :type Primitive%20Component%20Object%20Reference) (OtherBodyIndex :type Integer))
  (Utilities|Casting|CastToBP_Diplome_First_Person_Project OtherActor)
  (Variables|Default|SetCan_Turn_With_Player_? true)
  (Development|SetHiddeninGame (Variables|Default|GetClue_To_How_Get_Item) true false))

(event Custom|Start_Inspect
  (params (Inspector :type Pawn%20Object%20Reference) (Enigmes_Accomplie_? :type Boolean))
  (bind _returnvalue (Game|GetPlayerController 0))
  (bind _asbp_diplome_first_person_project (Utilities|Casting|CastToBP_Diplome_First_Person_Project Inspector))
  (bind _output_get (Variables|Default|SetFirst_Person _asbp_diplome_first_person_project))
  (Widget|SetVisibility (Variables|/Game/GD/ThirdPerson/Blueprints/BP_Diplome_First_Person_Project.BP_Diplome_First_Person_Project_C|GetHUD _output_get) "Visible")
  (Input|DisableInput Inspector _returnvalue)
  (Input|EnableInput _returnvalue))

(event EventBeginPlay)

(event Collision|EventActorBeginOverlap
  (params (OtherActor :type Actor%20Object%20Reference)))

(event EventTick
  (params (DeltaSeconds :type Float%20%28single-precision%29))
  (if (Variables|Default|GetCan_Turn_With_Player_?)
    (bind _asbp_diplome_first_person_project (Utilities|Casting|CastToBP_Diplome_First_Person_Project (Game|GetPlayerCharacter 0)))
    (Transformation|SetWorldRotation (Variables|Default|GetClue_To_How_Get_Item) (Math|Rotator|MakeRotator (.roll (Transformation|GetWorldRotation (Variables|/Game/GD/ThirdPerson/Blueprints/BP_Diplome_First_Person_Project.BP_Diplome_First_Person_Project_C|GetFirst_Person_Camera _asbp_diplome_first_person_project))) (+ (.pitch (Transformation|GetWorldRotation (Variables|/Game/GD/ThirdPerson/Blueprints/BP_Diplome_First_Person_Project.BP_Diplome_First_Person_Project_C|GetFirst_Person_Camera _asbp_diplome_first_person_project))) 9e+01) (.yaw (Transformation|GetWorldRotation (Variables|/Game/GD/ThirdPerson/Blueprints/BP_Diplome_First_Person_Project.BP_Diplome_First_Person_Project_C|GetFirst_Person_Camera _asbp_diplome_first_person_project)))) false false)))

(event Input|MouseEvents|MouseX
  (params (AxisValue :type Float%20%28single-precision%29))
  ;[1 1 1] How_To_Move_Actor_Depending_If_Text_Is_Shown
  (if (not (Variables|/Game/GD/ThirdPerson/Blueprints/BP_Diplome_First_Person_Project.BP_Diplome_First_Person_Project_C|GetShow_Text_? (Variables|Default|GetFirst_Person)))
    (Transformation|SetRelativeRotation (Variables|Default|GetArrow) (Math|Rotator|CombineRotators (Variables|/Script/Engine.SceneComponent|GetRelativeRotation (Variables|Default|GetArrow)) (Math|Rotator|MakeRotator (* AxisValue -1.0) 0.0 0.0)) false false)))

(event Input|MouseEvents|MouseY
  (params (AxisValue :type Float%20%28single-precision%29))
  ;[1 1 1] How_To_Move_Actor_Depending_If_Text_Is_Shown
  (if (not (Variables|/Game/GD/ThirdPerson/Blueprints/BP_Diplome_First_Person_Project.BP_Diplome_First_Person_Project_C|GetShow_Text_? (Variables|Default|GetFirst_Person)))
    (Transformation|SetRelativeRotation (Variables|Default|GetArrow) (Math|Rotator|CombineRotators (Variables|/Script/Engine.SceneComponent|GetRelativeRotation (Variables|Default|GetArrow)) (Math|Rotator|MakeRotator 0.0 (* AxisValue -1.0) 0.0)) false false)))

(event Input|KeyboardEvents|SpaceBar
  (params (Key :type Key%20Structure :default "None"))
  ;[1 1 1] Show_Text_Or_Not
)

(event Input|MouseEvents|RightMouseButton
  (params (Key :type Key%20Structure :default "None"))
  (:Pressed
    (Input|DisableInput (Game|GetPlayerController 0))
    (bind _asbp_diplome_first_person_project (Utilities|Casting|CastToBP_Diplome_First_Person_Project (stale Custom|Start_Inspect Inspector)))
    (if (not (Game|IsGamePaused))
      (Default|Inspect _asbp_diplome_first_person_project false)
      (else
        (Default|GetOutOfInventoryLetter _asbp_diplome_first_person_project)))))

(fn ConstructionScript)