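; Interactable hinged door that swings away from the side the player hits, optionally requiring a specific letter or held item.
; Activation checks that requirement, then snaps the door arrow's rotation open, plays dialogue and disables its trigger collisions.
; A failed held-item check wiggles and rattles the door, or gives rust dialogue if rusted.
; An overlap zone reveals two clues, which Tick turns to match the player camera.
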(event OnComponentBeginOverlap(Collision_To_Show_Clue_2)
  (params (OverlappedComponent :type Primitive%20Component%20Object%20Reference) (OtherActor :type Actor%20Object%20Reference) (OtherComp :type Primitive%20Component%20Object%20Reference) (OtherBodyIndex :type Integer) (bFromSweep :type Boolean) (SweepResult :type Hit%20Result%20Structure%20%28by%20ref%29))
  (Utilities|Casting|CastToBP_Diplome_First_Person_Project OtherActor)
  (Variables|Default|SetCan_Turn_With_Player_? true)
  (Development|SetHiddeninGame (Variables|Default|GetClue_To_How_Get_Item) false false))

(event OnComponentEndOverlap(Collision_To_Show_Clue_2)
  (params (OverlappedComponent :type Primitive%20Component%20Object%20Reference) (OtherActor :type Actor%20Object%20Reference) (OtherComp :type Primitive%20Component%20Object%20Reference) (OtherBodyIndex :type Integer))
  (Utilities|Casting|CastToBP_Diplome_First_Person_Project OtherActor)
  (Variables|Default|SetCan_Turn_With_Player_? false)
  (Development|SetHiddeninGame (Variables|Default|GetClue_To_How_Get_Item) true false))

(event Custom|Open_Doors
  (bind _arrow_door (Variables|Default|GetArrow_Door))
  (bind _arrow_door_2 (Variables|Default|GetArrow_Door))
  (bind _relativerotation (Variables|/Script/Engine.SceneComponent|GetRelativeRotation _arrow_door))
  (bind _relativerotation_2 (Variables|/Script/Engine.SceneComponent|GetRelativeRotation _arrow_door_2))
  (if (not (Variables|Default|GetRouille_?))
    (Audio|SpawnSoundAttached "/Game/GD/Sound/Environment_Noise/SC_Door_Opening_Cue.SC_Door_Opening_Cue" (Variables|Default|GetDoor) "None" "0, 0, 0" "0, 0, 0" "SnapToTarget" false 1.0 1.0 0.0 0 0)
    (Variables|Default|SetOpen_? true)
    (Transformation|SetRelativeRotation (Variables|Default|GetArrow_Door) (Math|Rotator|MakeRotator (.roll _relativerotation_2) (.pitch _relativerotation_2) (+ (.yaw _relativerotation_2) (* (Variables|Default|GetWhat_Side_To_Open) 1e+01))) false false)
    (Default|TransmissDialogue (Variables|Default|GetFirst_Person) (Variables|Default|GetDialogue_De_Succès))
    (Collision|SetCollisionProfileName (Variables|Default|GetBox_Back_Collision) "NoCollision" true :!class /Script/Engine.PrimitiveComponent)
    (else
      (Variables|Default|SetOpen_? true)
      (Transformation|SetRelativeRotation (Variables|Default|GetArrow_Door) (Math|Rotator|MakeRotator (.roll _relativerotation) (.pitch _relativerotation) (+ (.yaw _relativerotation) (* (Variables|Default|GetWhat_Side_To_Open) 9.0))) false false)
      (Default|TransmissDialogue (Variables|Default|GetFirst_Person) (Variables|Default|GetDialogue_Succès_Rouille))
      (Collision|SetCollisionProfileName (Variables|Default|GetBox_Back_Collision) "NoCollision" true :!class /Script/Engine.PrimitiveComponent))))

(event EventBeginPlay
  (|CallParentFunction) ; This node is disabled and will not be called.\nDrag off pins to build functionality.
)

(event Collision|EventActorBeginOverlap
  (params (OtherActor :type Actor%20Object%20Reference))
  (|CallParentFunction OtherActor) ; This node is disabled and will not be called.\nDrag off pins to build functionality.
)

(event EventTick
  (params (DeltaSeconds :type Float%20%28single-precision%29))
  (if (Variables|Default|GetCan_Turn_With_Player_?)
    (bind _asbp_diplome_first_person_project (Utilities|Casting|CastToBP_Diplome_First_Person_Project (Game|GetPlayerCharacter 0)))
    (Transformation|SetWorldRotation (Variables|Default|GetClue_To_How_Get_Item) (Math|Rotator|MakeRotator (.roll (Transformation|GetWorldRotation (Variables|/Game/GD/ThirdPerson/Blueprints/BP_Diplome_First_Person_Project.BP_Diplome_First_Person_Project_C|GetFirst_Person_Camera _asbp_diplome_first_person_project))) (+ (.pitch (Transformation|GetWorldRotation (Variables|/Game/GD/ThirdPerson/Blueprints/BP_Diplome_First_Person_Project.BP_Diplome_First_Person_Project_C|GetFirst_Person_Camera _asbp_diplome_first_person_project))) 9e+01) (.yaw (Transformation|GetWorldRotation (Variables|/Game/GD/ThirdPerson/Blueprints/BP_Diplome_First_Person_Project.BP_Diplome_First_Person_Project_C|GetFirst_Person_Camera _asbp_diplome_first_person_project)))) false false)))

(event EventActivationMovable
  (params (Actor_Hit :type Actor%20Object%20Reference) (Component_Hit :type Primitive%20Component%20Object%20Reference))
  (bind _get_item_needed_for_activites (Variables|Default|GetGet_Item_Needed_For_Activites))
  (bind _arrow_door (Variables|Default|GetArrow_Door))
  (bind _arrow_door_2 (Variables|Default|GetArrow_Door))
  (bind _arrow_door_3 (Variables|Default|GetArrow_Door))
  (bind _relativerotation (Variables|/Script/Engine.SceneComponent|GetRelativeRotation _arrow_door_2))
  (bind _relativerotation_2 (Variables|/Script/Engine.SceneComponent|GetRelativeRotation _arrow_door))
  (bind _relativerotation_3 (Variables|/Script/Engine.SceneComponent|GetRelativeRotation _arrow_door_2))
  (bind _relativerotation_4 (Variables|/Script/Engine.SceneComponent|GetRelativeRotation _arrow_door_3))
  (bind _asbp_diplome_first_person_project (Utilities|Casting|CastToBP_Diplome_First_Person_Project Actor_Hit))
  (Variables|Default|SetFirst_Person _asbp_diplome_first_person_project)
  (if (== Component_Hit (Variables|Default|GetBox_Back_Collision))
    (if (not (Variables|Default|GetOpen_?))
      (Variables|Default|SetWhat_Side_To_Open 1e+01)
      (if (Utilities|IsValidClass _get_item_needed_for_activites) :!label _label
        (Utilities|Casting|CastToBP_Base_Parent_Interactainable_DocumentsClass _get_item_needed_for_activites
          (:then
            (for _index (range (Variables|/Game/GD/ThirdPerson/Letter_Inventory.Letter_Inventory_C|GetMin_Index (Variables|/Game/GD/ThirdPerson/Blueprints/BP_Diplome_First_Person_Project.BP_Diplome_First_Person_Project_C|GetLetter_Inventory (Variables|Default|GetFirst_Person))) (Variables|/Game/GD/ThirdPerson/Letter_Inventory.Letter_Inventory_C|GetMax_Index (Variables|/Game/GD/ThirdPerson/Blueprints/BP_Diplome_First_Person_Project.BP_Diplome_First_Person_Project_C|GetLetter_Inventory (Variables|Default|GetFirst_Person))))
              (if (== (Utilities|GetClass (Utilities|Array|Get(acopy) (Variables|/Game/GD/ThirdPerson/Letter_Inventory.Letter_Inventory_C|GetAll_Letters (Variables|/Game/GD/ThirdPerson/Blueprints/BP_Diplome_First_Person_Project.BP_Diplome_First_Person_Project_C|GetLetter_Inventory (Variables|Default|GetFirst_Person))) _index)) (Variables|Default|GetGet_Item_Needed_For_Activites))
                (CallFunction|OpenDoors)
                (Default|TransmissDialogue (Variables|Default|GetFirst_Person) (Variables|Default|GetDialogue_De_Succès)))))
          (:CastFailed
            (Utilities|Casting|CastToBP_Base_Parent_Inventory_ItemClass _get_item_needed_for_activites
              (:then
                (if (== (Variables|Default|GetGet_Item_Needed_For_Activites) (Variables|/Script/Engine.ChildActorComponent|GetChildActorClass (Variables|/Game/GD/ThirdPerson/Blueprints/BP_Diplome_First_Person_Project.BP_Diplome_First_Person_Project_C|GetItem_Hold (Variables|Default|GetFirst_Person))))
                  (CallFunction|OpenDoors)
                  (elif (not (Variables|Default|GetRouille_?))
                    (Audio|SpawnSoundAttached "/Game/GD/Sound/Environment_Noise/SC_Trying_To_Open_Locked_Door_Cue.SC_Trying_To_Open_Locked_Door_Cue" (Variables|Default|GetDoor) "None" "0, 0, 0" "0, 0, 0" "SnapToTarget" false 1.0 1.0 0.0 0 0)
                    (Utilities|FlowControl|DoOnce false :!label _label_2
                      (:Completed
                        (Transformation|SetRelativeRotation _arrow_door_2 (Math|Rotator|MakeRotator (.roll _relativerotation_3) (.pitch _relativerotation_3) (+ (.yaw _relativerotation_3) 2.0)) false false)
                        (Utilities|FlowControl|Delay 0.1)
                        (Transformation|SetRelativeRotation _arrow_door_2 (Math|Rotator|MakeRotator (.roll _relativerotation) (.pitch _relativerotation) (- (.yaw _relativerotation) 4.0)) false false)
                        (Utilities|FlowControl|Delay 0.1)
                        (Transformation|SetRelativeRotation _arrow_door (Math|Rotator|MakeRotator (.roll _relativerotation_2) (.pitch _relativerotation_2) (+ (.yaw _relativerotation_2) 2.0)) false false)
                        (Default|TransmissDialogue (Variables|Default|GetFirst_Person) (Variables|Default|GetDialogue_Avec_Manque_Objet_Pour_Utilisation))
                        (Utilities|FlowControl|Delay 0.1)
                        (goto _label_2 Reset)))
                    (else
                      (Default|TransmissDialogue (Variables|Default|GetFirst_Person) (Variables|Default|GetDialogue_si_rouille))))))
              (:CastFailed
                (goto _label_2)))))
        (else
          (Audio|SpawnSoundAttached "/Game/GD/Sound/Environment_Noise/SC_Door_Opening_Cue.SC_Door_Opening_Cue" (Variables|Default|GetDoor) "None" "0, 0, 0" "0, 0, 0" "SnapToTarget" false 1.0 1.0 0.0 0 0)
          (Variables|Default|SetOpen_? true)
          (Transformation|SetRelativeRotation (Variables|Default|GetArrow_Door) (Math|Rotator|MakeRotator (.roll _relativerotation_4) (.pitch _relativerotation_4) (+ (.yaw _relativerotation_4) (* (Variables|Default|GetWhat_Side_To_Open) 1e+01))) false false)
          (Default|TransmissDialogue (Variables|Default|GetFirst_Person) (Variables|Default|GetDialogue_De_Succès))
          (Collision|SetCollisionProfileName (Variables|Default|GetBox_Back_Collision) "NoCollision" true :!class /Script/Engine.PrimitiveComponent))))
    (elif (== Component_Hit (Variables|Default|GetBox_Front_Collision))
      (if (not (Variables|Default|GetOpen_?))
        (Variables|Default|SetWhat_Side_To_Open -1e+01)
        (goto _label)))))

(fn ConstructionScript
  (|CallParentFunction))