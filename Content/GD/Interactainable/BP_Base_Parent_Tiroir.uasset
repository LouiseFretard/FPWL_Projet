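; Base parent actor for an inspectable interactable, named as a drawer (tiroir), with Start_Inspect left as an empty event.
; Pressing P clears Used, hands input from the actor back to the Inspector, and calls Inspect(false) on the first-person character.
; Mouse-drag Arrow rotation, input takeover and the angle-triggered text widget with blur fade remain only as disconnected logic that never runs.
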(event Custom|Start_Inspect
  (params (Inspector :type Pawn%20Object%20Reference) (Enigmes_Accomplie_? :type Boolean)))

(event EventBeginPlay)

(event Collision|EventActorBeginOverlap
  (params (OtherActor :type Actor%20Object%20Reference)))

(event EventTick
  (params (DeltaSeconds :type Float%20%28single-precision%29)))

(event Input|ActionEvents|InputActionInteraction
  (params (Key :type Key%20Structure)))

(event Input|ActionEvents|InputActionAnalyse
  (params (Key :type Key%20Structure))
  ;[1 1 1] Change_Input_To_Player
)

(event Input|MouseEvents|MouseX
  (params (AxisValue :type Float%20%28single-precision%29))
  ;[1 1 1] Make_Rotation_Depend_On_Mouse_Moving_On_Axis
)

(event Input|MouseEvents|MouseY
  (params (AxisValue :type Float%20%28single-precision%29))
  ;[1 1 1] Make_Rotation_Depend_On_Mouse_Moving_On_Axis
)

(event Input|KeyboardEvents|P
  (params (Key :type Key%20Structure))
  (bind _returnvalue (Game|GetPlayerController 0))
  ;[1 1 1] Change_Input_To_Player
  (:Pressed
    (Variables|Default|SetUsed? false)
    (Input|DisableInput _returnvalue)
    (Input|EnableInput (stale Custom|Start_Inspect Inspector) _returnvalue)
    (bind _asbp_diplome_first_person_project (Utilities|Casting|CastToBP_Diplome_First_Person_Project (stale Custom|Start_Inspect Inspector)))
    (Default|Inspect _asbp_diplome_first_person_project false)))

(event Input|KeyboardEvents|C
  (params (Key :type Key%20Structure)))

(event Input|KeyboardEvents|U
  (params (Key :type Key%20Structure)))

(fn ConstructionScript)